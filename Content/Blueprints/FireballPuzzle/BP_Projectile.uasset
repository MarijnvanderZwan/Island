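; Fireball puzzle projectile that reacts to what its collision component hits and then destroys itself.
; On hitting the player it applies per-shot damage credited to its shooter, with no explosion effects.
; Any other hit spawns an explosion emitter and a quiet fire sound at the projectile's location.
; Crates are also passed the impact point and normal through their own hit handler.
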(event `self.ReceiveBeginPlay`)

(event `self.Collision.OnComponentHit`
  (params (HitComponent :type "PrimitiveComponent Object Reference") (OtherActor :type "Actor Object Reference") (OtherComp :type "PrimitiveComponent Object Reference") (NormalImpulse :type "Vector Structure") (Hit :type "HitResult Structure (by ref)"))
  (bind (_bblockinghit _binitialoverlap _time _distance _location _impactpoint _normal _impactnormal) (`GameplayStatics.BreakHitResult` Hit))
  (bind _returnvalue (`self.K2_GetActorLocation`))
  (bind _asbp_player (cast `/Game/Blueprints/BP_Player` OtherActor)
    (:`then`
      (`GameplayStatics.ApplyDamage` _asbp_player (`self.DamagePerShot`) null (`self.Shooter`))
      (`self.K2_DestroyActor`))
    (:`CastFailed`
      (bind _asbp_crate (cast `/Game/Blueprints/BuildingBlocks/BP_Crate` OtherActor)
        (:`then`
          (`/Game/Blueprints/BuildingBlocks/BP_Crate.OnHitByProjectle` _asbp_crate _impactpoint _impactnormal))
        (:`CastFailed`
          _))
      (`GameplayStatics.SpawnEmitterAtLocation` "/Game/Effects/Particles/P_Explosion.P_Explosion" _returnvalue)
      (`self.K2_DestroyActor`)
      (`GameplayStatics.SpawnSoundAtLocation` "/Game/Audio/Effect/FireExplosion.FireExplosion" _returnvalue (struct) 0.05 1.0 0.0 null null))))

(fn `UserConstructionScript`)