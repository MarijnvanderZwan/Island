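; Behavior tree node for the ShyStalker AI that keeps the blackboard updated with the player target and its distance.
; On tick it caches the owning BP_ShyStalkerAIController on first use, then finds the first BP_Player through a GetAllActorsOfClass search repeated every tick.
; It writes that actor to TargetToFollow and its distance from the controlled pawn to DistanceToPlayer.
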(event `self.ReceiveTick`
  (params (OwnerActor :type "Actor Object Reference") (DeltaSeconds :type "Float (single-precision)"))
  (if (not (!= (`self.AIControllerRef`) null))
    (bind _asbp_shy_stalker_aicontroller (cast `/Game/Blueprints/ShyStalker/BP_ShyStalkerAIController` OwnerActor))
    (set `self.AIControllerRef` _asbp_shy_stalker_aicontroller))
  (bind _outactors (`GameplayStatics.GetAllActorsOfClass` "/Game/Blueprints/BP_Player.BP_Player_C"))
  (bind _item (`KismetArrayLibrary.Array_Get` _outactors))
  (`BTFunctionLibrary.SetBlackboardValueAsFloat` (`self.DistanceToPlayer`) (`Actor.GetDistanceTo` _item (`Controller.K2_GetPawn` (`self.AIControllerRef`))))
  (`BTFunctionLibrary.SetBlackboardValueAsObject` (`self.TargetToFollow`) _item))