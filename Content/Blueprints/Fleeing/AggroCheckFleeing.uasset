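; Behavior tree tick node, likely a service, that detects threats for AI controlled by BP_FleeingAIController.
; Each tick it sphere-traces around the pawn for desired object types, ignoring all Fleeing actors, then line-traces to each hit to confirm line of sight.
; Visible hits write TargetToFleeFrom and FleeLocation to the blackboard.
; A blocked hit or empty sweep clears only the target, so the last hit processed decides it.
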(event `self.ReceiveTick`
  (params (OwnerActor :type "Actor Object Reference") (DeltaSeconds :type "Float (single-precision)"))
  (bind _returnvalue (`Actor.K2_GetActorLocation` (`Controller.K2_GetPawn` (`self.AIControllerRef`))))
  (if (not (!= (`self.AIControllerRef`) null))
    (bind _asbp_fleeing_aicontroller (cast `/Game/Blueprints/Fleeing/BP_FleeingAIController` OwnerActor))
    (set `self.AIControllerRef` _asbp_fleeing_aicontroller))
  (bind _outactors (`GameplayStatics.GetAllActorsOfClass` "/Game/Blueprints/Fleeing/Fleeing.Fleeing_C"))
  (set `self.MyLocation` _returnvalue)
  (bind _outhits (`KismetSystemLibrary.SphereTraceMultiForObjects` _returnvalue (+ _returnvalue (0.0 0.0 15.0)) 500.0 (`self.DesiredObjectTypes`) false _outactors))
  (if (> (`KismetArrayLibrary.Array_Length` _outhits) 0)
    (for _array_element _outhits
      (bind (_bblockinghit _binitialoverlap _time _location _impactpoint _normal _impactnormal _physmat _hitactor) (`GameplayStatics.BreakHitResult` _array_element))
      (bind _outhit (`KismetSystemLibrary.LineTraceSingle` (`self.MyLocation`) (`Actor.K2_GetActorLocation` _hitactor) "TraceTypeQuery2" false _outactors))
      (bind (_bblockinghit_2 _binitialoverlap_2 _time_2 _location_2 _impactpoint_2 _normal_2 _impactnormal_2 _physmat_2 _hitactor_2) (`GameplayStatics.BreakHitResult` _outhit))
      (if (== _hitactor_2 _hitactor)
        (`BTFunctionLibrary.SetBlackboardValueAsObject` (`self.TargetToFleeFrom`) _hitactor_2)
        (`BTFunctionLibrary.SetBlackboardValueAsVector` (`self.FleeLocation`) (`Actor.K2_GetActorLocation` _hitactor_2))
        (else
          (`BTFunctionLibrary.SetBlackboardValueAsObject` (`self.TargetToFleeFrom`) :!label _label))))
    (else
      (goto _label))))