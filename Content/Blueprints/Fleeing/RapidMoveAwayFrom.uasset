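; Behavior tree task that moves a fleeing AI pawn a short step directly away from its blackboard TargetToFleeFrom actor.
; It caches the BP_FleeingAIController on first run, stops current movement, then offsets the pawn's location along the normalized away vector.
; AIMoveTo heads for a random reachable point near that offset.
; The task finishes only when the move succeeds; failed moves or casts never call FinishExecute.
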(event `self.ReceiveExecute`
  (params (OwnerActor :type "Actor Object Reference"))
  (bind _aicontrollerreference (`self.AIControllerReference`))
  (bind _returnvalue (`Controller.K2_GetPawn` _aicontrollerreference))
  (bind _returnvalue_2 (`Actor.K2_GetActorLocation` _returnvalue))
  (if (not (!= (`self.AIControllerReference`) null))
    (bind _asbp_fleeing_aicontroller (cast `/Game/Blueprints/Fleeing/BP_FleeingAIController` OwnerActor))
    (set `self.AIControllerReference` _asbp_fleeing_aicontroller))
  (`Controller.StopMovement` _aicontrollerreference)
  (`|AIMoveTo` _returnvalue (`NavigationSystem.GetRandomReachablePointInRadius` (+ _returnvalue_2 (* (`KismetMathLibrary.Normal` (- _returnvalue_2 (`Actor.K2_GetActorLocation` (`BTFunctionLibrary.GetBlackboardValueAsActor` (`self.TargetToFleeFrom`))))) 100.0)) 10.0) null 50.0
    (:`OnSuccess`
      (`self.FinishExecute` true))))