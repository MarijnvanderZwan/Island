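; BP_AnimatedDoor is a puzzle door that drops to a down position when triggered, then returns up after a set time.
; SetDown prints a debug message, resets the timer and moves the static mesh to DownLocation.
; Tick accumulates elapsed time while the door is down and restores UpLocation once DownTime is reached.
; Both moves are instant world-location changes without sweep or interpolation, despite the "Animated" name.
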(event `self.ReceiveTick`
  (params (DeltaSeconds :type "Float (single-precision)"))
  (if (`self.DoorIsDown`)
    (set `self.TimeActivated` (+ (`self.TimeActivated`) DeltaSeconds))
    (if (>= (`self.TimeActivated`) (`self.DownTime`))
      (`SceneComponent.K2_SetWorldLocation` (`self.StaticMesh`) (`self.UpLocation`) false false)
      (set `self.DoorIsDown` false))))

(event `SetDown`
  (`KismetSystemLibrary.PrintString` "Hello")
  (set `self.DoorIsDown` true)
  (set `self.TimeActivated` 0.0)
  (`SceneComponent.K2_SetWorldLocation` (`self.StaticMesh`) (`self.DownLocation`) false false))

(fn `UserConstructionScript`)