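; BP_DoorButton is a door puzzle button that responds to the player stepping into it.
; On overlap with BP_Player it flags the player as overlapping and calls SetUp on its Door.
; Its construction script registers the button with the BP_DoorButtonHandler in its ButtonHandler child actor.
; End overlap does nothing, as the logic that clears the flag and deactivates the button is disconnected.
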(event `self.ReceiveActorBeginOverlap`
  (params (OtherActor :type "Actor Object Reference"))
  (cast `/Game/Blueprints/BP_Player` OtherActor)
  (set `self.CurrentlyOverlappingPlayer` true)
  (`/Game/Blueprints/DoorPuzzle/BP_AnimatedDoor.SetUp` (`self.Door`)))

(event `self.ReceiveActorEndOverlap`
  (params (OtherActor :type "Actor Object Reference")))

(fn `UserConstructionScript`
  (bind _asbp_door_button_handler (cast `/Game/Blueprints/DoorPuzzle/BP_DoorButtonHandler` (`ChildActorComponent.ChildActor` (`self.ButtonHandler`))))
  (set `/Game/Blueprints/DoorPuzzle/BP_DoorButtonHandler.Button` self _asbp_door_button_handler))