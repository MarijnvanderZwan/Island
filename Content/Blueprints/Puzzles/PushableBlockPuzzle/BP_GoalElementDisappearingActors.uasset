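; Goal element for the pushable block puzzle that makes a set of actors disappear when the puzzle is solved.
; Its PuzzleSolved event loops over ActorsToDisappear, hiding each root component without propagating to children and disabling that actor's collision.
; The actors are not destroyed, and a debug "Disappearing" message prints after the loop.
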(event `self.PuzzleSolved`
  (for _array_element (`self.ActorsToDisappear`)
    (`SceneComponent.SetVisibility` (`Actor.RootComponent` _array_element) false false)
    (`self.SetActorEnableCollision` _array_element false))
  (`KismetSystemLibrary.PrintString` "Disappearing"))

(fn `UserConstructionScript`
  (`parent.UserConstructionScript`))