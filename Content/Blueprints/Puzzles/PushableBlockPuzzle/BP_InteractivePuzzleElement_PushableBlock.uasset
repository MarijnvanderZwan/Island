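; Pushable block element of a grid-style block puzzle that slides away from the side it is pushed on.
; Push picks the closest of four side colliders, inverts its relative X/Y signs into a direction, and asks the owning BP_Puzzle_PushableBlockPuzzle for the destination.
; Tick moves the block there at constant speed, blocking further pushes until it arrives.
; ResetToStartingLocation teleports it back to its BeginPlay position.
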(event `self.ReceiveBeginPlay`
  (bind _returnvalue (`self.K2_GetActorLocation`))
  (set `self.StartingPosition` _returnvalue)
  (set `self.EndLocation` _returnvalue)
  (`self.AddColliders`))

(event `self.ReceiveTick`
  (params (DeltaSeconds :type "Float (single-precision)"))
  (bind _endlocation (`self.EndLocation`))
  (bind _returnvalue (`SceneComponent.K2_GetComponentLocation` (`self.StaticMesh`)))
  (bind _returnvalue_2 (- _endlocation _returnvalue))
  (if (`self.Pushable`)
    _
    (elif (<= (`KismetMathLibrary.VSize` _returnvalue_2) 10.0)
      (`self.K2_SetActorLocation` _endlocation)
      (set `self.Pushable` true)
      (else
        (`self.K2_SetActorLocation` (+ (* (`KismetMathLibrary.Normal` _returnvalue_2) (* DeltaSeconds (`self.MovementSpeed`))) _returnvalue))))))

(fn `AddColliders`
  (bind _colliders (`self.Colliders`))
  (`KismetArrayLibrary.Array_Add` _colliders (`self.South`))
  (`KismetArrayLibrary.Array_Add` _colliders (`self.North`))
  (`KismetArrayLibrary.Array_Add` _colliders (`self.West`))
  (`KismetArrayLibrary.Array_Add` _colliders (`self.East`)))

(fn `GetClosestCollider`
  (params (Position :type "Vector Structure"))
  (returns (MinCollision :type "BoxComponent Object Reference"))
  (locals (MinCollider :type "BoxComponent Object Reference") (MinDistance :type "Float (double-precision)" :default 100000.0))
  (for _array_element (`self.Colliders`)
    (bind (_outpointonbody _returnvalue) (`PrimitiveComponent.GetClosestPointOnCollision` _array_element Position "None"))
    (if (< _returnvalue (`local.MinDistance`))
      (set `local.MinDistance` _returnvalue)
      (set `local.MinCollider` _array_element)))
  (return (`local.MinCollider`)))

(fn `Push`
  (params (`From Location` :type "Vector Structure"))
  (bind (_returnvalue_x _returnvalue_y _returnvalue_z) (`KismetMathLibrary.BreakVector` (`self.K2_GetActorLocation`)))
  (`KismetSystemLibrary.PrintString` "Pushing block!")
  (if (`self.Pushable`)
    (bind _mincollision (`self.GetClosestCollider` `From Location`))
    (bind _asbp_puzzle_pushable_block_puzzle (cast `/Game/Blueprints/Puzzles/PushableBlockPuzzle/BP_Puzzle_PushableBlockPuzzle` (`self.Puzzle`)))
    (bind (_relativelocation_x _relativelocation_y) (`KismetMathLibrary.BreakVector` (`SceneComponent.RelativeLocation` _mincollision)))
    (bind _output (`/Game/Blueprints/Puzzles/PushableBlockPuzzle/BP_Puzzle_PushableBlockPuzzle.PushBlockInDirection` _asbp_puzzle_pushable_block_puzzle self (`KismetMathLibrary.FTrunc` (* (`KismetMathLibrary.SignOfFloat` _relativelocation_x) -1.0)) (`KismetMathLibrary.FTrunc` (* (`KismetMathLibrary.SignOfFloat` _relativelocation_y) -1.0))))
    (set `self.EndLocation` (`KismetMathLibrary.MakeVector` (.x _output) (.y _output) _returnvalue_z))
    (set `self.Pushable` false)))

(fn `ResetToStartingLocation`
  (`self.K2_SetActorLocation` (`self.StartingPosition`) false true)
  (set `self.Direction` (0.0 0.0 0.0)))

(fn `UserConstructionScript`
  (`parent.UserConstructionScript`))