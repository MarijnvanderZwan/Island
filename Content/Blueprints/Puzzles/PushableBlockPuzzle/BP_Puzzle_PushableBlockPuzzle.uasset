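; Pushable block puzzle actor that maps placed puzzle elements onto a logical grid of 200-unit cells sized from its Grid box.
; On BeginPlay it registers obstacles, goals and pushable blocks with a child-actor PuzzleGrid and links interactive elements to itself.
; PushBlockInDirection delegates the move to PuzzleGrid and returns the destination in world space.
; ResetPuzzle teleports blocks to their starting positions and rebuilds the grid.
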(event `self.ReceiveBeginPlay`
  (`parent.ReceiveBeginPlay`)
  (`self.InitializeGrid`)
  (for _array_element (`self.InteractivePuzzleElements`)
    (set `/Game/Blueprints/GenericPuzzle/BP_InteractivePuzzleElement.Puzzle` self _array_element)))

(event `self.Reset Puzzle`
  (for _array_element (`self.InteractivePuzzleElements`)
    (bind _asbp_interactive_puzzle_element_pushable_block (cast `/Game/Blueprints/Puzzles/PushableBlockPuzzle/BP_InteractivePuzzleElement_PushableBlock` _array_element))
    (`self.K2_SetActorLocation` _asbp_interactive_puzzle_element_pushable_block (`/Game/Blueprints/Puzzles/PushableBlockPuzzle/BP_InteractivePuzzleElement_PushableBlock.StartingPosition` _asbp_interactive_puzzle_element_pushable_block) false true))
  (`self.InitializeGrid`))

(fn `GetGridLocationForWorldLocation`
  (params (`World Location` :type "Vector Structure"))
  (returns (NewParam :type "IntVector Structure"))
  (bind _top_left (`self.GetTopLeft`))
  (bind (_returnvalue_x _returnvalue_y) (`KismetMathLibrary.BreakVector` (- `World Location` _top_left)))
  (return (make `IntVector` (`KismetMathLibrary.FTrunc` (/ _returnvalue_x 200.0)) (`KismetMathLibrary.FTrunc` (/ _returnvalue_y 200.0)))))

(fn `GetPuzzleGrid`
  (returns (NewParam :type "PuzzleGrid Object Reference"))
  (bind _aspuzzle_grid (cast `PuzzleGrid` (`ChildActorComponent.ChildActor` (`self.PuzzleGrid`)))
    (:`then`
      (return _aspuzzle_grid))
    (:`CastFailed`
      (return _aspuzzle_grid))))

(fn `GetTopLeft`
  (returns (`Top Left` :type "Vector Structure"))
  (bind _grid (`self.Grid`))
  (return (- (`SceneComponent.K2_GetComponentLocation` _grid) (`BoxComponent.BoxExtent` _grid))))

(fn `GetWorldLocationForGridLocation`
  (params (`Grid Location` :type "IntVector Structure"))
  (returns (`World Location` :type "Vector Structure"))
  (bind _top_left (`self.GetTopLeft`))
  (return (+ _top_left (* (`KismetMathLibrary.Conv_IntVectorToVector` `Grid Location`) 200.0) (100.0 100.0 0.0))))

(fn `InitializeGrid`
  (bind (_returnvalue_x _returnvalue_y) (break `IntVector` (`KismetMathLibrary.FTruncVector` (/ (* (`BoxComponent.BoxExtent` (`self.Grid`)) 2.0) 200.0))))
  (bind _newparam (`self.GetPuzzleGrid`))
  (`PuzzleGrid.InitializeWithSize` _newparam _returnvalue_x _returnvalue_y)
  (for _array_element (`self.PuzzleElements`)
    (bind _newparam_2 (`self.GetGridLocationForWorldLocation` (`SceneComponent.K2_GetComponentLocation` (`/Game/Blueprints/GenericPuzzle/BP_PuzzleElement.StaticMesh` _array_element))))
    (cast `/Game/Blueprints/Puzzles/PushableBlockPuzzle/BP_PuzzleElement_ObstacleBlock` _array_element
      (:`then`
        (`PuzzleGrid.AddObstacle` _newparam (break `IntVector` _newparam_2) (`.Y` (break `IntVector` _newparam_2)) :!label _label))
      (:`CastFailed`
        (cast `/Game/Blueprints/Puzzles/PushableBlockPuzzle/BP_PuzzleElement_GoalObstacleBlock` _array_element
          (:`then`
            (goto _label))
          (:`CastFailed`
            (cast `/Game/Blueprints/Puzzles/PushableBlockPuzzle/BP_PuzzleElement_GoalBlock` _array_element)
            (`PuzzleGrid.AddGoal` _newparam (break `IntVector` _newparam_2) (`.Y` (break `IntVector` _newparam_2))))))))
  (for _array_element_2 (`self.InteractivePuzzleElements`)
    (bind _asbp_interactive_puzzle_element_pushable_block (cast `/Game/Blueprints/Puzzles/PushableBlockPuzzle/BP_InteractivePuzzleElement_PushableBlock` _array_element_2))
    (bind _newparam_3 (`self.GetGridLocationForWorldLocation` (`SceneComponent.K2_GetComponentLocation` (`/Game/Blueprints/Puzzles/PushableBlockPuzzle/BP_InteractivePuzzleElement_PushableBlock.StaticMesh` _asbp_interactive_puzzle_element_pushable_block))))
    (`PuzzleGrid.AddPushableBlock` _newparam (break `IntVector` _newparam_3) (`.Y` (break `IntVector` _newparam_3)))))

(fn `PushBlockInDirection`
  (params (Actor :type "Actor Object Reference") (DirectionX :type Integer) (DirectionY :type Integer))
  (returns (Output :type "Vector Structure"))
  (bind _newparam (`self.GetPuzzleGrid`))
  (bind _newparam_2 (`self.GetGridLocationForWorldLocation` (`self.K2_GetActorLocation` Actor)))
  (bind _returnvalue (`PuzzleGrid.PushBlockInDirection` _newparam (break `IntVector` _newparam_2) (`.Y` (break `IntVector` _newparam_2)) DirectionX DirectionY))
  (bind _world_location (`self.GetWorldLocationForGridLocation` (`KismetMathLibrary.FTruncVector` _returnvalue)))
  (return _world_location))

(fn `UserConstructionScript`
  (`parent.UserConstructionScript`))