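; Puzzle goal condition for the pushable block puzzle, deciding whether it is solved.
; CheckSolved filters the owning Puzzle's elements to BP_PuzzleElement, then casts each to BP_PuzzleElement_GoalBlock.
; It returns false if the filtered list is empty or any goal block is not Active, and true once the loop finds no inactive one.
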(fn `CheckSolved`
  (returns (Solved :type Boolean))
  (bind _filteredarray (`KismetArrayLibrary.FilterArray` (`/Game/Blueprints/GenericPuzzle/BP_Puzzle.PuzzleElements` (`self.Puzzle`)) "/Game/Blueprints/GenericPuzzle/BP_PuzzleElement.BP_PuzzleElement_C"))
  (if (> (`KismetArrayLibrary.Array_Length` _filteredarray) 0)
    (for _array_element _filteredarray
      (bind _asbp_puzzle_element_goal_block (cast `/Game/Blueprints/Puzzles/PushableBlockPuzzle/BP_PuzzleElement_GoalBlock` _array_element))
      (if (not (`/Game/Blueprints/Puzzles/PushableBlockPuzzle/BP_PuzzleElement_GoalBlock.Active` _asbp_puzzle_element_goal_block))
        (return false)))
    (return true)
    (else
      (return false))))

(fn `UserConstructionScript`
  (`parent.UserConstructionScript`))