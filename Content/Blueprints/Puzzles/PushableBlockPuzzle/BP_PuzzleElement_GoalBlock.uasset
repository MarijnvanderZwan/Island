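; BP_PuzzleElement_GoalBlock is a goal element for the pushable block puzzle that tracks whether a pushable block rests on it.
; When a pushable block enters its Box while inactive, it sets Activated and swaps that block's material to the lit blue rune.
; A pushable block leaving while active clears Activated and restores the unlit rune.
; It notifies nothing else and only maintains the flag.
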(event `self.Box.OnComponentBeginOverlap`
  (params (OverlappedComponent :type "PrimitiveComponent Object Reference") (OtherActor :type "Actor Object Reference") (OtherComp :type "PrimitiveComponent Object Reference") (OtherBodyIndex :type Integer) (bFromSweep :type Boolean) (SweepResult :type "HitResult Structure (by ref)"))
  (if (not (`self.Activated`))
    (bind _asbp_interactive_puzzle_element_pushable_block (cast `/Game/Blueprints/Puzzles/PushableBlockPuzzle/BP_InteractivePuzzleElement_PushableBlock` OtherActor))
    (set `self.Activated` true)
    (`PrimitiveComponent.SetMaterial` (`/Game/Blueprints/Puzzles/PushableBlockPuzzle/BP_InteractivePuzzleElement_PushableBlock.StaticMesh` _asbp_interactive_puzzle_element_pushable_block) 0 "/Game/Materials/M_BlockBlueRune.M_BlockBlueRune")))

(event `self.Box.OnComponentEndOverlap`
  (params (OverlappedComponent :type "PrimitiveComponent Object Reference") (OtherActor :type "Actor Object Reference") (OtherComp :type "PrimitiveComponent Object Reference") (OtherBodyIndex :type Integer))
  (if (`self.Activated`)
    (bind _asbp_interactive_puzzle_element_pushable_block (cast `/Game/Blueprints/Puzzles/PushableBlockPuzzle/BP_InteractivePuzzleElement_PushableBlock` OtherActor))
    (set `self.Activated` false)
    (`PrimitiveComponent.SetMaterial` (`/Game/Blueprints/Puzzles/PushableBlockPuzzle/BP_InteractivePuzzleElement_PushableBlock.StaticMesh` _asbp_interactive_puzzle_element_pushable_block) 0 "/Game/Materials/M_BlockBlueRune_off.M_BlockBlueRune_off")))

(fn `UserConstructionScript`
  (`parent.UserConstructionScript`))