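; Interactable actor for the lightbeam puzzle that players rotate around yaw in fixed increments.
; Primary and secondary interactions set a clockwise or counterclockwise step of MinimumRotation, and releasing either clears it.
; Tick turns the actor at a constant speed toward TargetRotation, which HandleRotation advances by one step when nearly reached while input is held, so released rotation finishes on its current increment.
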(event `self.ReceiveBeginPlay`
  (bind (_returnvalue_roll _returnvalue_pitch _returnvalue_yaw) (`KismetMathLibrary.BreakRotator` (`self.K2_GetActorRotation`)))
  (set `self.TargetRotation` _returnvalue_yaw))

(event `self.ReceiveTick`
  (params (DeltaSeconds :type "Float (single-precision)"))
  (bind (_returnvalue_roll _returnvalue_pitch) (`KismetMathLibrary.BreakRotator` (`self.K2_GetActorRotation`)))
  (bind _rotation (`self.HandleRotation` (* (`self.RotationDegreesPerSecond`) DeltaSeconds)))
  (`self.K2_SetActorRotation` (`KismetMathLibrary.MakeRotator` _returnvalue_roll _returnvalue_pitch _rotation)))

(event `RotateClockwise`
  (set `self.RotationDirection` (`self.MinimumRotation`)))

(event `RotateCounterClockwise`
  (set `self.RotationDirection` (* (`self.MinimumRotation`) -1.0)))

(event `/Game/Blueprints/Gameplay/InteractableObject.InteractWithObject`
  (params (TriggerLocation :type "Vector Structure"))
  (`self.RotateClockwise`))

(event `StopRotation`
  (set `self.RotationDirection` 0.0))

(event `/Game/Blueprints/Gameplay/InteractableObject.SecondaryInteractWithObject`
  (params (TriggerLocation :type "Vector Structure"))
  (`self.RotateCounterClockwise`))

(event `/Game/Blueprints/Gameplay/InteractableObject.InteractWithObjectReleased`
  (params (TriggerLocation :type "Vector Structure"))
  (`self.StopRotation`))

(event `/Game/Blueprints/Gameplay/InteractableObject.SecondaryInteractWithObjectReleased`
  (params (TriggerLocation :type "Vector Structure"))
  (`self.StopRotation`))

(fn `HandleRotation`
  (params (NewParam :type "Float (double-precision)"))
  (returns (Rotation :type "Float (double-precision)"))
  (locals (DegreesToRotate :type "Float (double-precision)") (CurrentRotation :type "Float (double-precision)"))
  (bind (_returnvalue_roll _returnvalue_pitch _returnvalue_yaw) (`KismetMathLibrary.BreakRotator` (`self.K2_GetActorRotation`)))
  (set `local.DegreesToRotate` NewParam)
  (bind _output_get (set `local.CurrentRotation` _returnvalue_yaw))
  (`|ExecutionSequence`
    (:`then_0`
      ;[1 1 1] Adjust target rotation
      (if (< (`KismetMathLibrary.Abs` (- _output_get (`self.TargetRotation`))) (`local.DegreesToRotate`))
        (if (== (`self.RotationDirection`) 0.0)
          (return (`self.TargetRotation`))
          (else
            (set `self.TargetRotation` (+ (`self.TargetRotation`) (`self.RotationDirection`)))))))
    (:`then_1`
      ;[1 1 1] Adjust current rotation towards target rotation
      (return (+ (* (`KismetMathLibrary.SignOfFloat` (- (`self.TargetRotation`) (`local.CurrentRotation`))) (`local.DegreesToRotate`)) (`local.CurrentRotation`))))))

(fn `UserConstructionScript`)