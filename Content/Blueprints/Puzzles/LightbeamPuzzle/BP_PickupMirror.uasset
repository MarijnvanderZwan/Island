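; BP_PickupMirror is a pickup mirror for the lightbeam puzzle that the player can hold and aim to redirect light.
; It finds BP_Player at BeginPlay, assigns itself a GUID, and compares that against the player's selected object and active physics handle to detect being held.
; While held, Tick matches the mesh's rotation to the player's.
; GetRedirectVector supplies the redirect origin at Center and a long vector along the mesh's forward axis.
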(event `self.ReceiveBeginPlay`
  (bind _outactors (`GameplayStatics.GetAllActorsOfClass` "/Game/Blueprints/BP_Player.BP_Player_C"))
  (if (> (`KismetArrayLibrary.Array_Length` _outactors) 0)
    (set `self.Player` (`|GetArrayItem` _outactors))
    (set `self.ObjectId` (`KismetGuidLibrary.NewGuid`))
    (else
      (`KismetSystemLibrary.PrintString` "BP_PickupMirror.EventGraph: Player not found"))))

(event `self.ReceiveTick`
  (params (DeltaSeconds :type "Float (single-precision)"))
  (bind _ispickedup (`self.IsCurrentlyPickedUp`))
  (if _ispickedup
    (`SceneComponent.K2_SetWorldRotation` (`self.StaticMesh`) (`self.K2_GetActorRotation` (`self.Player`)) false false)))

(fn `GetRedirectVector`
  (returns (Start :type "Vector Structure") (Direction :type "Vector Structure"))
  (return (`SceneComponent.K2_GetComponentLocation` (`self.Center`)) (* (`SceneComponent.GetForwardVector` (`self.StaticMesh`)) 10000.0)))

(fn `IsCurrentlyPickedUp`
  (returns (IsPickedUp :type Boolean))
  (bind _player (`self.Player`))
  (if (!= _player null)
    (bind _asbp_pickup_mirror (cast `/Game/Blueprints/Puzzles/LightbeamPuzzle/BP_PickupMirror` (`/Game/Blueprints/BP_Player.SelectedObject` _player)))
    (return (and (== (`/Game/Blueprints/Puzzles/LightbeamPuzzle/BP_PickupMirror.ObjectId` _asbp_pickup_mirror) (`self.ObjectId`)) (`/Game/Blueprints/BP_Player.PhysicsHandleActive` _player)))
    (else
      (return false))))

(fn `UserConstructionScript`)