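; Lightbeam puzzle crystal that supplies an outgoing beam origin and direction from its Out component.
; GetReflectedResult returns Out's world location and its forward vector scaled to a long range, independent of any incoming beam angle.
; The Absorb event runs a complex line trace against WorldStatic objects along that same path, but nothing uses the hit result yet.
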(event `Absorb`
  (bind _out (`self.Out`))
  (bind _returnvalue (`SceneComponent.K2_GetComponentLocation` _out))
  (bind _outhit (`KismetSystemLibrary.LineTraceSingleForObjects` _returnvalue (+ _returnvalue (* (`SceneComponent.GetForwardVector` _out) 10000.0)) (`|MakeArray` "ObjectTypeQuery1" :!type "EObjectTypeQuery Enum") true)))

(fn `GetReflectedResult`
  (returns (Start :type "Vector Structure") (Direction :type "Vector Structure"))
  (bind _out (`self.Out`))
  (return (`SceneComponent.K2_GetComponentLocation` _out) (* (`SceneComponent.GetForwardVector` _out) 10000.0)))

(fn `UserConstructionScript`)