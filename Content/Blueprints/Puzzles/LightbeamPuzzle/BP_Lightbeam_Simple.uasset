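; Simplified lightbeam for a light puzzle that draws a particle beam between two hardcoded world positions on BeginPlay or Initialize.
; RecalculateBeam spawns two movable StaticMeshActors as endpoints and feeds them to a particle component's BeamSource and BeamTarget instance parameters.
; Arrow-directed line tracing (Bounce) and endpoint repositioning are unfinished: their calls are disconnected, and Tick only accumulates time.
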(event `self.ReceiveBeginPlay`
  (`self.RecalculateBeam`))

(event `Initialize`
  (`self.RecalculateBeam`))

(event `RecalculateBeam`
  (`|ExecutionSequence`
    (:`then_2`
      (`self.SpawnComponentsForPositions` (13100.0 -13500.0 400.0) (12100.0 -13500.0 400.0)))))

(event `self.ReceiveTick`
  (params (DeltaSeconds :type "Float (single-precision)"))
  (bind _output_get (set `self.TimeSinceLastTick` (+ (`self.TimeSinceLastTick`) DeltaSeconds)))
  (if (> _output_get (`self.TimeBetweenTicks`))
    _))

(event `Bounce`
  (params (ActorsToIgnore :type "Array of Actor Object Reference"))
  (bind _start (`self.Start`))
  (bind (_outhit _returnvalue) (`KismetSystemLibrary.LineTraceSingleForObjects` _start (+ _start (* (`self.BeamDirection`) 10.0)) (`|MakeArray` "ObjectTypeQuery1" "ObjectTypeQuery2" "ObjectTypeQuery3" "ObjectTypeQuery4" "ObjectTypeQuery6" :!type "EObjectTypeQuery Enum") false ActorsToIgnore))
  (bind (_bblockinghit _binitialoverlap _time _distance _location _impactpoint _normal _impactnormal _physmat _hitactor) (`GameplayStatics.BreakHitResult` _outhit))
  (if (and _returnvalue (!= _hitactor null))
    (`KismetArrayLibrary.Array_Add` (`self.Positions`) _impactpoint)
    (`GameplayStatics.SpawnEmitterAtLocation` "/Game/Effects/Particles/P_ArcaneBolt.P_ArcaneBolt" _impactpoint (struct) (1.0 1.0 1.0) false)))

(event `SetPositions`)

(fn `DestroyComponents`
  (for _array_element (`SceneComponent.GetChildrenComponents` (`self.Arrow`) false)
    (`ActorComponent.K2_DestroyComponent` _array_element)))

(fn `SetComponentPositions`
  (params (Vector1 :type "Vector Structure") (Vector2 :type "Vector Structure"))
  (bind _actors (`self.Actors`))
  (`self.K2_SetActorLocation` (`|GetArrayItem` _actors) Vector1 false true)
  (`self.K2_SetActorLocation` (`|GetArrayItem` _actors 1) Vector2 false true)
  (set `ParticleSystemComponent.InstanceParameters` (`|MakeArray` (make `ParticleSysParam` "BeamSource" "PSPT_Actor" 0.0 0.0 Vector1) (make `ParticleSysParam` "BeamTarget" "PSPT_Actor" 0.0 0.0 Vector2)) (`self.ParticleComponent`)))

(fn `SpawnComponentsForPositions`
  (params (Position1 :type "Vector Structure") (Position2 :type "Vector Structure"))
  (bind _actors (`self.Actors`))
  (bind _returnvalue (`AddComponent|NODE_AddParticleSystemComponent-1`))
  (set `self.ParticleComponent` _returnvalue)
  (bind _returnvalue_2 (`|SpawnActorFromClass` "/Script/Engine.StaticMeshActor" (`KismetMathLibrary.MakeTransform` Position1) "AlwaysSpawn" "OverrideRootScale" null null))
  (`StaticMeshActor.SetMobility` _returnvalue_2 "Movable")
  (`KismetArrayLibrary.Array_Add` _actors _returnvalue_2)
  (bind _returnvalue_3 (`|SpawnActorFromClass` "/Script/Engine.StaticMeshActor" (`KismetMathLibrary.MakeTransform` Position2) "AlwaysSpawn" "OverrideRootScale" null null))
  (`StaticMeshActor.SetMobility` _returnvalue_3 "Movable")
  (`KismetArrayLibrary.Array_Add` _actors _returnvalue_3)
  (set `ParticleSystemComponent.InstanceParameters` (`|MakeArray` (make `ParticleSysParam` "BeamSource" "PSPT_Actor" 0.0 0.0 Position1 (0.0 0.0 0.0) (struct) _returnvalue_2) (make `ParticleSysParam` "BeamTarget" "PSPT_Actor" 0.0 0.0 Position2 (0.0 0.0 0.0) (struct) _returnvalue_3)) _returnvalue))

(fn `UserConstructionScript`)