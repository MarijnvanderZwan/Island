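; Light beam source for the lightbeam puzzle, building a bouncing beam that can activate detectors.
; Bounce recursively line-traces and records points by hit-actor tag: mirroring off reflectors, redirecting through crystals, activating detectors at goals.
; SetPositions rebuilds particle beam segments between those points, using spawned StaticMeshActors as endpoints.
; Tick and RecalculateBeam are empty; their timed recalculation logic is disconnected, so this graph never starts the beam itself.
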(event `self.ReceiveTick`
  (params (DeltaSeconds :type "Float (single-precision)")))

(event `RecalculateBeam`)

(event `Bounce`
  (params (ActorsToIgnore :type "Array of Actor Object Reference"))
  (bind _start (`self.Start`))
  (bind _positions (`self.Positions`))
  (bind _returnvalue (+ _start (* (`self.BeamDirection`) 10.0)))
  (bind (_outhit _returnvalue_2) (`KismetSystemLibrary.LineTraceSingleForObjects` _start _returnvalue (`|MakeArray` "ObjectTypeQuery1" "ObjectTypeQuery2" "ObjectTypeQuery3" "ObjectTypeQuery4" "ObjectTypeQuery6" :!type "EObjectTypeQuery Enum") false ActorsToIgnore))
  (bind (_bblockinghit _binitialoverlap _time _distance _location _impactpoint _normal _impactnormal _physmat _hitactor) (`GameplayStatics.BreakHitResult` _outhit))
  (if (and _returnvalue_2 (!= _hitactor null))
    (bind _tags (`Actor.Tags` _hitactor))
    (if (`KismetArrayLibrary.Array_Contains` _tags "Reflect")
      (set `self.BeamDirection` (`KismetMathLibrary.MirrorVectorByNormal` (- _impactpoint (`self.Start`)) _impactnormal))
      (bind _output_get (set `self.Start` _impactpoint))
      (`KismetArrayLibrary.Array_Add` (`self.Positions`) _output_get)
      (`GameplayStatics.SpawnEmitterAtLocation` "/Game/Effects/Particles/P_ArcaneBolt.P_ArcaneBolt" _output_get)
      (`self.Bounce` (`|MakeArray` _hitactor))
      (elif (`KismetArrayLibrary.Array_Contains` _tags "ReflectGoal")
        (bind _asbp_puzzle_element_lightbeam_detector (cast `/Game/Blueprints/Puzzles/LightbeamPuzzle/BP_PuzzleElement_LightbeamDetector` _hitactor)
          (:`then`
            (set `/Game/Blueprints/Puzzles/LightbeamPuzzle/BP_PuzzleElement_LightbeamDetector.Activated` true _asbp_puzzle_element_lightbeam_detector))
          (:`CastFailed`
            _))
        (`KismetArrayLibrary.Array_Add` (`self.Positions`) _impactpoint)
        (`GameplayStatics.SpawnEmitterAtLocation` "/Game/Effects/Particles/P_ArcaneBolt.P_ArcaneBolt" _impactpoint)
        (elif (`KismetArrayLibrary.Array_Contains` _tags "Absorb")
          (bind _asbp_puzzle_element_lightbeam_crystal (cast `/Game/Blueprints/Puzzles/LightbeamPuzzle/BP_PuzzleElement_LightbeamCrystal` _hitactor))
          (bind (_start_2 _direction) (`/Game/Blueprints/Puzzles/LightbeamPuzzle/BP_PuzzleElement_LightbeamCrystal.GetReflectedResult` _asbp_puzzle_element_lightbeam_crystal))
          (`KismetArrayLibrary.Array_Add` _positions _impactpoint)
          (set `self.Start` _start_2)
          (`KismetArrayLibrary.Array_Add` _positions _start_2)
          (`GameplayStatics.SpawnEmitterAtLocation` "/Game/Effects/Particles/P_ArcaneBolt.P_ArcaneBolt" _start_2)
          (set `self.BeamDirection` _direction)
          (`self.Bounce` (`|MakeArray` _hitactor))
          (else
            (`KismetArrayLibrary.Array_Add` (`self.Positions`) _location)
            (`GameplayStatics.SpawnEmitterAtLocation` "/Game/Effects/Particles/P_ArcaneBolt.P_ArcaneBolt" _location)))))
    (else
      (`KismetArrayLibrary.Array_Add` (`self.Positions`) _returnvalue))))

(event `SetPositions`
  (bind _positions (`self.Positions`))
  (bind _actors (`self.Actors`))
  (`self.DestroyComponents`)
  (for _array_element _actors
    (`self.K2_DestroyActor` _array_element))
  (`KismetArrayLibrary.Array_Clear` _actors)
  (for _index (range 1 (`KismetArrayLibrary.Array_Length` (`self.Positions`)))
    (`self.SpawnComponentsForPositions` (`|GetArrayItem` _positions _index) (`|GetArrayItem` _positions (- _index 1)))
    (set `self.TimeSinceLastTick` 0.0)))

(fn `DestroyComponents`
  (for _array_element (`SceneComponent.GetChildrenComponents` (`self.Arrow`) false)
    (`ActorComponent.K2_DestroyComponent` _array_element)))

(fn `SpawnComponentsForPositions`
  (params (Position1 :type "Vector Structure") (Position2 :type "Vector Structure"))
  (bind _actors (`self.Actors`))
  (bind _returnvalue (`AddComponent|NODE_AddParticleSystemComponent-1`))
  (bind _returnvalue_2 (`|SpawnActorFromClass` "/Script/Engine.StaticMeshActor" (`KismetMathLibrary.MakeTransform` Position1) "AlwaysSpawn" "OverrideRootScale" null null))
  (`KismetArrayLibrary.Array_Add` _actors _returnvalue_2)
  (bind _returnvalue_3 (`|SpawnActorFromClass` "/Script/Engine.StaticMeshActor" (`KismetMathLibrary.MakeTransform` Position2) "AlwaysSpawn" "OverrideRootScale" null null))
  (`KismetArrayLibrary.Array_Add` _actors _returnvalue_3)
  (set `ParticleSystemComponent.InstanceParameters` (`|MakeArray` (make `ParticleSysParam` "BeamSource" "PSPT_Actor" 0.0 0.0 Position1 (0.0 0.0 0.0) (struct) _returnvalue_2) (make `ParticleSysParam` "BeamTarget" "PSPT_Actor" 0.0 0.0 Position2 (0.0 0.0 0.0) (struct) _returnvalue_3)) _returnvalue))

(fn `UserConstructionScript`)