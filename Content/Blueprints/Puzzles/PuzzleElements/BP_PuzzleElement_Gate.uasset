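; A puzzle element gate actor that animates open and closed on its skeletal mesh, opening as soon as play begins.
; Open and Close events share one non-looping Gate_Anim, setting the play rate forward or negative before calling PlayAnimation.
; Close also prints a debug message, and nothing in this Blueprint calls it.
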(event `self.ReceiveBeginPlay`
  (`parent.ReceiveBeginPlay`)
  (`self.Open`))

(event `Close`
  (bind _skeletalmesh (`self.SkeletalMesh`))
  (`SkeletalMeshComponent.SetPlayRate` _skeletalmesh -1.0)
  (`SkeletalMeshComponent.PlayAnimation` _skeletalmesh "/Game/Meshes/Arnimated/Gate_Anim.Gate_Anim" false)
  (`KismetSystemLibrary.PrintString` "Closing"))

(event `Open`
  (bind _skeletalmesh (`self.SkeletalMesh`))
  (`SkeletalMeshComponent.SetPlayRate` _skeletalmesh 1.0)
  (`SkeletalMeshComponent.PlayAnimation` _skeletalmesh "/Game/Meshes/Arnimated/Gate_Anim.Gate_Anim" false))

(fn `UserConstructionScript`
  (`parent.UserConstructionScript`))