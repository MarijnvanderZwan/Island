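; BP_PuzzleElement_FireballShooter is a puzzle actor, filed under the fireball survival puzzle, that fires projectiles at a regular interval.
; Tick accumulates delta time and calls ShootFireball once it exceeds TimeBetweenTicks, resetting the timer to zero.
; ShootFireball spawns BP_Projectile at the ShootLocation component's world position and rotation.
; It then passes that component's world forward vector, scaled by the projectile's max speed, to SetVelocityInLocalSpace.
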(event `self.ReceiveTick`
  (params (DeltaSeconds :type "Float (single-precision)"))
  (bind _output_get (set `self.TimeSinceLastShot` (+ DeltaSeconds (`self.TimeSinceLastShot`))))
  (if (> _output_get (`self.TimeBetweenTicks`))
    (set `self.TimeSinceLastShot` 0.0)
    (`self.ShootFireball`)))

(fn `ShootFireball`
  (bind _shootlocation (`self.ShootLocation`))
  (bind _returnvalue (`|SpawnActorFromClass` "/Game/Blueprints/FireballPuzzle/BP_Projectile.BP_Projectile_C" (`KismetMathLibrary.MakeTransform` (`SceneComponent.K2_GetComponentLocation` _shootlocation) (`SceneComponent.K2_GetComponentRotation` (`self.ShootLocation`))) "Undefined" "OverrideRootScale" null null))
  (bind _projectilemovement (`/Game/Blueprints/FireballPuzzle/BP_Projectile.ProjectileMovement` _returnvalue))
  (`ProjectileMovementComponent.SetVelocityInLocalSpace` _projectilemovement (* (`SceneComponent.GetForwardVector` _shootlocation) (`MovementComponent.GetMaxSpeed` _projectilemovement))))

(fn `UserConstructionScript`
  (`parent.UserConstructionScript`))