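; Goal condition actor for the fireball survival puzzle, met once survival has lasted a set number of seconds.
; Tick accumulates elapsed time while Activated is true and resets it to zero whenever it is false.
; CheckSolved reports success when the accumulated time reaches NumberOfSecondsToSurvive.
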(event `self.ReceiveTick`
  (params (DeltaSeconds :type "Float (single-precision)"))
  (if (`self.Activated`)
    (set `self.NumberOfSecondsSurvived` (+ DeltaSeconds (`self.NumberOfSecondsSurvived`)))
    (else
      (set `self.NumberOfSecondsSurvived` 0.0))))

(fn `CheckSolved`
  (returns (Solved :type Boolean))
  (return (>= (`self.NumberOfSecondsSurvived`) (`self.NumberOfSecondsToSurvive`))))

(fn `UserConstructionScript`
  (`parent.UserConstructionScript`))