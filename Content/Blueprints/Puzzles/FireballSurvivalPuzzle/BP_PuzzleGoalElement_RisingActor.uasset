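; BP_PuzzleGoalElement_RisingActor is a puzzle goal element that raises its static mesh when the puzzle is solved.
; On BeginPlay it records the mesh's starting Z and computes an end height from HeightToRise.
; PuzzleSolved sets a rising flag, and Tick then moves the mesh up in world space at a constant speed, clamped to the end height.
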(event `self.ReceiveBeginPlay`
  (bind (_returnvalue_x _returnvalue_y _returnvalue_z) (`KismetMathLibrary.BreakVector` (`SceneComponent.K2_GetComponentLocation` (`self.StaticMesh`))))
  (`parent.ReceiveBeginPlay`)
  (set `self.StartingHeight` _returnvalue_z)
  (set `self.EndHeight` (+ _returnvalue_z (`self.HeightToRise`))))

(event `self.ReceiveTick`
  (params (DeltaSeconds :type "Float (single-precision)"))
  (bind _staticmesh (`self.StaticMesh`))
  (bind (_returnvalue_x _returnvalue_y _returnvalue_z) (`KismetMathLibrary.BreakVector` (`SceneComponent.K2_GetComponentLocation` _staticmesh)))
  (`parent.ReceiveTick` DeltaSeconds)
  (if (`self.CurrentlyRising`)
    (if (< _returnvalue_z (`self.EndHeight`))
      (`SceneComponent.K2_SetWorldLocation` _staticmesh (`KismetMathLibrary.MakeVector` _returnvalue_x _returnvalue_y (`KismetMathLibrary.FMin` (+ _returnvalue_z (* DeltaSeconds (`self.RisingSpeedPerSecond`))) (`self.EndHeight`))) false false))))

(event `self.PuzzleSolved`
  (set `self.CurrentlyRising` true))

(fn `UserConstructionScript`
  (`parent.UserConstructionScript`))