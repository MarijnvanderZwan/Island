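; Puzzle element that lines a spline with intelligent fireball shooters, as part of a fireball survival puzzle.
; On BeginPlay it derives the shooter count from spline length and spacing, then spawns the shooters at even intervals from the spline start.
; Each shooter is rotated in yaw only to face the FocusPoint component, staying level regardless of height difference.
; Shooters exist only at runtime, since the construction script adds nothing.
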(event `self.ReceiveBeginPlay`
  (`parent.ReceiveBeginPlay`)
  (`self.InitializeShooters`))

(fn `InitializeShooters`
  (locals (numberOfShooters :type Integer))
  (bind _output_get (set `local.numberOfShooters` (`KismetMathLibrary.FTrunc` (/ (`SplineComponent.GetSplineLength` (`self.Spline`)) (`self.DistanceBetweenShooters`)))))
  (for _index (range _output_get)
    (bind _returnvalue (`SplineComponent.GetLocationAtDistanceAlongSpline` (`self.Spline`) (* _index (`self.DistanceBetweenShooters`)) "World"))
    (`|SpawnActorFromClass` "/Game/Blueprints/Puzzles/FireballSurvivalPuzzle/BP_PuzzleElement_IntelligentFireballShooter.BP_PuzzleElement_IntelligentFireballShooter_C" (`KismetMathLibrary.MakeTransform` _returnvalue (`KismetMathLibrary.MakeRotator` 0.0 0.0 (.yaw (`KismetMathLibrary.FindLookAtRotation` _returnvalue (`SceneComponent.K2_GetComponentLocation` (`self.FocusPoint`)))))) "Undefined" "OverrideRootScale" null null)))

(fn `UserConstructionScript`
  (`parent.UserConstructionScript`))