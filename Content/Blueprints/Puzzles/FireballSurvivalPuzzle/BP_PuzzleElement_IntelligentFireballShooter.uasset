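; Fireball shooter puzzle element that fires either toward the player or along its own facing, chosen at random per shot.
; BeginPlay randomly offsets the inherited TimeBetweenTicks so timing varies between instances.
; ShootFireball calls ShootAtPlayer or ShootAtShootLocation, each spawning a BP_Projectile at ShootLocation with slight random yaw spread.
; Both pass the projectile's world forward vector at max speed into SetVelocityInLocalSpace.
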(event `self.ReceiveBeginPlay`
  (bind _timebetweenticks (`self.TimeBetweenTicks`))
  (`parent.ReceiveBeginPlay`)
  (set `self.TimeBetweenTicks` (`KismetMathLibrary.RandomFloatInRange` (- _timebetweenticks 1.0) (+ _timebetweenticks 1.0))))

(event `self.ShootFireball`
  (if (`KismetMathLibrary.RandomBool`)
    (`self.ShootAtPlayer`)
    (else
      (`self.ShootAtShootLocation`))))

(fn `ShootAtPlayer`
  (bind _returnvalue (`SceneComponent.K2_GetComponentLocation` (`self.ShootLocation`)))
  (bind _outactors (`GameplayStatics.GetAllActorsOfClass` "/Game/Blueprints/BP_Player.BP_Player_C"))
  (bind (_returnvalue_roll _returnvalue_pitch _returnvalue_yaw) (`KismetMathLibrary.BreakRotator` (`KismetMathLibrary.FindLookAtRotation` _returnvalue (`self.K2_GetActorLocation` (`|GetArrayItem` _outactors)))))
  (bind _returnvalue_2 (`|SpawnActorFromClass` "/Game/Blueprints/FireballPuzzle/BP_Projectile.BP_Projectile_C" (`KismetMathLibrary.MakeTransform` _returnvalue (`KismetMathLibrary.MakeRotator` 0.0 0.0 (`KismetMathLibrary.RandomFloatInRange` (- _returnvalue_yaw 5.0) (+ _returnvalue_yaw 5.0)))) "Undefined" "OverrideRootScale" null null))
  (bind _projectilemovement (`/Game/Blueprints/FireballPuzzle/BP_Projectile.ProjectileMovement` _returnvalue_2))
  (`ProjectileMovementComponent.SetVelocityInLocalSpace` _projectilemovement (* (`self.GetActorForwardVector` _returnvalue_2) (`MovementComponent.GetMaxSpeed` _projectilemovement))))

(fn `ShootAtShootLocation`
  (bind _shootlocation (`self.ShootLocation`))
  (bind (_returnvalue_roll _returnvalue_pitch _returnvalue_yaw) (`KismetMathLibrary.BreakRotator` (`SceneComponent.K2_GetComponentRotation` _shootlocation)))
  (bind _returnvalue (`|SpawnActorFromClass` "/Game/Blueprints/FireballPuzzle/BP_Projectile.BP_Projectile_C" (`KismetMathLibrary.MakeTransform` (`SceneComponent.K2_GetComponentLocation` _shootlocation) (`KismetMathLibrary.MakeRotator` 0.0 0.0 (`KismetMathLibrary.RandomFloatInRange` (- _returnvalue_yaw 5.0) (+ _returnvalue_yaw 5.0)))) "Undefined" "OverrideRootScale" null null))
  (bind _projectilemovement (`/Game/Blueprints/FireballPuzzle/BP_Projectile.ProjectileMovement` _returnvalue))
  (`ProjectileMovementComponent.SetVelocityInLocalSpace` _projectilemovement (* (`self.GetActorForwardVector` _returnvalue) (`MovementComponent.GetMaxSpeed` _projectilemovement))))

(fn `UserConstructionScript`
  (`parent.UserConstructionScript`))