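; BP_PuzzleElement_ActivationArea is a one-shot trigger area that activates a puzzle when the player enters it.
; Its Box overlap checks for BP_Player, teleports the whole actor vertically by ActivationZOffset and latches Activated.
; It then plays StoneFallSound at the world origin and calls Activated on its Puzzle reference.
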(event `self.Box.OnComponentBeginOverlap`
  (params (OverlappedComponent :type "PrimitiveComponent Object Reference") (OtherActor :type "Actor Object Reference") (OtherComp :type "PrimitiveComponent Object Reference") (OtherBodyIndex :type Integer) (bFromSweep :type Boolean) (SweepResult :type "HitResult Structure (by ref)"))
  (if (not (`self.Activated`))
    (cast `/Game/Blueprints/BP_Player` OtherActor)
    (`self.K2_AddActorWorldOffset` (`KismetMathLibrary.MakeVector` 0.0 0.0 (`self.ActivationZOffset`)) false true)
    (set `self.Activated` true)
    (`GameplayStatics.PlaySoundAtLocation` "/Game/Audio/Effect/StoneFallSound.StoneFallSound")
    (`/Game/Blueprints/GenericPuzzle/BP_Puzzle.Activated` (`self.Puzzle`))))

(fn `UserConstructionScript`
  (`parent.UserConstructionScript`))