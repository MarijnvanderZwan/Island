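; BP_Puzzle_FireballSurvival is the controller for the fireball survival puzzle, relaying activation and completion to the actors that make up the puzzle.
; Activate switches on every BP_PuzzleElement in PuzzleElements.
; PuzzleIsSolved notifies every BP_PuzzleGoalElement in PuzzleGoalElements, deactivates the puzzle elements and sets the PuzzleSolved flag.
; The graph holds no survival or win-condition logic of its own.
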(event `self.ReceiveBeginPlay`
  (`parent.ReceiveBeginPlay`))

(event `self.Activate`
  (`|ExecutionSequence`
    (:`then_1`
      (for _array_element (`self.PuzzleElements`)
        (bind _asbp_puzzle_element (cast `/Game/Blueprints/GenericPuzzle/BP_PuzzleElement` _array_element))
        (`/Game/Blueprints/GenericPuzzle/BP_PuzzleElement.Activate` _asbp_puzzle_element)))))

(event `self.PuzzleIsSolved`
  (`|ExecutionSequence`
    (:`then_0`
      (for _array_element (`self.PuzzleGoalElements`)
        (bind _asbp_puzzle_goal_element (cast `/Game/Blueprints/GenericPuzzle/BP_PuzzleGoalElement` _array_element))
        (`/Game/Blueprints/GenericPuzzle/BP_PuzzleGoalElement.PuzzleSolved` _asbp_puzzle_goal_element)))
    (:`then_1`
      (for _array_element_2 (`self.PuzzleElements`)
        (bind _asbp_puzzle_element (cast `/Game/Blueprints/GenericPuzzle/BP_PuzzleElement` _array_element_2))
        (`/Game/Blueprints/GenericPuzzle/BP_PuzzleElement.Deactivate` _asbp_puzzle_element)))
    (:`then_2`
      (set `self.PuzzleSolved` true))))

(fn `UserConstructionScript`
  (`parent.UserConstructionScript`))