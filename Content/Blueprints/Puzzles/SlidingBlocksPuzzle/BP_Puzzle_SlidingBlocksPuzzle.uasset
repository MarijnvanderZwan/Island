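; Sliding block puzzle actor that lays out a Width by Depth grid of pushable and blocking blocks.
; The construction script builds the tile meshes centred on the actor and prints the top-left offset.
; BeginPlay registers blocks and obstacles, from their world positions, in a PuzzleGrid child actor.
; PushBlockInDirection converts a block's position to cell coordinates, delegates the push to that grid and returns the resulting world location.
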(event `self.ReceiveBeginPlay`
  (`self.InitializeGrid`)
  (`self.SetPuzzleForElements`))

(fn `CreateGrid`
  (bind _cellsize (`self.CellSize`))
  (bind _topleft (`self.GetTopLeft`))
  (for _index (range 1 (+ (`self.Depth`) 1))
    (for _index_2 (range 1 (+ (`self.Width`) 1))
      (`AddComponent|NODE_AddStaticMeshComponent-1` :`RelativeTransform` (`KismetMathLibrary.MakeTransform` (+ _topleft (`KismetMathLibrary.MakeVector` (* _index_2 _cellsize) (* _index _cellsize))))))))

(fn `GetGridLocationForBlock`
  (params (Location :type "Actor Object Reference"))
  (returns (GridLocation :type "Vector Structure"))
  (bind _cellsize (`self.CellSize`))
  (bind _topleft (`self.GetTopLeft`))
  (bind (_returnvalue_x _returnvalue_y) (`KismetMathLibrary.BreakVector` (- (- (`self.K2_GetActorLocation` Location) (+ _topleft (`self.K2_GetActorLocation`) (100.0 100.0 0.0))) (100.0 100.0 0.0))))
  (return (`KismetMathLibrary.MakeVector` (/ _returnvalue_x _cellsize) (/ _returnvalue_y _cellsize))))

(fn `GetPuzzleGrid`
  (returns (`Puzzle Grid` :type "PuzzleGrid Object Reference"))
  (bind _aspuzzle_grid (cast `PuzzleGrid` (`ChildActorComponent.ChildActor` (`self.PuzzleGrid`)))
    (:`then`
      _)
    (:`CastFailed`
      _))
  (return _aspuzzle_grid))

(fn `GetTopLeft`
  (returns (TopLeft :type "Vector Structure"))
  (bind _cellsize (`self.CellSize`))
  (return (`KismetMathLibrary.MakeVector` (* (+ (`KismetMathLibrary.Conv_IntToDouble` (`self.Width`)) 1.0) _cellsize -0.5) (* (+ (`KismetMathLibrary.Conv_IntToDouble` (`self.Depth`)) 1.0) _cellsize -0.5))))

(fn `GetWorldLocationForGridLocation`
  (params (GridLocation :type "Vector Structure"))
  (returns (WorldLocation :type "Vector Structure"))
  (bind _topleft (`self.GetTopLeft`))
  (return (+ (* (+ GridLocation (1.0 1.0 0.0)) (`self.CellSize`)) (`self.K2_GetActorLocation`) _topleft)))

(fn `InitializeGrid`
  (bind _puzzle_grid (`self.GetPuzzleGrid`))
  (`PuzzleGrid.InitializeWithSize` _puzzle_grid (`self.Width`) (`self.Depth`))
  (bind _filteredarray (`KismetArrayLibrary.FilterArray` (`self.InteractivePuzzleElements`) "/Game/Blueprints/Puzzles/SlidingBlocksPuzzle/BP_PuzzleElement_PushableBLock.BP_PuzzleElement_PushableBlock_C"))
  (for _array_element _filteredarray
    (bind _gridlocation (`self.GetGridLocationForBlock` _array_element))
    (bind _puzzle_grid_2 (`self.GetPuzzleGrid`))
    (`PuzzleGrid.AddPushableBlock` _puzzle_grid_2 (`KismetMathLibrary.FTrunc` (.x _gridlocation)) (`KismetMathLibrary.FTrunc` (.y _gridlocation))))
  (bind _filteredarray_2 (`KismetArrayLibrary.FilterArray` (`self.PuzzleElements`) "/Game/Blueprints/Puzzles/SlidingBlocksPuzzle/BP_PuzzleElement_BlockingBlock.BP_PuzzleElement_BlockingBlock_C"))
  (for _array_element_2 _filteredarray_2
    (bind _gridlocation_2 (`self.GetGridLocationForBlock` _array_element_2))
    (bind _puzzle_grid_3 (`self.GetPuzzleGrid`))
    (`PuzzleGrid.AddObstacle` _puzzle_grid_3 (`KismetMathLibrary.FTrunc` (.x _gridlocation_2)) (`KismetMathLibrary.FTrunc` (.y _gridlocation_2)))))

(fn `PushBlockInDirection`
  (params (Actor :type "Actor Object Reference") (Direction :type "Vector Structure"))
  (returns (EndLocation :type "Vector Structure"))
  (bind _puzzle_grid (`self.GetPuzzleGrid`))
  (bind _gridlocation (`self.GetGridLocationForBlock` Actor))
  (bind _returnvalue (`PuzzleGrid.PushBlockInDirection` _puzzle_grid (`KismetMathLibrary.FTrunc` (.x _gridlocation)) (`KismetMathLibrary.FTrunc` (.y _gridlocation)) (`KismetMathLibrary.FTrunc` Direction_X) (`KismetMathLibrary.FTrunc` Direction_Y)))
  (bind _worldlocation (`self.GetWorldLocationForGridLocation` _returnvalue))
  (return _worldlocation))

(fn `UserConstructionScript`
  (`self.CreateGrid`)
  (bind _topleft (`self.GetTopLeft`))
  (`KismetSystemLibrary.PrintString` (`KismetStringLibrary.Conv_VectorToString` _topleft)))