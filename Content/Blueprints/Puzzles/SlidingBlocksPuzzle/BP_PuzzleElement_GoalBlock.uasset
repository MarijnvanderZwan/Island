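; BP_PuzzleElement_GoalBlock is a goal element for the sliding blocks puzzle that detects when a pushable block rests on it.
; When its Box begins overlapping a BP_PuzzleElement_PushableBlock while inactive, it sets Active and switches that block's mesh to the lit blue rune material.
; An end overlap by a pushable block while active clears the flag and applies the unlit rune material.
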(event `self.ReceiveBeginPlay`)

(event `self.ReceiveTick`
  (params (DeltaSeconds :type "Float (single-precision)")))

(event `self.Box.OnComponentBeginOverlap`
  (params (OverlappedComponent :type "PrimitiveComponent Object Reference") (OtherActor :type "Actor Object Reference") (OtherComp :type "PrimitiveComponent Object Reference") (OtherBodyIndex :type Integer) (bFromSweep :type Boolean) (SweepResult :type "HitResult Structure (by ref)"))
  (if (not (`self.Active`))
    (bind _asbp_puzzle_element_pushable_block (cast `/Game/Blueprints/Puzzles/SlidingBlocksPuzzle/BP_PuzzleElement_PushableBLock` OtherActor))
    (set `self.Active` true)
    (`PrimitiveComponent.SetMaterial` (`/Game/Blueprints/Puzzles/SlidingBlocksPuzzle/BP_PuzzleElement_PushableBLock.Mesh` _asbp_puzzle_element_pushable_block) 0 "/Game/Materials/M_BlockBlueRune.M_BlockBlueRune")))

(event `self.Box.OnComponentEndOverlap`
  (params (OverlappedComponent :type "PrimitiveComponent Object Reference") (OtherActor :type "Actor Object Reference") (OtherComp :type "PrimitiveComponent Object Reference") (OtherBodyIndex :type Integer))
  (if (`self.Active`)
    (bind _asbp_puzzle_element_pushable_block (cast `/Game/Blueprints/Puzzles/SlidingBlocksPuzzle/BP_PuzzleElement_PushableBLock` OtherActor))
    (set `self.Active` false)
    (`PrimitiveComponent.SetMaterial` (`/Game/Blueprints/Puzzles/SlidingBlocksPuzzle/BP_PuzzleElement_PushableBLock.Mesh` _asbp_puzzle_element_pushable_block) 0 "/Game/Materials/M_BlockBlueRune_off.M_BlockBlueRune_off")))

(fn `UserConstructionScript`)