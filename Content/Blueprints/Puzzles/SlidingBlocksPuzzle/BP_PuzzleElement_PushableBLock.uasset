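; Pushable block element for the sliding blocks puzzle that slides away from the side it is pushed from.
; Push finds the nearest of four side colliders, inverts the sign of its relative offset, and asks the owning puzzle for the destination.
; Tick moves the block there at constant speed, snaps it when close, and re-enables pushing.
; A reset function teleports it back to its starting position.
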(event `self.ReceiveBeginPlay`
  (bind _returnvalue (`self.K2_GetActorLocation`))
  (set `self.StartingPosition` _returnvalue)
  (set `self.EndLocation` _returnvalue)
  (`self.AddColliders`))

(event `self.ReceiveTick`
  (params (DeltaSeconds :type "Float (single-precision)"))
  (bind _endlocation (`self.EndLocation`))
  (bind _returnvalue (`SceneComponent.K2_GetComponentLocation` (`self.Mesh`)))
  (bind _returnvalue_2 (- _endlocation _returnvalue))
  (if (`self.Pushable`)
    _
    (elif (<= (`KismetMathLibrary.VSize` _returnvalue_2) 10.0)
      (`self.K2_SetActorLocation` _endlocation)
      (set `self.Pushable` true)
      (else
        (`self.K2_SetActorLocation` (+ (* (`KismetMathLibrary.Normal` _returnvalue_2) (* DeltaSeconds (`self.MovementSpeed`))) _returnvalue))))))

(fn `AddColliders`
  (bind _colliders (`self.Colliders`))
  (`KismetArrayLibrary.Array_Add` _colliders (`self.South`))
  (`KismetArrayLibrary.Array_Add` _colliders (`self.North`))
  (`KismetArrayLibrary.Array_Add` _colliders (`self.West`))
  (`KismetArrayLibrary.Array_Add` _colliders (`self.East`)))

(fn `GetClosestCollider`
  (params (Location :type "Vector Structure"))
  (returns (Collider :type "BoxComponent Object Reference"))
  (locals (minDistance :type "Float (double-precision)" :default 5000.0) (minCollider :type "BoxComponent Object Reference"))
  (for _array_element (`self.Colliders`)
    (bind (_outpointonbody _returnvalue) (`PrimitiveComponent.GetClosestPointOnCollision` _array_element Location "None"))
    (if (< _returnvalue (`local.minDistance`))
      (set `local.minDistance` _returnvalue)
      (set `local.minCollider` _array_element)))
  (return (`local.minCollider`)))

(fn `Push`
  (params (FromLocation :type "Vector Structure"))
  (bind (_returnvalue_x _returnvalue_y _returnvalue_z) (`KismetMathLibrary.BreakVector` (`self.K2_GetActorLocation`)))
  (if (`self.Pushable`)
    (bind _collider (`self.GetClosestCollider` FromLocation))
    (bind _asbp_puzzle_sliding_blocks_puzzle (cast `/Game/Blueprints/Puzzles/SlidingBlocksPuzzle/BP_Puzzle_SlidingBlocksPuzzle` (`self.Puzzle`)))
    (bind (_relativelocation_x _relativelocation_y) (`KismetMathLibrary.BreakVector` (`SceneComponent.RelativeLocation` _collider)))
    (bind _endlocation (`/Game/Blueprints/Puzzles/SlidingBlocksPuzzle/BP_Puzzle_SlidingBlocksPuzzle.PushBlockInDirection` _asbp_puzzle_sliding_blocks_puzzle self (`KismetMathLibrary.MakeVector` (* (`KismetMathLibrary.SignOfFloat` _relativelocation_x) -1.0) (* (`KismetMathLibrary.SignOfFloat` _relativelocation_y) -1.0))))
    (set `self.EndLocation` (`KismetMathLibrary.MakeVector` (.x _endlocation) (.y _endlocation) _returnvalue_z))
    (set `self.Pushable` false)))

(fn `ResetToStartingLocation`
  (`self.K2_SetActorLocation` (`self.StartingPosition`) false true)
  (set `self.Direction` (0.0 0.0 0.0)))

(fn `UserConstructionScript`)