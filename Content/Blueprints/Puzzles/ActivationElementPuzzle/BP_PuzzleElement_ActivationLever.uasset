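; BP_PuzzleElement_ActivationLever is an interactable lever element for the activation element puzzle, switching between up and down states.
; Interacting calls Activate, which toggles the Activated flag and plays the matching non-looping Lever_Up or Lever_Down animation on Lever2.
; Deactivate reuses the raise branch, always playing Lever_Up and clearing the flag regardless of current state.
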(event `self.Activate`
  (bind _lever2 (`self.Lever2`))
  (if (`self.Activated`)
    (`SkeletalMeshComponent.PlayAnimation` _lever2 "/Game/Animations/lever_Up.lever_Up" false :!label _label)
    (set `self.Activated` false)
    (else
      (`SkeletalMeshComponent.PlayAnimation` _lever2 "/Game/Animations/lever_Down.lever_Down" false)
      (set `self.Activated` true))))

(event `self.Deactivate`
  (goto _label))

(event `/Game/Blueprints/Gameplay/InteractableObject.InteractWithObject`
  (params (TriggerLocation :type "Vector Structure"))
  (`self.Activate`))

(fn `UserConstructionScript`
  (`parent.UserConstructionScript`))