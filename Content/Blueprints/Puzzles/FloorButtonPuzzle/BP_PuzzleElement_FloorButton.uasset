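; BP_PuzzleElement_FloorButton is a timed floor button that serves as one element of a floor-button puzzle.
; A player overlapping its box activates it when inactive, swapping material and playing a click; stepping on it in any other state resets the owning puzzle.
; Tick counts down the active time and deactivates the button on expiry, and both countdown and overlap stop once solved.
; SetVariables supplies the duration and both materials.
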(event `Activate`
  (set `self.FloorButtonState` "NewEnumerator2")
  (set `self.RemainingTimeActive` (`self.TimeEnabled`))
  (`PrimitiveComponent.SetMaterial` (`self.StaticMesh`) 1 (`self.EnabledMaterial`))
  (`GameplayStatics.PlaySoundAtLocation` "/Game/Audio/Effect/SubtleClickSound.SubtleClickSound" (`self.K2_GetActorLocation`)))

(event `Deactivate`
  (set `self.FloorButtonState` "NewEnumerator0")
  (`PrimitiveComponent.SetMaterial` (`self.StaticMesh`) 1 (`self.DisabledMaterial`))
  (set `self.RemainingTimeActive` 0.0))

(event `self.ReceiveTick`
  (params (DeltaSeconds :type "Float (single-precision)"))
  (if (and (`|EnumEquality` (`self.FloorButtonState`) "NewEnumerator2") (not (`self.PuzzleSolved`)))
    (bind _output_get (set `self.RemainingTimeActive` (- (`self.RemainingTimeActive`) DeltaSeconds)))
    (if (< _output_get 0.0)
      (`self.Deactivate`))))

(event `self.Box.OnComponentBeginOverlap`
  (params (OverlappedComponent :type "PrimitiveComponent Object Reference") (OtherActor :type "Actor Object Reference") (OtherComp :type "PrimitiveComponent Object Reference") (OtherBodyIndex :type Integer) (bFromSweep :type Boolean) (SweepResult :type "HitResult Structure (by ref)"))
  (if (not (`self.PuzzleSolved`))
    (cast `/Game/Blueprints/BP_Player` OtherActor)
    (if (`|EnumEquality` (`self.FloorButtonState`) "NewEnumerator0")
      (`self.Activate`)
      (else
        (`/Game/Blueprints/GenericPuzzle/BP_Puzzle.Reset Puzzle` (`self.Puzzle`))))))

(fn `SetVariables`
  (params (TimeEnabled :type "Float (double-precision)") (EnabledMaterial :type "Material Object Reference") (DisabledMaterial :type "Material Object Reference"))
  (set `self.TimeEnabled` TimeEnabled)
  (set `self.EnabledMaterial` EnabledMaterial)
  (set `self.DisabledMaterial` DisabledMaterial))

(fn `UserConstructionScript`)