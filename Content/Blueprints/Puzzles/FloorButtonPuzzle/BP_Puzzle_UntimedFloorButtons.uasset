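; Floor button puzzle controller that sets up untimed button elements and can block player jumping inside its area until the puzzle is solved.
; On BeginPlay it passes shared materials and a zero enabled time to each button in PuzzleElements.
; The JumpingCollisionDisabled overlap toggles BP_Player's JumpMaxCount when that option is on.
; PuzzleIsSolved restores jumping, notifies PuzzleGoalElements and marks every button solved.
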(event `self.ReceiveBeginPlay`
  (for _array_element (`self.PuzzleElements`)
    (bind _asbp_puzzle_element_floor_button_untimed (cast `/Game/Blueprints/Puzzles/FloorButtonPuzzle/BP_PuzzleElement_FloorButtonUntimed` _array_element))
    (`/Game/Blueprints/Puzzles/FloorButtonPuzzle/BP_PuzzleElement_FloorButton.SetVariables` _asbp_puzzle_element_floor_button_untimed 0.0 (`self.EnabledMaterial`) (`self.DisabledMaterial`))))

(event `self.PuzzleIsSolved`
  (set `self.PuzzleSolved` true)
  (bind _outactors (`GameplayStatics.GetAllActorsOfClass` "/Game/Blueprints/BP_Player.BP_Player_C"))
  (set `Character.JumpMaxCount` 1 (`|GetArrayItem` _outactors))
  (for _array_element (`self.PuzzleGoalElements`)
    (`/Game/Blueprints/GenericPuzzle/BP_PuzzleGoalElement.PuzzleSolved` _array_element))
  (for _array_element_2 (`self.PuzzleElements`)
    (bind _asbp_puzzle_element_floor_button_untimed (cast `/Game/Blueprints/Puzzles/FloorButtonPuzzle/BP_PuzzleElement_FloorButtonUntimed` _array_element_2))
    (set `/Game/Blueprints/Puzzles/FloorButtonPuzzle/BP_PuzzleElement_FloorButton.PuzzleSolved` true _asbp_puzzle_element_floor_button_untimed)))

(event `self.JumpingCollisionDisabled.OnComponentBeginOverlap`
  (params (OverlappedComponent :type "PrimitiveComponent Object Reference") (OtherActor :type "Actor Object Reference") (OtherComp :type "PrimitiveComponent Object Reference") (OtherBodyIndex :type Integer) (bFromSweep :type Boolean) (SweepResult :type "HitResult Structure (by ref)"))
  (if (`self.JumpingDuringPuzzleDisabled`)
    (if (not (`self.PuzzleSolved`))
      (bind _asbp_player (cast `/Game/Blueprints/BP_Player` OtherActor))
      (set `Character.JumpMaxCount` 0 _asbp_player))))

(event `self.JumpingCollisionDisabled.OnComponentEndOverlap`
  (params (OverlappedComponent :type "PrimitiveComponent Object Reference") (OtherActor :type "Actor Object Reference") (OtherComp :type "PrimitiveComponent Object Reference") (OtherBodyIndex :type Integer))
  (if (`self.JumpingDuringPuzzleDisabled`)
    (if (not (`self.PuzzleSolved`))
      (bind _asbp_player (cast `/Game/Blueprints/BP_Player` OtherActor))
      (set `Character.JumpMaxCount` 1 _asbp_player))))

(fn `UserConstructionScript`
  (`parent.UserConstructionScript`))