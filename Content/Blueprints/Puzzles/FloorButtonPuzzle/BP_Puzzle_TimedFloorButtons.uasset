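; Timed floor button puzzle that gives each linked button its enabled duration and materials on BeginPlay.
; An optional trigger volume disables the player's jump while the puzzle is unsolved.
; Any end overlap on that volume resets the puzzle, deactivating the buttons and resetting the InteractionTimeManager.
; Solving, signalled through the parent puzzle's event, restores jumping and marks every button as solved.
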(event `self.ReceiveBeginPlay`
  (`parent.ReceiveBeginPlay`)
  (for _array_element (`self.PuzzleElements`)
    (set `/Game/Blueprints/GenericPuzzle/BP_PuzzleElement.Puzzle` self _array_element)
    (bind _asbp_puzzle_element_floor_button (cast `/Game/Blueprints/Puzzles/FloorButtonPuzzle/BP_PuzzleElement_FloorButton` _array_element))
    (`/Game/Blueprints/Puzzles/FloorButtonPuzzle/BP_PuzzleElement_FloorButton.SetVariables` _asbp_puzzle_element_floor_button (`self.FloorButtonsTimeEnabled`) (`self.EnabledMaterial`) (`self.DisabledMaterial`))))

(event `self.PuzzleIsSolved`
  (`parent.PuzzleIsSolved`)
  (bind _outactors (`GameplayStatics.GetAllActorsOfClass` "/Game/Blueprints/BP_Player.BP_Player_C"))
  (set `Character.JumpMaxCount` 1 (`|GetArrayItem` _outactors))
  (for _array_element (`self.PuzzleElements`)
    (bind _asbp_puzzle_element_floor_button (cast `/Game/Blueprints/Puzzles/FloorButtonPuzzle/BP_PuzzleElement_FloorButton` _array_element))
    (set `/Game/Blueprints/Puzzles/FloorButtonPuzzle/BP_PuzzleElement_FloorButton.PuzzleSolved` true _asbp_puzzle_element_floor_button)))

(event `self.JumpingCollisionDisabled.OnComponentBeginOverlap`
  (params (OverlappedComponent :type "PrimitiveComponent Object Reference") (OtherActor :type "Actor Object Reference") (OtherComp :type "PrimitiveComponent Object Reference") (OtherBodyIndex :type Integer) (bFromSweep :type Boolean) (SweepResult :type "HitResult Structure (by ref)"))
  (if (`self.JumpingDuringPuzzleDisabled`)
    (if (not (`self.PuzzleSolved`))
      (bind _asbp_player (cast `/Game/Blueprints/BP_Player` OtherActor))
      (set `Character.JumpMaxCount` 0 _asbp_player))))

(event `self.JumpingCollisionDisabled.OnComponentEndOverlap`
  (params (OverlappedComponent :type "PrimitiveComponent Object Reference") (OtherActor :type "Actor Object Reference") (OtherComp :type "PrimitiveComponent Object Reference") (OtherBodyIndex :type Integer))
  (`self.Reset Puzzle`)
  (if (`self.JumpingDuringPuzzleDisabled`)
    (if (not (`self.PuzzleSolved`))
      (bind _asbp_player (cast `/Game/Blueprints/BP_Player` OtherActor))
      (set `Character.JumpMaxCount` 1 _asbp_player))))

(event `self.Reset Puzzle`
  (bind _filteredarray (`KismetArrayLibrary.FilterArray` (`self.PuzzleElements`) "/Game/Blueprints/Puzzles/FloorButtonPuzzle/BP_PuzzleElement_FloorButton.BP_PuzzleElement_FloorButton_C"))
  (for _array_element _filteredarray
    (bind _asbp_puzzle_element_floor_button (cast `/Game/Blueprints/Puzzles/FloorButtonPuzzle/BP_PuzzleElement_FloorButton` _array_element))
    (`/Game/Blueprints/Puzzles/FloorButtonPuzzle/BP_PuzzleElement_FloorButton.Deactivate` _asbp_puzzle_element_floor_button)
    (bind _outactors (`GameplayStatics.GetAllActorsOfClass` "/Game/Blueprints/InteractionTimeManager.InteractionTimeManager_C"))
    (`/Game/Blueprints/InteractionTimeManager.ResetTime` (`|GetArrayItem` _outactors))))

(fn `UserConstructionScript`
  (`parent.UserConstructionScript`))