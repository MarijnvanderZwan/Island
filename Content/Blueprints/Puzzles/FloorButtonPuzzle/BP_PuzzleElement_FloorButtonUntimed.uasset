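; An untimed floor button puzzle element that toggles on or off when the player steps on it.
; A box overlap from BP_Player flips the button between two enum states, unless the puzzle is already solved.
; Activate and Deactivate set the state, swap the mesh's material between enabled and disabled, and play a subtle click sound at the button.
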(event `Activate`
  (`KismetSystemLibrary.PrintString` "activate")
  (set `self.FloorButtonState` "NewEnumerator2")
  (`PrimitiveComponent.SetMaterial` (`self.StaticMesh`) 1 (`self.EnabledMaterial`))
  (`GameplayStatics.PlaySoundAtLocation` "/Game/Audio/Effect/SubtleClickSound.SubtleClickSound" (`self.K2_GetActorLocation`)))

(event `Deactivate`
  (`KismetSystemLibrary.PrintString` "deactivate")
  (set `self.FloorButtonState` "NewEnumerator0")
  (`PrimitiveComponent.SetMaterial` (`self.StaticMesh`) 1 (`self.DisabledMaterial`))
  (`GameplayStatics.PlaySoundAtLocation` "/Game/Audio/Effect/SubtleClickSound.SubtleClickSound" (`self.K2_GetActorLocation`)))

(event `self.ReceiveTick`
  (params (DeltaSeconds :type "Float (single-precision)")))

(event `self.Box.OnComponentBeginOverlap`
  (params (OverlappedComponent :type "PrimitiveComponent Object Reference") (OtherActor :type "Actor Object Reference") (OtherComp :type "PrimitiveComponent Object Reference") (OtherBodyIndex :type Integer) (bFromSweep :type Boolean) (SweepResult :type "HitResult Structure (by ref)"))
  (cast `/Game/Blueprints/BP_Player` OtherActor)
  (if (`self.PuzzleSolved`)
    _
    (elif (`|EnumEquality` (`self.FloorButtonState`) "NewEnumerator0")
      (`self.Activate`)
      (else
        (`self.Deactivate`)))))

(fn `UserConstructionScript`
  (`parent.UserConstructionScript`))