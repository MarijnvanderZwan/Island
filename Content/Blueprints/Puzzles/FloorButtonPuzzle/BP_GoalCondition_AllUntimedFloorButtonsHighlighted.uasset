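; Goal condition for floor button puzzles that counts as solved when all of the puzzle's untimed floor buttons are highlighted.
; CheckSolved filters the owning Puzzle's elements to untimed floor buttons and returns false as soon as any is in the first button-state enum value.
; It also returns false when the puzzle has no untimed buttons, so an empty set never counts as solved.
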(fn `CheckSolved`
  (returns (Solved :type Boolean))
  (bind _filteredarray (`KismetArrayLibrary.FilterArray` (`/Game/Blueprints/GenericPuzzle/BP_Puzzle.PuzzleElements` (`self.Puzzle`)) "/Game/Blueprints/Puzzles/FloorButtonPuzzle/BP_PuzzleElement_FloorButtonUntimed.BP_PuzzleElement_FloorButtonUntimed_C"))
  (if (> (`KismetArrayLibrary.Array_Length` _filteredarray) 0)
    (for _array_element _filteredarray
      (bind _asbp_puzzle_element_floor_button_untimed (cast `/Game/Blueprints/Puzzles/FloorButtonPuzzle/BP_PuzzleElement_FloorButtonUntimed` _array_element))
      (if (`|EnumEquality` (`/Game/Blueprints/Puzzles/FloorButtonPuzzle/BP_PuzzleElement_FloorButton.FloorButtonState` _asbp_puzzle_element_floor_button_untimed) "NewEnumerator0")
        (return false)))
    (return true)
    (else
      (return false))))

(fn `UserConstructionScript`
  (`parent.UserConstructionScript`))