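; Player controller that owns the pause menu and handles pausing, restarting and quitting the game.
; On BeginPlay it finds the GlobalPuzzleHandler, creates the UI_PauseMenu widget with a reference to itself, and immediately toggles pause.
; Tab toggles pause, syncing menu visibility, game pause and the puzzle handler, while Up, Down and Enter drive menu selection.
; New Game, Continue and Exit events restart the level, toggle pause or quit.
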(event `self.ReceiveBeginPlay`
  (bind _outactors (`GameplayStatics.GetAllActorsOfClass` "/Game/Blueprints/GlobalPuzzleHandler.GlobalPuzzleHandler_C"))
  (set `self.GlobalPuzzleHandler` (`|GetArrayItem` _outactors))
  (bind _returnvalue (`|CreateWidget` "/Game/Blueprints/UI/PauseMenu/UI_PauseMenu.UI_PauseMenu_C"))
  (bind _output_get (set `self.PauseMenu` _returnvalue))
  (`UserWidget.AddToViewport` _output_get 0)
  (set `/Game/Blueprints/UI/PauseMenu/UI_PauseMenu.PlayerController` self _output_get)
  (`self.PauseButtonPressed`))

(event `Key|Tab` :paused true
  (params (Key :type "Key Structure"))
  (:`Pressed`
    (`self.PauseButtonPressed`)))

(event `Key|Down` :paused true
  (params (Key :type "Key Structure"))
  (:`Pressed`
    (`/Game/Blueprints/UI/PauseMenu/UI_PauseMenu.SelectNextMenuItem` (`self.PauseMenu`))))

(event `Key|Up` :paused true
  (params (Key :type "Key Structure"))
  (:`Pressed`
    (`/Game/Blueprints/UI/PauseMenu/UI_PauseMenu.SelectPreviousMenuItem` (`self.PauseMenu`))))

(event `Key|Enter` :paused true
  (params (Key :type "Key Structure"))
  (:`Pressed`
    (`/Game/Blueprints/UI/PauseMenu/UI_PauseMenu.ConfirmSelectedMenuItem` (`self.PauseMenu`))))

(event `PauseButtonPressed`
  (bind _globalpuzzlehandler (`self.GlobalPuzzleHandler`))
  (bind _pausemenu (`self.PauseMenu`))
  (bind _output_get (set `self.Paused` (not (`self.Paused`))))
  (if _output_get
    (`Widget.SetVisibility` _pausemenu "Visible")
    (`GameplayStatics.SetGamePaused` true)
    (`/Game/Blueprints/GlobalPuzzleHandler.GamePaused` _globalpuzzlehandler true)
    (else
      (`Widget.SetVisibility` _pausemenu "Hidden")
      (`GameplayStatics.SetGamePaused` false)
      (`/Game/Blueprints/GlobalPuzzleHandler.GamePaused` _globalpuzzlehandler false))))

(event `NewGameEvent`
  (`KismetSystemLibrary.ExecuteConsoleCommand` "RestartLevel" null))

(event `ContinueGameEvent`
  (`self.PauseButtonPressed`))

(event `ExitGameEvent`
  (`KismetSystemLibrary.QuitGame` null "Quit"))

(fn `UserConstructionScript`)