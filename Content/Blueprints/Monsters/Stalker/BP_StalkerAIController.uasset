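; AI controller for the Stalker monster that points its behavior tree at the player.
; On BeginPlay it loads StalkerBlackboard and writes TargetToFollow twice, first as the pawn's location vector, then as the first BP_Player actor found in the level.
; It then runs StalkerTree, with no per-frame logic in the controller.
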(event `self.ReceiveBeginPlay`
  (bind _returnvalue (`AIBlueprintHelperLibrary.GetBlackboard` self))
  (`self.UseBlackboard` "/Game/Blueprints/Monsters/Stalker/StalkerBlackboard.StalkerBlackboard")
  (`BlackboardComponent.SetValueAsVector` _returnvalue (`self.TargetToFollow`) (`self.K2_GetActorLocation` (`self.K2_GetPawn`)))
  (bind _outactors (`GameplayStatics.GetAllActorsOfClass` "/Game/Blueprints/BP_Player.BP_Player_C"))
  (`BlackboardComponent.SetValueAsObject` _returnvalue (`self.TargetToFollow`) (`|GetArrayItem` _outactors))
  (`self.RunBehaviorTree` "/Game/Blueprints/Monsters/Stalker/StalkerTree.StalkerTree"))

(fn `UserConstructionScript`)