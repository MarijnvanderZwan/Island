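; Dialogue trigger actor that shows its configured message when something begins overlapping its sphere.
; The overlap finds the first BP_DialogueSystem in the level through GetAllActorsOfClass and passes it the message.
; It then either destroys itself, or disables its collision and re-enables it by timer after a cooldown, so the message can repeat.
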(event `self.Sphere1.OnComponentBeginOverlap`
  (params (OverlappedComponent :type "PrimitiveComponent Object Reference") (OtherActor :type "Actor Object Reference") (OtherComp :type "PrimitiveComponent Object Reference") (OtherBodyIndex :type Integer) (bFromSweep :type Boolean) (SweepResult :type "HitResult Structure (by ref)"))
  (bind _outactors (`GameplayStatics.GetAllActorsOfClass` "/Game/Blueprints/BP_DialogueSystem.BP_DialogueSystem_C"))
  (`/Game/Blueprints/BP_DialogueSystem.ShowMessage` (`KismetArrayLibrary.Array_Get` _outactors) (`self.Message`))
  (if (`self.DestroyAfterMessage`)
    (`self.K2_DestroyActor`)
    (else
      (`self.SetActorEnableCollision` false)
      (`KismetSystemLibrary.K2_SetTimerDelegate` (delegate `Reset`) (`self.Cooldown`)))))

(event `Reset`
  (`self.SetActorEnableCollision` true))

(fn `UserConstructionScript`)