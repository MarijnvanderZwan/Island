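; BP_DialogueSystem is an actor that shows and dismisses a single on-screen message box for dialogue or notices.
; On BeginPlay it creates a UI_Message widget, adds it to the viewport and keeps it hidden.
; ShowMessage passes text to the widget and flags it visible, and pressing the Action input hides it while that flag is set.
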(event `self.ReceiveBeginPlay`
  (bind _returnvalue (`|CreateWidget` "/Game/Blueprints/UI_Message.UI_Message_C"))
  (`UserWidget.AddToViewport` _returnvalue 0)
  (bind _output_get (set `self.MessageBox` _returnvalue))
  (`/Game/Blueprints/UI_Message.Hide` _output_get)
  (set `self.MessageVisible` false))

(event `InputAction|Action` :consume false
  (params (Key :type "Key Structure" :default "AnyKey"))
  (:`Pressed`
    (if (`self.MessageVisible`)
      (`/Game/Blueprints/UI_Message.Hide` (`self.MessageBox`))
      (set `self.MessageVisible` false))))

(fn `ShowMessage`
  (params (Message :type String))
  (`/Game/Blueprints/UI_Message.ShowWithMessage` (`self.MessageBox`) Message)
  (set `self.MessageVisible` true))

(fn `UserConstructionScript`)