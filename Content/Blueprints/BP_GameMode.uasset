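; Game mode for an island puzzle game that handles saving and loading of puzzle progress and initializes the player controller and player interface on BeginPlay.
; SaveGame copies completed puzzles, coins and completion percentage from GlobalPuzzleHandler into an IslandSaveGame in a fixed slot.
; LoadGame reopens Map_Island with slot and user index in the options string.
; BeginPlay parses that string and restores the saved state to the handler before initialization.
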(event `self.ReceiveBeginPlay`
  (bind _optionsstring (`self.OptionsString`))
  (bind _returnvalue (`KismetStringLibrary.Len` _optionsstring))
  (bind (_lefts _rights) (`KismetStringLibrary.Split` (`KismetStringLibrary.GetSubstring` _optionsstring 1 _returnvalue) "|"))
  (`|ExecutionSequence`
    (:`then_0`
      (if (> _returnvalue 0)
        (bind _returnvalue_2 (`GameplayStatics.LoadGameFromSlot` _lefts (`KismetStringLibrary.Conv_StringToInt` _rights)))
        (bind _asisland_save_game (cast `/Game/Blueprints/Saving/IslandSaveGame` _returnvalue_2))
        (bind _outactors (`GameplayStatics.GetAllActorsOfClass` "/Game/Blueprints/GlobalPuzzleHandler.GlobalPuzzleHandler_C"))
        (bind _output (`|GetArrayItem` _outactors))
        (`/Game/Blueprints/GlobalPuzzleHandler.SetPuzzlesCompleted` _output (`/Game/Blueprints/Saving/IslandSaveGame.CompletedPuzzles` _asisland_save_game))
        (`/Game/Blueprints/GlobalPuzzleHandler.SetCoinsCollected` _output (`/Game/Blueprints/Saving/IslandSaveGame.CollectedCoins` _asisland_save_game))))
    (:`then_1`
      (bind _outactors_2 (`GameplayStatics.GetAllActorsOfClass` "/Game/Blueprints/BP_PlayerController.BP_PlayerController_C"))
      (`/Game/Blueprints/BP_PlayerController.Initialize` (`|GetArrayItem` _outactors_2)))
    (:`then_2`
      (bind _outactors_3 (`GameplayStatics.GetAllActorsOfClass` "/Game/Blueprints/BP_Player.BP_Player_C"))
      (`/Game/Blueprints/BP_Player.InitializeInterface` (`|GetArrayItem` _outactors_3)))))

(event `Save Game`
  (bind _outactors (`GameplayStatics.GetAllActorsOfClass` "/Game/Blueprints/GlobalPuzzleHandler.GlobalPuzzleHandler_C"))
  (bind _returnvalue (`GameplayStatics.CreateSaveGameObject` "/Game/Blueprints/Saving/IslandSaveGame.IslandSaveGame_C"))
  (`|ExecutionSequence`
    (:`then_0`
      (set `/Game/Blueprints/Saving/IslandSaveGame.SaveSlotName` "Slot0" _returnvalue))
    (:`then_1`
      (set `/Game/Blueprints/Saving/IslandSaveGame.UserIndex` 0 _returnvalue))
    (:`then_2`
      (bind _output (`|GetArrayItem` _outactors))
      (set `/Game/Blueprints/Saving/IslandSaveGame.CompletedPuzzles` (`/Game/Blueprints/GlobalPuzzleHandler.PuzzlesCompleted` _output) _returnvalue))
    (:`then_3`
      (set `/Game/Blueprints/Saving/IslandSaveGame.CollectedCoins` (`/Game/Blueprints/GlobalPuzzleHandler.CoinsCollected` _output) _returnvalue))
    (:`then_4`
      (bind _completionpercentage (`/Game/Blueprints/GlobalPuzzleHandler.ComputeCompletionPercentage` _output))
      (bind _output_get (set `/Game/Blueprints/Saving/IslandSaveGame.CompletionPercentage` _completionpercentage _returnvalue))
      (`KismetSystemLibrary.PrintString` (`KismetStringLibrary.Conv_DoubleToString` _output_get)))
    (:`then_5`
      (`GameplayStatics.SaveGameToSlot` _returnvalue (`/Game/Blueprints/Saving/IslandSaveGame.SaveSlotName` _returnvalue) (`/Game/Blueprints/Saving/IslandSaveGame.UserIndex` _returnvalue))
      (`KismetSystemLibrary.PrintString` "Saved Game"))))

(event `Load Game`
  (`GameplayStatics.OpenLevel` "Map_Island" false "Slot0|0"))

(fn `UserConstructionScript`)