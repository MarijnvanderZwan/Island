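; Gate goal element for the timed tile puzzle that opens when the puzzle is solved.
; PuzzleSolved calls SetGateDown, which plays the gate animation once and disables collision.
; SetGateUp restores physics-only collision and plays the same Gate_Anim forward, with no reversed playback; nothing in this Blueprint calls it.
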(event `self.PuzzleSolved`
  (`self.SetGateDown`))

(event `SetGateUp`
  (`SkeletalMeshComponent.PlayAnimation` (`self.SkeletalMesh`) "/Game/Meshes/Arnimated/Gate_Anim.Gate_Anim" false)
  (`PrimitiveComponent.SetCollisionEnabled` (`self.Collision`) "PhysicsOnly"))

(event `SetGateDown`
  (`SkeletalMeshComponent.PlayAnimation` (`self.SkeletalMesh`) "/Game/Meshes/Arnimated/Gate_Anim.Gate_Anim" false)
  (`PrimitiveComponent.SetCollisionEnabled` (`self.Collision`) "NoCollision"))

(fn `UserConstructionScript`
  (`parent.UserConstructionScript`))