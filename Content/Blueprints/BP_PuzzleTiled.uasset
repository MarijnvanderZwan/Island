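; BP_PuzzleTiled is an actor that lays out a tiled grid of static meshes, with no runtime logic.
; The construction script calls CreateGrid, which loops over Width and Depth and adds a static mesh component per cell, spaced by CellSize.
; GetTopLeft offsets the one-based loop indices so the grid is centered on the actor's origin.
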(fn `CreateGrid`
  (bind _cellsize (`self.CellSize`))
  (bind _topleft (`self.GetTopLeft`))
  (for _index (range 1 (+ (`self.Depth`) 1))
    (for _index_2 (range 1 (+ (`self.Width`) 1))
      (`AddComponent|NODE_AddStaticMeshComponent-0` :`RelativeTransform` (`KismetMathLibrary.MakeTransform` (+ _topleft (`KismetMathLibrary.MakeVector` (* _index_2 _cellsize) (* _index _cellsize))))))))

(fn `GetTopLeft`
  (returns (TopLeft :type "Vector Structure"))
  (bind _cellsize (`self.CellSize`))
  (return (`KismetMathLibrary.MakeVector` (* (+ (`KismetMathLibrary.Conv_IntToDouble` (`self.Width`)) 1.0) _cellsize -0.5) (* (+ (`KismetMathLibrary.Conv_IntToDouble` (`self.Depth`)) 1.0) _cellsize -0.5))))

(fn `UserConstructionScript`
  (`self.CreateGrid`))