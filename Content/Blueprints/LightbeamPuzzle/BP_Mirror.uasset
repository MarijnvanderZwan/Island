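; BP_Mirror is a mirror actor for the lightbeam puzzle that turns around its yaw axis.
; RotateClockwise, RotateCounterClockwise and StopRotation events set a signed Rotation speed in degrees per second, or zero it.
; Tick adds that speed, scaled by DeltaSeconds, to the actor's yaw while preserving pitch and roll.
; The Blueprint contains no beam reflection or input logic, only these rotation events.
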(event `self.ReceiveTick`
  (params (DeltaSeconds :type "Float (single-precision)"))
  (bind (_returnvalue_roll _returnvalue_pitch _returnvalue_yaw) (`KismetMathLibrary.BreakRotator` (`self.K2_GetActorRotation`)))
  (`self.K2_SetActorRotation` (`KismetMathLibrary.MakeRotator` _returnvalue_roll _returnvalue_pitch (+ _returnvalue_yaw (* (`self.Rotation`) DeltaSeconds)))))

(event `RotateClockwise`
  (set `self.Rotation` 20.0))

(event `RotateCounterClockwise`
  (set `self.Rotation` -20.0))

(event `StopRotation`
  (set `self.Rotation` 0.0))

(fn `UserConstructionScript`)