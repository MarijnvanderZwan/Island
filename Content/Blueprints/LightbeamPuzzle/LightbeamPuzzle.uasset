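; Lightbeam puzzle actor that marks its goal flag as completed once the puzzle's goal is solved.
; Until solved, it checks the referenced LightbeamGoal's Solved state every Tick.
; When that turns true, it latches its own Solved flag and calls SetCompleted on the BP_GoalFlag held in its GoalFlag child actor component.
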(event `self.ReceiveTick`
  (params (DeltaSeconds :type "Float (single-precision)"))
  (if (not (`self.Solved`))
    (bind _aslightbeam_goal (cast `/Game/Blueprints/LightbeamPuzzle/LightbeamGoal` (`self.Goal`)))
    (if (`/Game/Blueprints/LightbeamPuzzle/LightbeamGoal.Solved` _aslightbeam_goal)
      (set `self.Solved` true)
      (bind _asbp_goal_flag (cast `/Game/Blueprints/Goals/BP_GoalFlag` (`ChildActorComponent.ChildActor` (`self.GoalFlag`))))
      (`/Game/Blueprints/Goals/BP_GoalFlag.SetCompleted` _asbp_goal_flag))))

(fn `UserConstructionScript`
  (`parent.UserConstructionScript`))