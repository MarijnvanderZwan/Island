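; Light beam emitter for a reflection puzzle, shown only through debug-drawn line traces.
; Each Tick traces forward from the Arrow, and hits on "Reflect"-tagged actors call the recursive, count-capped Bounce event.
; Bounces mirror the End position vector, not the beam direction, by the impact normal.
; Tagged end hits set Solved on a LightbeamGoal or call Absorb on a BP_Crystal.
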(event `Bounce`
  (if (< (`self.BounceCount`) 10)
    (bind _outhit (`KismetSystemLibrary.LineTraceSingleForObjects` :`Start` (`self.Start`) :`End` (`self.End`) :`ObjectTypes` (`|MakeArray` "ObjectTypeQuery1" "ObjectTypeQuery2" :!type "EObjectTypeQuery Enum") :`bTraceComplex` true :`DrawDebugType` "ForOneFrame" :`DrawTime` 1.0))
    (bind (_bblockinghit _binitialoverlap _time _location _impactpoint _normal _impactnormal _physmat _hitactor) (`GameplayStatics.BreakHitResult` _outhit))
    (if (!= _hitactor null)
      (bind _tags (`Actor.Tags` _hitactor))
      (if (`KismetArrayLibrary.Array_Contains` _tags "Reflect")
        (set `self.End` (`KismetMathLibrary.MirrorVectorByNormal` (`self.End`) _impactnormal))
        (set `self.Start` (+ _impactpoint _normal))
        (set `self.BounceCount` (+ (`self.BounceCount`) 1))
        (`self.Bounce`)
        (else
          (set `self.BounceCount` 0)
          (if (`KismetArrayLibrary.Array_Contains` _tags "ReflectGoal")
            (bind _aslightbeam_goal (cast `/Game/Blueprints/LightbeamPuzzle/LightbeamGoal` _hitactor))
            (set `/Game/Blueprints/LightbeamPuzzle/LightbeamGoal.Solved` true _aslightbeam_goal)
            (elif (`KismetArrayLibrary.Array_Contains` _tags "Absorb")
              (`KismetSystemLibrary.PrintString` "Absorb")
              (bind _asbp_crystal (cast `/Game/Blueprints/LightbeamPuzzle/BP_Crystal` _hitactor))
              (`/Game/Blueprints/LightbeamPuzzle/BP_Crystal.Absorb` _asbp_crystal))))))
    (else
      (set `self.BounceCount` 0))))

(event `self.ReceiveTick`
  (params (DeltaSeconds :type "Float (single-precision)"))
  (bind _arrow (`self.Arrow`))
  (bind _returnvalue (`SceneComponent.K2_GetComponentLocation` _arrow))
  (`|ExecutionSequence`
    (:`then_0`
      (if (<= (`self.BounceCount`) 0)
        (set `self.Start` _returnvalue)
        (set `self.End` (+ _returnvalue (* (`SceneComponent.GetForwardVector` _arrow) 10000.0)))))
    (:`then_1`
      (bind _outhit (`KismetSystemLibrary.LineTraceSingleForObjects` :`Start` (`self.Start`) :`End` (`self.End`) :`ObjectTypes` (`|MakeArray` "ObjectTypeQuery1" "ObjectTypeQuery2" :!type "EObjectTypeQuery Enum") :`bTraceComplex` true :`DrawDebugType` "ForOneFrame"))
      (bind (_bblockinghit _binitialoverlap _time _location _impactpoint _normal _impactnormal _physmat _hitactor) (`GameplayStatics.BreakHitResult` _outhit))
      (if (!= _hitactor null)
        (bind _tags (`Actor.Tags` _hitactor))
        (if (`KismetArrayLibrary.Array_Contains` _tags "Reflect")
          (set `self.End` (`KismetMathLibrary.MirrorVectorByNormal` (`self.End`) _impactnormal))
          (set `self.Start` (+ _impactpoint _normal))
          (`self.Bounce`)
          (elif (`KismetArrayLibrary.Array_Contains` _tags "ReflectGoal")
            (bind _aslightbeam_goal (cast `/Game/Blueprints/LightbeamPuzzle/LightbeamGoal` _hitactor))
            (set `/Game/Blueprints/LightbeamPuzzle/LightbeamGoal.Solved` true _aslightbeam_goal)
            (elif (`KismetArrayLibrary.Array_Contains` _tags "Absorb")
              (`KismetSystemLibrary.PrintString` "Absorb")
              (bind _asbp_crystal (cast `/Game/Blueprints/LightbeamPuzzle/BP_Crystal` _hitactor))
              (`/Game/Blueprints/LightbeamPuzzle/BP_Crystal.Absorb` _asbp_crystal))))))))

(fn `UserConstructionScript`)