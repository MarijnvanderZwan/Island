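; BP_LightbeamDoor is a door for the lightbeam puzzle that slides its static mesh between a closed and an open position.
; BeginPlay records the starting position as closed, and the SetDoorOpen and SetDoorClosed events switch the target between that position plus UpOffset and the position itself.
; Tick eases the mesh toward the target by a fraction scaled by delta time and AnimationSpeed, snapping into place when close.
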(event `self.ReceiveBeginPlay`
  (bind _output_get (set `self.DownLocation` (`SceneComponent.K2_GetComponentLocation` (`self.StaticMesh`))))
  (set `self.TargetLocation` _output_get))

(event `SetDoorOpen`
  (set `self.TargetLocation` (+ (`self.DownLocation`) (`self.UpOffset`))))

(event `SetDoorClosed`
  (set `self.TargetLocation` (`self.DownLocation`)))

(event `self.ReceiveTick`
  (params (DeltaSeconds :type "Float (single-precision)"))
  (bind _returnvalue (`SceneComponent.K2_GetComponentLocation` (`self.StaticMesh`)))
  (bind _returnvalue_2 (- (`self.TargetLocation`) _returnvalue))
  (if (< (`KismetMathLibrary.VSize` _returnvalue_2) 5.0)
    (`SceneComponent.K2_SetWorldLocation` (`self.StaticMesh`) (`self.TargetLocation`) false false)
    (else
      (`SceneComponent.K2_SetWorldLocation` (`self.StaticMesh`) (+ (* _returnvalue_2 (* DeltaSeconds (`self.AnimationSpeed`))) _returnvalue) false false))))

(fn `UserConstructionScript`)