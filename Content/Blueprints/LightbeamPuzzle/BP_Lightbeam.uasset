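; Light beam emitter for a reflection puzzle, tracing a bouncing beam from its Arrow and rebuilding it on a short Tick timer.
; Recursive line traces mirror off "Reflect" actors, redirect through BP_Crystal on "Absorb" and mark LightbeamGoal solved on "ReflectGoal", with no bounce limit.
; Each rebuild destroys and respawns a beam particle component per segment, using temporary StaticMeshActors as source and target, plus impact emitters at hits.
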(event `self.ReceiveTick`
  (params (DeltaSeconds :type "Float (single-precision)"))
  (bind _output_get (set `self.TimeSinceLastTick` (+ DeltaSeconds (`self.TimeSinceLastTick`))))
  (if (> _output_get 0.01)
    (`KismetArrayLibrary.Array_Clear` (`self.Positions`))
    (`self.RecalculateBeam`)
    (`self.SetPositions`)))

(event `RecalculateBeam`
  (bind _arrow (`self.Arrow`))
  (bind _returnvalue (`SceneComponent.K2_GetComponentLocation` _arrow))
  (`|ExecutionSequence`
    (:`then_0`
      (`KismetArrayLibrary.Array_Clear` (`self.Positions`))
      (bind _output_get (set `self.Start` _returnvalue))
      (set `self.BeamDirection` (- (+ _returnvalue (* (`SceneComponent.GetForwardVector` _arrow) 10000.0)) _output_get))
      (`KismetArrayLibrary.Array_Add` (`self.Positions`) _output_get))
    (:`then_1`
      (`self.Bounce`))))

(event `Bounce`
  (bind _start (`self.Start`))
  (bind _positions (`self.Positions`))
  (bind _returnvalue (+ _start (* (`self.BeamDirection`) 10.0)))
  (bind (_outhit _returnvalue_2) (`KismetSystemLibrary.LineTraceSingleForObjects` _start _returnvalue (`|MakeArray` "ObjectTypeQuery1" "ObjectTypeQuery2" "ObjectTypeQuery3" "ObjectTypeQuery4" :!type "EObjectTypeQuery Enum") true))
  (bind (_bblockinghit _binitialoverlap _time _location _impactpoint _normal _impactnormal _physmat _hitactor) (`GameplayStatics.BreakHitResult` _outhit))
  (if (and _returnvalue_2 (!= _hitactor null))
    (bind _tags (`Actor.Tags` _hitactor))
    (if (`KismetArrayLibrary.Array_Contains` _tags "Reflect")
      (set `self.BeamDirection` (`KismetMathLibrary.MirrorVectorByNormal` (- _impactpoint (`self.Start`)) _impactnormal))
      (bind _output_get (set `self.Start` _impactpoint))
      (`KismetArrayLibrary.Array_Add` (`self.Positions`) _output_get)
      (`GameplayStatics.SpawnEmitterAtLocation` "/Game/Effects/Particles/P_ArcaneBolt.P_ArcaneBolt" _output_get)
      (`self.Bounce`)
      (elif (`KismetArrayLibrary.Array_Contains` _tags "ReflectGoal")
        (bind _aslightbeam_goal (cast `/Game/Blueprints/LightbeamPuzzle/LightbeamGoal` _hitactor)
          (:`then`
            (set `/Game/Blueprints/LightbeamPuzzle/LightbeamGoal.Solved` true _aslightbeam_goal))
          (:`CastFailed`
            _))
        (`KismetArrayLibrary.Array_Add` (`self.Positions`) _impactpoint)
        (`GameplayStatics.SpawnEmitterAtLocation` "/Game/Effects/Particles/P_ArcaneBolt.P_ArcaneBolt" _impactpoint)
        (elif (`KismetArrayLibrary.Array_Contains` _tags "Absorb")
          (bind _asbp_crystal (cast `/Game/Blueprints/LightbeamPuzzle/BP_Crystal` _hitactor))
          (bind (_start_2 _direction) (`/Game/Blueprints/LightbeamPuzzle/BP_Crystal.GetReflectedResult` _asbp_crystal))
          (`KismetArrayLibrary.Array_Add` _positions _impactpoint)
          (set `self.Start` _start_2)
          (`KismetArrayLibrary.Array_Add` _positions _start_2)
          (`GameplayStatics.SpawnEmitterAtLocation` "/Game/Effects/Particles/P_ArcaneBolt.P_ArcaneBolt" _start_2)
          (set `self.BeamDirection` _direction)
          (`self.Bounce`)
          (else
            (set `self.BounceCount` 0)
            (`KismetArrayLibrary.Array_Add` (`self.Positions`) _location)
            (`GameplayStatics.SpawnEmitterAtLocation` "/Game/Effects/Particles/P_ArcaneBolt.P_ArcaneBolt" _location)))))
    (else
      (set `self.BounceCount` 0)
      (`KismetArrayLibrary.Array_Add` (`self.Positions`) _returnvalue))))

(event `SetPositions`
  (bind _positions (`self.Positions`))
  (bind _actors (`self.Actors`))
  (`self.DestroyComponents`)
  (for _array_element _actors
    (`self.K2_DestroyActor` _array_element))
  (`KismetArrayLibrary.Array_Clear` _actors)
  (for _index (range 1 (`KismetArrayLibrary.Array_Length` (`self.Positions`)))
    (`self.SpawnComponentsForPositions` (`|GetArrayItem` _positions _index) (`|GetArrayItem` _positions (- _index 1)))
    (set `self.TimeSinceLastTick` 0.0)))

(fn `DestroyComponents`
  (for _array_element (`SceneComponent.GetChildrenComponents` (`self.Arrow`) false)
    (`ActorComponent.K2_DestroyComponent` _array_element)))

(fn `SpawnComponentsForPositions`
  (params (Position1 :type "Vector Structure") (Position2 :type "Vector Structure"))
  (bind _actors (`self.Actors`))
  (bind _returnvalue (`AddComponent|NODE_AddParticleSystemComponent-1`))
  (bind _returnvalue_2 (`|SpawnActorFromClass` "/Script/Engine.StaticMeshActor" (`KismetMathLibrary.MakeTransform` Position1) "AlwaysSpawn" "OverrideRootScale"))
  (`KismetArrayLibrary.Array_Add` _actors _returnvalue_2)
  (bind _returnvalue_3 (`|SpawnActorFromClass` "/Script/Engine.StaticMeshActor" (`KismetMathLibrary.MakeTransform` Position2) "AlwaysSpawn" "OverrideRootScale"))
  (`KismetArrayLibrary.Array_Add` _actors _returnvalue_3)
  (set `ParticleSystemComponent.InstanceParameters` (`|MakeArray` (make `ParticleSysParam` "BeamSource" "PSPT_Actor" 0.0 0.0 Position1 (0.0 0.0 0.0) (struct) _returnvalue_2) (make `ParticleSysParam` "BeamTarget" "PSPT_Actor" 0.0 0.0 Position2 (0.0 0.0 0.0) (struct) _returnvalue_3)) _returnvalue))

(fn `UserConstructionScript`)