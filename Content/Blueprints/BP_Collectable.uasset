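; BP_Collectable is a spinning pickup that the player collects by touch, optionally reporting to a puzzle.
; Tick adds a fixed yaw step to the mesh every frame, without delta-time scaling.
; When BP_Player first overlaps the Box, it sets the Collected flag, prints a message, hides the mesh and plays the Victory sound.
; If a Puzzle reference is set, it then calls CoinCollectedInPuzzle on it; the actor is never destroyed.
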(event `self.ReceiveTick`
  (params (DeltaSeconds :type "Float (single-precision)"))
  (bind _mesh (`self.Mesh`))
  (bind (_relativerotation_roll _relativerotation_pitch _relativerotation_yaw) (`KismetMathLibrary.BreakRotator` (`SceneComponent.RelativeRotation` _mesh)))
  (`SceneComponent.K2_SetRelativeRotation` _mesh (`KismetMathLibrary.MakeRotator` _relativerotation_roll _relativerotation_pitch (+ _relativerotation_yaw 1.0)) false false))

(event `self.Box.OnComponentBeginOverlap`
  (params (OverlappedComponent :type "PrimitiveComponent Object Reference") (OtherActor :type "Actor Object Reference") (OtherComp :type "PrimitiveComponent Object Reference") (OtherBodyIndex :type Integer) (bFromSweep :type Boolean) (SweepResult :type "HitResult Structure (by ref)"))
  (bind _puzzle (`self.Puzzle`))
  (if (not (`self.Collected`))
    (cast `/Game/Blueprints/BP_Player` OtherActor)
    (`KismetSystemLibrary.PrintString` "Collected collectible")
    (set `self.Collected` true)
    (`SceneComponent.SetVisibility` (`self.Mesh`) false false)
    (`GameplayStatics.PlaySound2D` "/Game/Audio/Effect/Victory.Victory")
    (if (!= _puzzle null)
      (`/Game/Blueprints/GenericPuzzle/BP_Puzzle.CoinCollectedInPuzzle` _puzzle))))

(fn `UserConstructionScript`)