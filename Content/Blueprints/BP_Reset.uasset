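; BP_Reset is an interactable lever that resets the block puzzle when the player uses it.
; Begin and end overlap events with BP_Player set a flag tracking whether the player is in range.
; Pressing the Action input while in range calls ResetPuzzle on the first BP_BlockPuzzle found in the level and plays the Lever animation.
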(event `self.ReceiveActorBeginOverlap`
  (params (OtherActor :type "Actor Object Reference"))
  (cast `/Game/Blueprints/BP_Player` OtherActor)
  (set `self.CurrentlyOverlappingPlayer` true))

(event `self.ReceiveActorEndOverlap`
  (params (OtherActor :type "Actor Object Reference"))
  (cast `/Game/Blueprints/BP_Player` OtherActor)
  (set `self.CurrentlyOverlappingPlayer` false))

(event `InputAction|Action` :consume false
  (params (Key :type "Key Structure" :default "AnyKey"))
  (:`Pressed`
    (if (`self.CurrentlyOverlappingPlayer`)
      (bind _outactors (`GameplayStatics.GetAllActorsOfClass` "/Game/Blueprints/BP_BlockPuzzle.BP_BlockPuzzle_C"))
      (`/Game/Blueprints/BP_BlockPuzzle.ResetPuzzle` (`KismetArrayLibrary.Array_Get` _outactors))
      (`SkeletalMeshComponent.Play` (`self.Lever`) false))))

(fn `UserConstructionScript`)