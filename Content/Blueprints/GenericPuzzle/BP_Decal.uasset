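; Generic puzzle decal actor that glows brightly when activated and dims when deactivated.
; The construction script applies its DecalMaterial to the Decal component, and SetDecalMaterial swaps that material at runtime.
; Activate and Deactivate each create a new dynamic instance of the stored material, set its Emmissive Intensity high or low, and assign it to the decal.
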(event `Activate`
  (bind _decalmaterial (`self.DecalMaterial`))
  (bind _returnvalue (`KismetMaterialLibrary.CreateDynamicMaterialInstance` _decalmaterial _decalmaterial))
  (`MaterialInstanceDynamic.SetScalarParameterValue` _returnvalue "Emmissive Intensity" 15.0)
  (`DecalComponent.SetDecalMaterial` (`self.Decal`) _returnvalue))

(event `Deactivate`
  (bind _decalmaterial (`self.DecalMaterial`))
  (bind _returnvalue (`KismetMaterialLibrary.CreateDynamicMaterialInstance` _decalmaterial _decalmaterial))
  (`MaterialInstanceDynamic.SetScalarParameterValue` _returnvalue "Emmissive Intensity" 1.0)
  (`DecalComponent.SetDecalMaterial` (`self.Decal`) _returnvalue))

(event `SetDecalMaterial`
  (params (DecalMaterial :type "MaterialInstance Object Reference"))
  (bind _output_get (set `self.DecalMaterial` DecalMaterial))
  (`DecalComponent.SetDecalMaterial` (`self.Decal`) _output_get))

(fn `UserConstructionScript`
  (bind _output_get (set `self.DecalMaterial` (`self.DecalMaterial`)))
  (`DecalComponent.SetDecalMaterial` (`self.Decal`) _output_get))