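; BP_Puzzle is a generic puzzle manager that detects when its puzzle is solved.
; On BeginPlay it registers itself with its puzzle, goal and interactive elements and its GoalCondition.
; Until solved, it polls GoalCondition every Tick; on success it sets PuzzleSolved, notifies the goal elements and plays a victory sound.
; ResetPuzzle is a stub that only prints a message.
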(event `self.ReceiveBeginPlay`
  (`self.SetPuzzleForElements`))

(event `self.ReceiveTick`
  (params (DeltaSeconds :type "Float (single-precision)"))
  (if (not (`self.PuzzleSolved`))
    (bind _solved (`/Game/Blueprints/GenericPuzzle/BP_GoalCondition.CheckSolved` (`self.GoalCondition`)))
    (if _solved
      (`self.PuzzleIsSolved`)
      (`GameplayStatics.PlaySound2D` "/Game/Audio/Effect/Victory.Victory"))))

(event `Reset Puzzle`
  (`KismetSystemLibrary.PrintString` "Resetting puzzle"))

(fn `PuzzleIsSolved`
  (set `self.PuzzleSolved` true)
  (for _array_element (`self.PuzzleGoalElements`)
    (`/Game/Blueprints/GenericPuzzle/BP_PuzzleGoalElement.PuzzleSolved` _array_element)))

(fn `SetPuzzleForElements`
  (for _array_element (`self.PuzzleElements`)
    (set `/Game/Blueprints/GenericPuzzle/BP_PuzzleElement.Puzzle` self _array_element))
  (for _array_element_2 (`self.PuzzleGoalElements`)
    (set `/Game/Blueprints/GenericPuzzle/BP_PuzzleGoalElement.Puzzle` self _array_element_2))
  (for _array_element_3 (`self.InteractivePuzzleElements`)
    (set `/Game/Blueprints/GenericPuzzle/BP_InteractivePuzzleElement.Puzzle` self _array_element_3))
  (set `/Game/Blueprints/GenericPuzzle/BP_GoalCondition.Puzzle` self (`self.GoalCondition`)))

(fn `UserConstructionScript`)