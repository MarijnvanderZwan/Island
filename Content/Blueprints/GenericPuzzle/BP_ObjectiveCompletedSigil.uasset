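; Puzzle sigil controller that shows when a set of objectives is complete by toggling its linked sigils.
; Every tick it checks whether all GoalsToSatisfy report solved and stores the result in SigilSatisfied.
; It then activates or deactivates every entry in SigilsToUpdate, so the sigils switch off again if any goal becomes unsolved.
; The construction script applies a shared DecalMaterial to those sigils.
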(event `self.ReceiveTick`
  (params (DeltaSeconds :type "Float (single-precision)"))
  (bind _sigilstoupdate (`self.SigilsToUpdate`))
  (bind _satisfied (`self.CheckSigilSatisfied`))
  (bind _output_get (set `self.SigilSatisfied` _satisfied))
  (if _output_get
    (for _array_element _sigilstoupdate
      (`/Game/Blueprints/GenericPuzzle/BP_Decal.Activate` _array_element))
    (else
      (for _array_element_2 _sigilstoupdate
        (`/Game/Blueprints/GenericPuzzle/BP_Decal.Deactivate` _array_element_2)))))

(fn `CheckSigilSatisfied`
  (returns (satisfied :type Boolean))
  (for _array_element (`self.GoalsToSatisfy`)
    (bind _solved (`/Game/Blueprints/GenericPuzzle/BP_GoalCondition.CheckSolved` _array_element))
    (if (not _solved)
      (return false)))
  (return true))

(fn `UserConstructionScript`
  (for _array_element (`self.SigilsToUpdate`)
    (`/Game/Blueprints/GenericPuzzle/BP_Decal.SetDecalMaterial` _array_element (`self.DecalMaterial`))))