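; Crumbling platform that shakes, sinks and vanishes after the player touches it, then respawns at its original spot.
; Overlap with BP_Player starts shaking and a rock-crumbling sound; Tick then accumulates time, lowering the mesh linearly and wobbling pitch and yaw with sine and cosine.
; Past the fall threshold, it stops the sound, disables visibility and collision, resets transform and state, then reappears after a delay.
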(event `self.ReceiveBeginPlay`
  (set `self.OriginalWorldLocation` (`SceneComponent.K2_GetComponentLocation` (`self.StaticMesh`))))

(event `self.ReceiveTick`
  (params (DeltaSeconds :type "Float (single-precision)"))
  (bind _shakingintensity (`self.ShakingIntensity`))
  (bind _sound (`self.Sound`))
  (if (> (`self.CurrentValue`) (`self.TimeBeforeFallingDown`))
    (`self.SetMeshVisibility` false)
    (`AudioComponent.Stop` _sound)
    (`ActorComponent.K2_DestroyComponent` _sound)
    (`KismetSystemLibrary.Delay` (`self.TimeBeforeRespawning`))
    (`self.SetMeshVisibility` true)
    (elif (`self.Shaking`)
      (bind _output_get (set `self.CurrentValue` (+ DeltaSeconds (`self.CurrentValue`))))
      (`SceneComponent.K2_SetWorldLocation` (`self.StaticMesh`) (- (`self.OriginalWorldLocation`) (`KismetMathLibrary.MakeVector` 0.0 0.0 (* _output_get 10.0))) false false)
      (bind _returnvalue (* _output_get (`self.ShakingSpeed`)))
      (`SceneComponent.K2_SetRelativeRotation` (`self.StaticMesh`) (`KismetMathLibrary.MakeRotator` 0.0 (* (`KismetMathLibrary.Sin` _returnvalue) _shakingintensity) (* (`KismetMathLibrary.Cos` _returnvalue) _shakingintensity)) false false))))

(event `self.Collision.OnComponentBeginOverlap`
  (params (OverlappedComponent :type "PrimitiveComponent Object Reference") (OtherActor :type "Actor Object Reference") (OtherComp :type "PrimitiveComponent Object Reference") (OtherBodyIndex :type Integer) (bFromSweep :type Boolean) (SweepResult :type "HitResult Structure (by ref)"))
  (cast `/Game/Blueprints/BP_Player` OtherActor)
  (set `self.Shaking` true)
  (bind _returnvalue (`GameplayStatics.SpawnSoundAtLocation` "/Game/Audio/Effect/CrumblingRocks.CrumblingRocks" (`SceneComponent.K2_GetComponentLocation` (`self.StaticMesh`)) (struct) 0.5 0.5 0.0 null null))
  (set `self.Sound` _returnvalue))

(fn `Reset`
  (bind _staticmesh (`self.StaticMesh`))
  (`SceneComponent.K2_SetWorldLocation` _staticmesh (`self.OriginalWorldLocation`) false false)
  (`SceneComponent.K2_SetRelativeRotation` :`self` _staticmesh)
  (set `self.CurrentValue` 0.0)
  (set `self.Shaking` false))

(fn `SetMeshVisibility`
  (params (Visible :type Boolean))
  (bind _staticmesh (`self.StaticMesh`))
  (`SceneComponent.SetVisibility` _staticmesh Visible false)
  (`self.Reset`)
  (if Visible
    (`PrimitiveComponent.SetCollisionEnabled` _staticmesh "QueryAndPhysics")
    (else
      (`PrimitiveComponent.SetCollisionEnabled` _staticmesh "NoCollision"))))

(fn `UserConstructionScript`)