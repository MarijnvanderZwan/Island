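; RisingBlock is a platform block that rises to a target position when its PuzzleSolved event fires, playing a gate-opening sound.
; It records its starting location on BeginPlay.
; While rising, Tick linearly interpolates from that start to TargetPosition using accumulated time over TimeToRise, then snaps to the target and stops once within a small distance threshold.
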(event `self.ReceiveBeginPlay`
  (set `self.StartPosition` (`self.K2_GetActorLocation`)))

(event `self.ReceiveTick`
  (params (DeltaSeconds :type "Float (single-precision)"))
  (bind _targetposition (`self.TargetPosition`))
  (if (`self.Rising`)
    (if (< (`KismetMathLibrary.VSize` (- (`self.K2_GetActorLocation`) (`self.TargetPosition`))) 10.0)
      (`self.K2_SetActorLocation` _targetposition)
      (set `self.Rising` false)
      (else
        (bind _output_get (set `self.TimePassed` (+ DeltaSeconds (`self.TimePassed`))))
        (`self.K2_SetActorLocation` (`KismetMathLibrary.VLerp` (`self.StartPosition`) _targetposition (/ _output_get (`self.TimeToRise`))))))))

(event `self.PuzzleSolved`
  (set `self.Rising` true)
  (`GameplayStatics.PlaySoundAtLocation` "/Game/Audio/Effect/Gate_opening.Gate_Opening" (`self.K2_GetActorLocation`) (struct) 1.0 1.0 0.0 null null null))

(fn `UserConstructionScript`)