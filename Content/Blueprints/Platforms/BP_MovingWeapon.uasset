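; BP_MovingWeapon is a swinging hazard that damages the player on contact.
; Tick feeds accumulated time through a sine wave scaled by SwingingTime and SwingingAngle to produce a pendulum-like swing.
; SetRotation clamps that angle and adds it to the pitch of the root's world rotation captured at BeginPlay, applying the result as relative rotation.
; A Sphere overlap applies fixed damage to BP_Player.
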(event `self.ReceiveBeginPlay`
  (set `self.BaseRotation` (`SceneComponent.K2_GetComponentRotation` (`self.DefaultSceneRoot`))))

(event `self.ReceiveTick`
  (params (DeltaSeconds :type "Float (single-precision)"))
  (bind _output_get (set `self.TotalTime` (+ DeltaSeconds (`self.TotalTime`))))
  (`self.SetRotation` (* (`KismetMathLibrary.Sin` (`KismetMathLibrary.MultiplyByPi` (/ _output_get (`self.SwingingTime`)))) (`self.SwingingAngle`))))

(event `self.Sphere.OnComponentBeginOverlap`
  (params (OverlappedComponent :type "PrimitiveComponent Object Reference") (OtherActor :type "Actor Object Reference") (OtherComp :type "PrimitiveComponent Object Reference") (OtherBodyIndex :type Integer) (bFromSweep :type Boolean) (SweepResult :type "HitResult Structure (by ref)"))
  (bind _asbp_player (cast `/Game/Blueprints/BP_Player` OtherActor))
  (`GameplayStatics.ApplyDamage` _asbp_player 75.0 null self))

(fn `SetRotation`
  (params (Angle :type "Float (double-precision)"))
  (bind _swingingangle (`self.SwingingAngle`))
  (bind (_baserotation_roll _baserotation_pitch _baserotation_yaw) (`KismetMathLibrary.BreakRotator` (`self.BaseRotation`)))
  (`SceneComponent.K2_SetRelativeRotation` (`self.DefaultSceneRoot`) (`KismetMathLibrary.MakeRotator` _baserotation_roll (+ _baserotation_pitch (`KismetMathLibrary.FClamp` Angle (* _swingingangle -1.0) _swingingangle)) _baserotation_yaw) false false))

(fn `UserConstructionScript`)