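; Squashing block platform hazard that cycles up and down between an air position and a ground position.
; Tick runs a four-state timer machine (In Air, Falling, On Ground, Rising), each phase with its own duration.
; Falling and Rising linearly interpolate the static mesh between the two marker components' world locations by elapsed time, snapping to the endpoint when the phase ends.
; Movement is unswept; no overlap or damage logic is implemented.
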(event `self.ReceiveTick`
  (params (DeltaSeconds :type "Float (single-precision)"))
  (set `self.TimePassed` (+ (`self.TimePassed`) DeltaSeconds))
  (switch `/Game/Blueprints/Platforms/SquashingState` (`self.SquashingState`)
    (:`NewEnumerator0`
      (if (> (`self.TimePassed`) (`self.TimeInAir`))
        (set `self.SquashingState` "NewEnumerator1")
        (set `self.TimePassed` 0.0)))
    (:`NewEnumerator1`
      (if (> (`self.TimePassed`) (`self.TimeFalling`))
        (set `self.SquashingState` "NewEnumerator2")
        (`SceneComponent.K2_SetWorldLocation` (`self.StaticMesh`) (`SceneComponent.K2_GetComponentLocation` (`self.GroundPosition`)) false false)
        (set `self.TimePassed` 0.0)
        (else
          (`self.Falling`))))
    (:`NewEnumerator2`
      (if (> (`self.TimePassed`) (`self.TimeOnGround`))
        (set `self.SquashingState` "NewEnumerator3")
        (set `self.TimePassed` 0.0)))
    (:`NewEnumerator3`
      (if (> (`self.TimePassed`) (`self.TimeRising`))
        (set `self.SquashingState` "NewEnumerator0")
        (`SceneComponent.K2_SetWorldLocation` (`self.StaticMesh`) (`SceneComponent.K2_GetComponentLocation` (`self.AirPosition`)) false false)
        (set `self.TimePassed` 0.0)
        (else
          (`self.Rising`))))))

(fn `Falling`
  (`SceneComponent.K2_SetWorldLocation` (`self.StaticMesh`) (`KismetMathLibrary.VLerp` (`SceneComponent.K2_GetComponentLocation` (`self.AirPosition`)) (`SceneComponent.K2_GetComponentLocation` (`self.GroundPosition`)) (/ (`self.TimePassed`) (`self.TimeFalling`))) false false))

(fn `Rising`
  (`SceneComponent.K2_SetWorldLocation` (`self.StaticMesh`) (`KismetMathLibrary.VLerp` (`SceneComponent.K2_GetComponentLocation` (`self.GroundPosition`)) (`SceneComponent.K2_GetComponentLocation` (`self.AirPosition`)) (/ (`self.TimePassed`) (`self.TimeRising`))) false false))

(fn `UserConstructionScript`)