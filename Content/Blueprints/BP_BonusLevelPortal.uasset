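; BP_BonusLevelPortal is an actor gated by a cylinder that clears once all coins in its Area are collected.
; On BeginPlay it counts BP_Collectable actors with a matching AreaIdentifier and binds to the GlobalPuzzleHandler's coin-collected dispatcher.
; Each matching pickup updates a TextRender showing the coins remaining.
; When none remain, the cylinder and its children are hidden and the cylinder's collision is disabled.
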(event `self.ReceiveBeginPlay`
  (bind _outactors (`GameplayStatics.GetAllActorsOfClass` "/Game/Blueprints/GlobalPuzzleHandler.GlobalPuzzleHandler_C"))
  (add `/Game/Blueprints/GlobalPuzzleHandler.CoinCollectedDispatcher` (`|GetArrayItem` _outactors) (delegate `CoinCollected`))
  (`self.InitializeCoinCounter`)
  (`self.SetCoinCounter`)
  (`self.CheckCompletion`))

(event `CoinCollected`
  (params (AreaIdentifier :type "/Game/Blueprints/Puzzles/PuzzleAreaIdentifier Enum" :default "NewEnumerator0"))
  (if (`|EnumEquality` AreaIdentifier (`self.Area`))
    (set `self.CollectedCoins` (+ (`self.CollectedCoins`) 1))
    (`self.SetCoinCounter`)
    (`self.CheckCompletion`)))

(fn `CheckCompletion`
  (bind _cylinder (`self.Cylinder`))
  (if (>= (`self.CollectedCoins`) (`self.TotalCoins`))
    (`SceneComponent.SetVisibility` _cylinder false true)
    (`PrimitiveComponent.SetCollisionEnabled` _cylinder "NoCollision")))

(fn `InitializeCoinCounter`
  (locals (Count :type Integer))
  (bind _outactors (`GameplayStatics.GetAllActorsOfClass` "/Game/Blueprints/BP_Collectable.BP_Collectable_C"))
  (for _array_element _outactors
    (if (`|EnumEquality` (`/Game/Blueprints/BP_Collectable.Area Identifier` _array_element) (`self.Area`))
      (`/Engine/EditorBlueprintResources/StandardMacros.IncrementInt` (`local.Count`))))
  (set `self.TotalCoins` (`local.Count`)))

(fn `SetCoinCounter`
  (`TextRenderComponent.K2_SetText` (`self.TextRender`) (`KismetTextLibrary.Conv_IntToText` (- (`self.TotalCoins`) (`self.CollectedCoins`)))))

(fn `UserConstructionScript`)