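; BP_PortalPair is a one-way teleporter that moves a player from an entry portal to an exit point.
; On BeginPlay it registers itself as Parent on the BP_Portal child actor in PortalIn.
; Its PortalEntered event aligns the controller's rotation to the Arrow component, teleports the player to PortalOut without sweeping, and zeroes their velocity.
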(event `self.ReceiveBeginPlay`
  (bind _asbp_portal (cast `/Game/Blueprints/Portals/BP_Portal` (`ChildActorComponent.ChildActor` (`self.PortalIn`))))
  (set `/Game/Blueprints/Portals/BP_Portal.Parent` self _asbp_portal))

(event `PortalEntered`
  (params (Player :type "/Game/Blueprints/BP_Player Object Reference"))
  (`Controller.SetControlRotation` (`Pawn.GetController` Player) (`SceneComponent.K2_GetComponentRotation` (`self.Arrow`)))
  (`self.K2_SetActorLocation` Player (`SceneComponent.K2_GetComponentLocation` (`self.PortalOut`)) false true)
  (set `MovementComponent.Velocity` (0.0 0.0 0.0) (`Pawn.GetMovementComponent` Player)))

(fn `UserConstructionScript`)