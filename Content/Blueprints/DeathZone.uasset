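; DeathZone is a hazard actor that makes actors tagged Pickup sink slowly with a burn effect, then destroys them.
; Entering the SinkZone switches the pickup's mesh to overlap all channels, zeroes its velocity, raises linear damping and spawns P_Burn above it.
; Leaving the SinkZone zeroes velocity again and lowers damping, without restoring collision.
; Overlapping the DeathZone component destroys the pickup.
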(event `self.SinkZone.OnComponentBeginOverlap`
  (params (OverlappedComponent :type "PrimitiveComponent Object Reference") (OtherActor :type "Actor Object Reference") (OtherComp :type "PrimitiveComponent Object Reference") (OtherBodyIndex :type Integer) (bFromSweep :type Boolean) (SweepResult :type "HitResult Structure (by ref)"))
  (bind _returnvalue (`self.GetComponentByClass` OtherActor "/Script/Engine.StaticMeshComponent"))
  (if (`self.ActorHasTag` OtherActor "Pickup")
    (`PrimitiveComponent.SetCollisionResponseToAllChannels` _returnvalue "ECR_Overlap")
    (`PrimitiveComponent.SetAllPhysicsLinearVelocity` _returnvalue (0.0 0.0 0.0) false)
    (`PrimitiveComponent.SetLinearDamping` _returnvalue 20.0)
    (`GameplayStatics.SpawnEmitterAtLocation` "/Game/Effects/Particles/P_Burn.P_Burn" (+ (`SceneComponent.K2_GetComponentLocation` _returnvalue) (0.0 0.0 100.0)) (struct))))

(event `self.SinkZone.OnComponentEndOverlap`
  (params (OverlappedComponent :type "PrimitiveComponent Object Reference") (OtherActor :type "Actor Object Reference") (OtherComp :type "PrimitiveComponent Object Reference") (OtherBodyIndex :type Integer))
  (bind _returnvalue (`self.GetComponentByClass` OtherActor "/Script/Engine.StaticMeshComponent"))
  (if (`self.ActorHasTag` OtherActor "Pickup")
    (`PrimitiveComponent.SetAllPhysicsLinearVelocity` _returnvalue (0.0 0.0 0.0) false)
    (`PrimitiveComponent.SetLinearDamping` _returnvalue 0.01)))

(event `self.DeathZone.OnComponentBeginOverlap`
  (params (OverlappedComponent :type "PrimitiveComponent Object Reference") (OtherActor :type "Actor Object Reference") (OtherComp :type "PrimitiveComponent Object Reference") (OtherBodyIndex :type Integer) (bFromSweep :type Boolean) (SweepResult :type "HitResult Structure (by ref)"))
  (if (`self.ActorHasTag` OtherActor "Pickup")
    (`self.K2_DestroyActor` OtherActor)))

(fn `UserConstructionScript`)