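; Debug cheat Blueprint that marks puzzles as completed from the keyboard.
; On BeginPlay it finds and caches the first GlobalPuzzleHandler in the level.
; Numpad keys 1 to 6 each call that handler's CallPuzzleCompletedDispatcher with the matching puzzle enum value, with no validity check on the cached reference.
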(event `self.ReceiveBeginPlay`
  (bind _outactors (`GameplayStatics.GetAllActorsOfClass` "/Game/Blueprints/GlobalPuzzleHandler.GlobalPuzzleHandler_C"))
  (if (> (`KismetArrayLibrary.Array_Length` _outactors) 0)
    (set `self.GlobalPuzzleHandler` (`|GetArrayItem` _outactors))))

(event `Key|NumPadOne`
  (params (Key :type "Key Structure"))
  (:`Pressed`
    (`/Game/Blueprints/GlobalPuzzleHandler.PuzzleCompletedDispatcher` (`self.GlobalPuzzleHandler`) "NewEnumerator0")))

(event `Key|NumPadTwo`
  (params (Key :type "Key Structure"))
  (:`Pressed`
    (`/Game/Blueprints/GlobalPuzzleHandler.PuzzleCompletedDispatcher` (`self.GlobalPuzzleHandler`) "NewEnumerator1")))

(event `Key|NumPadThree`
  (params (Key :type "Key Structure"))
  (:`Pressed`
    (`/Game/Blueprints/GlobalPuzzleHandler.PuzzleCompletedDispatcher` (`self.GlobalPuzzleHandler`) "NewEnumerator2")))

(event `Key|NumPadFour`
  (params (Key :type "Key Structure"))
  (:`Pressed`
    (`/Game/Blueprints/GlobalPuzzleHandler.PuzzleCompletedDispatcher` (`self.GlobalPuzzleHandler`) "NewEnumerator3")))

(event `Key|NumPadFive`
  (params (Key :type "Key Structure"))
  (:`Pressed`
    (`/Game/Blueprints/GlobalPuzzleHandler.PuzzleCompletedDispatcher` (`self.GlobalPuzzleHandler`) "NewEnumerator4")))

(event `Key|NumPadSix`
  (params (Key :type "Key Structure"))
  (:`Pressed`
    (`/Game/Blueprints/GlobalPuzzleHandler.PuzzleCompletedDispatcher` (`self.GlobalPuzzleHandler`) "NewEnumerator5")))

(fn `UserConstructionScript`)