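; Light beam variant that deals damage over time to the player while the beam hits them.
; It extends the parent's ProcessLasers, using CheckPlayerHit to scan HitActors for a BP_Player before calling the parent logic.
; On a hit it applies DamagePerSecond scaled by world delta time to the first BP_Player found in the level, rather than to the hit actor itself.
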(event `self.ProcessLasers`
  (bind _playerhit (`self.CheckPlayerHit`))
  (if _playerhit
    (bind _outactors (`GameplayStatics.GetAllActorsOfClass` "/Game/Blueprints/BP_Player.BP_Player_C"))
    (`GameplayStatics.ApplyDamage` (`|GetArrayItem` _outactors) (* (`GameplayStatics.GetWorldDeltaSeconds`) (`self.DamagePerSecond`)) null self)
    (`parent.ProcessLasers`)
    (else
      (`parent.ProcessLasers`))))

(fn `CheckPlayerHit`
  (returns (PlayerHit :type Boolean))
  (for _array_element (`self.HitActors`)
    (cast `/Game/Blueprints/BP_Player` _array_element)
    (return true))
  (return false))

(fn `UserConstructionScript`
  (`parent.UserConstructionScript`))