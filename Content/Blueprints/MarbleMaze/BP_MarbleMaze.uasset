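; BP_MarbleMaze is an actor that the player tilts with the keyboard, apparently as the board of a marble maze.
; T/G and F/H add to a Direction vector on press and undo it on release, so held keys combine or cancel.
; Each Tick scales Direction by Movespeed and delta time and adds it to the actor's roll and pitch, with no angle clamp.
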(event `self.ReceiveTick`
  (params (DeltaSeconds :type "Float (single-precision)"))
  (bind (_returnvalue_roll _returnvalue_pitch) (`KismetMathLibrary.BreakRotator` (`self.K2_GetActorRotation`)))
  (bind (_returnvalue_x _returnvalue_y) (`KismetMathLibrary.BreakVector` (* (`self.Direction`) (* DeltaSeconds (`self.Movespeed`)))))
  (`self.K2_SetActorRotation` (`KismetMathLibrary.MakeRotator` (+ _returnvalue_x _returnvalue_roll) (+ _returnvalue_y _returnvalue_pitch))))

(event `Key|T`
  (params (Key :type "Key Structure"))
  (bind (_direction_x _direction_y) (`KismetMathLibrary.BreakVector` (`self.Direction`)))
  (bind (_direction_x_2 _direction_y_2) (`KismetMathLibrary.BreakVector` (`self.Direction`)))
  (:`Pressed`
    (set `self.Direction` (`KismetMathLibrary.MakeVector` _direction_x (+ _direction_y 1.0))))
  (:`Released`
    (set `self.Direction` (`KismetMathLibrary.MakeVector` _direction_x_2 (- _direction_y_2 1.0)))))

(event `Key|F`
  (params (Key :type "Key Structure"))
  (bind (_direction_x _direction_y) (`KismetMathLibrary.BreakVector` (`self.Direction`)))
  (bind (_direction_x_2 _direction_y_2) (`KismetMathLibrary.BreakVector` (`self.Direction`)))
  (:`Pressed`
    (set `self.Direction` (`KismetMathLibrary.MakeVector` (+ _direction_x 1.0) _direction_y)))
  (:`Released`
    (set `self.Direction` (`KismetMathLibrary.MakeVector` (- _direction_x_2 1.0) _direction_y_2))))

(event `Key|G`
  (params (Key :type "Key Structure"))
  (bind (_direction_x _direction_y) (`KismetMathLibrary.BreakVector` (`self.Direction`)))
  (bind (_direction_x_2 _direction_y_2) (`KismetMathLibrary.BreakVector` (`self.Direction`)))
  (:`Pressed`
    (set `self.Direction` (`KismetMathLibrary.MakeVector` _direction_x (- _direction_y 1.0))))
  (:`Released`
    (set `self.Direction` (`KismetMathLibrary.MakeVector` _direction_x_2 (+ _direction_y_2 1.0)))))

(event `Key|H`
  (params (Key :type "Key Structure"))
  (bind (_direction_x _direction_y) (`KismetMathLibrary.BreakVector` (`self.Direction`)))
  (bind (_direction_x_2 _direction_y_2) (`KismetMathLibrary.BreakVector` (`self.Direction`)))
  (:`Pressed`
    (set `self.Direction` (`KismetMathLibrary.MakeVector` (- _direction_x_2 1.0) _direction_y_2)))
  (:`Released`
    (set `self.Direction` (`KismetMathLibrary.MakeVector` (+ _direction_x 1.0) _direction_y))))

(fn `UserConstructionScript`
  (`parent.UserConstructionScript`))