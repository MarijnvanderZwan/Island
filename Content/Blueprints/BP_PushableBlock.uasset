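; Pushable block for a block puzzle that keeps moving in the direction it was pushed, driven by movement input every Tick.
; Push finds which of four side colliders is nearest the pusher's location and sets Direction opposite that side from the signs of its relative X/Y.
; The construction script registers the block with the first BP_BlockPuzzle found.
; ResetToStartingLocation teleports it to its BeginPlay position and clears Direction.
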(event `self.ReceiveBeginPlay`
  (set `self.StartingPosition` (`self.K2_GetActorLocation`)))

(event `self.ReceiveTick`
  (params (DeltaSeconds :type "Float (single-precision)"))
  (`self.AddMovementInput` (* (`self.Direction`) (* DeltaSeconds 20000.0))))

(fn `GetClosestCollider`
  (params (Location :type "Vector Structure"))
  (returns (Collider :type "BoxComponent Object Reference"))
  (locals (minDistance :type "Float (double-precision)" :default 5000.0) (minCollider :type "BoxComponent Object Reference"))
  (for _array_element (`self.Colliders`)
    (bind (_outpointonbody _returnvalue) (`PrimitiveComponent.GetClosestPointOnCollision` _array_element Location "None"))
    (if (< _returnvalue (`local.minDistance`))
      (set `local.minDistance` _returnvalue)
      (set `local.minCollider` _array_element)))
  (return (`local.minCollider`)))

(fn `Push`
  (params (FromLocation :type "Vector Structure"))
  (bind _collider (`self.GetClosestCollider` FromLocation))
  (bind (_relativelocation_x _relativelocation_y) (`KismetMathLibrary.BreakVector` (`SceneComponent.RelativeLocation` _collider)))
  (set `self.Direction` (`KismetMathLibrary.MakeVector` (* (`KismetMathLibrary.SignOfFloat` _relativelocation_x) -1.0) (* (`KismetMathLibrary.SignOfFloat` _relativelocation_y) -1.0))))

(fn `ResetToStartingLocation`
  (`self.K2_SetActorLocation` (`self.StartingPosition`) false true)
  (set `self.Direction` (0.0 0.0 0.0)))

(fn `UserConstructionScript`
  (bind _colliders (`self.Colliders`))
  (`KismetArrayLibrary.Array_Add` _colliders (`self.South`))
  (`KismetArrayLibrary.Array_Add` _colliders (`self.North`))
  (`KismetArrayLibrary.Array_Add` _colliders (`self.West`))
  (`KismetArrayLibrary.Array_Add` _colliders (`self.East`))
  (bind _outactors (`GameplayStatics.GetAllActorsOfClass` "/Game/Blueprints/BP_BlockPuzzle.BP_BlockPuzzle_C"))
  (`/Game/Blueprints/BP_BlockPuzzle.RegisterPushableblock` (`KismetArrayLibrary.Array_Get` _outactors) self))