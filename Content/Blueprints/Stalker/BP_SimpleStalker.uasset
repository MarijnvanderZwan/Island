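; BP_SimpleStalker is an actor that keeps within a distance band of the player, backing away when too close and approaching when too far.
; BeginPlay caches the first BP_Player, and each Tick SetStalkerState picks Flee, Stalk or Idle by comparing that distance to MinDistance and MaxDistance.
; Flee and Stalk teleport it a fixed step without delta-time scaling, so speed depends on frame rate, and also write a GOal variable.
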(event `self.ReceiveBeginPlay`
  (bind _outactors (`GameplayStatics.GetAllActorsOfClass` "/Game/Blueprints/BP_Player.BP_Player_C"))
  (set `self.Player` (`KismetArrayLibrary.Array_Get` _outactors)))

(event `self.ReceiveTick`
  (params (DeltaSeconds :type "Float (single-precision)"))
  (bind _returnvalue (`self.K2_GetActorLocation`))
  (bind _player (`self.Player`))
  (bind _returnvalue_2 (`self.K2_GetActorLocation` _player))
  (bind _returnvalue_3 (* (`KismetMathLibrary.Normal` (- _returnvalue _returnvalue_2)) 50.0))
  (bind _returnvalue_4 (+ _returnvalue _returnvalue_3))
  (`self.SetStalkerState` (`self.GetDistanceTo` _player))
  (switch `/Game/Blueprints/Stalker/StalkerState` (`self.State`)
    (:`NewEnumerator0`
      (`self.K2_SetActorLocation` _returnvalue_4 false true)
      (set `self.GOal` _returnvalue_4))
    (:`NewEnumerator2`
      (`self.K2_SetActorLocation` (- _returnvalue _returnvalue_3) false true)
      (set `self.GOal` _returnvalue_2))))

(fn `SetStalkerState`
  (params (Distance :type "Float (double-precision)"))
  (if (<= Distance (`self.MinDistance`))
    (set `self.State` "NewEnumerator0")
    (elif (>= Distance (`self.MaxDistance`))
      (set `self.State` "NewEnumerator2")
      (else
        (set `self.State` "NewEnumerator1")))))

(fn `UserConstructionScript`)