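; Behavior tree decorator for the Stalker AI that gates a branch on its distance to the actor it follows.
; It casts its owner to BP_StalkerAIController and measures from the controlled pawn to the TargetToFollow blackboard actor.
; Despite the CloseEnough name, it passes when that distance is at or beyond AcceptableDistance.
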(fn `PerformConditionCheck`
  (params (OwnerActor :type "Actor Object Reference"))
  (returns (ReturnValue :type Boolean))
  (bind _asbp_stalker_aicontroller (cast `/Game/Blueprints/Stalker/BP_StalkerAIController` OwnerActor))
  (set `self.AIControllerReference` _asbp_stalker_aicontroller)
  (return (>= (`KismetMathLibrary.VSize` (- (`Actor.K2_GetActorLocation` (`BTFunctionLibrary.GetBlackboardValueAsActor` (`self.TargetToFollow`))) (`Actor.K2_GetActorLocation` (`Controller.K2_GetPawn` (`self.AIControllerReference`))))) (`self.AcceptableDistance`))))