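; RapidMoveTo is a behavior tree task that moves the Stalker AI's pawn toward the actor in the TargetToFollow blackboard key.
; On first execution it casts the owner to BP_StalkerAIController and caches it for later runs.
; An AI MoveTo with a small acceptance radius drives the pawn.
; Both success and failure print the result and finish the task as successful, alongside other debug prints.
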(event `self.ReceiveExecute`
  (params (OwnerActor :type "Actor Object Reference"))
  (bind _returnvalue (`BTFunctionLibrary.GetBlackboardValueAsActor` (`self.TargetToFollow`)))
  (if (!= (`self.AIControllerReference`) null)
    (`KismetSystemLibrary.PrintString` "Hello")
    (else
      (bind _asbp_stalker_aicontroller (cast `/Game/Blueprints/Stalker/BP_StalkerAIController` OwnerActor))
      (`KismetSystemLibrary.PrintString` "Initial set of AIController")
      (set `self.AIControllerReference` _asbp_stalker_aicontroller)))
  (bind _movementresult (`|AIMoveTo` (`Controller.K2_GetPawn` (`self.AIControllerReference`)) (`Actor.K2_GetActorLocation` _returnvalue) _returnvalue 50.0)
    (:`OnSuccess`
      _)
    (:`OnFail`
      _))
  (`KismetSystemLibrary.PrintString` (`|GetEnumeratorNameAsString` _movementresult))
  (`self.FinishExecute` true))