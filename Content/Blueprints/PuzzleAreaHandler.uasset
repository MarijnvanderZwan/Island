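; PuzzleAreaHandler tracks completion of the puzzles linked to one puzzle area.
; On BeginPlay it maps linked identifiers to BP_Puzzle actors and binds to the GlobalPuzzleHandler's puzzle-completed dispatcher, which flags matching puzzles as done.
; CheckAreaCompletion, not called within this graph, fires the global area-completed dispatcher once when all tracked puzzles are done.
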(event `self.ReceiveBeginPlay`
  (bind _outactors (`GameplayStatics.GetAllActorsOfClass` "/Game/Blueprints/GlobalPuzzleHandler.GlobalPuzzleHandler_C"))
  (bind _output_get (set `self.GlobalPuzzleHandler` (`|GetArrayItem` _outactors)))
  (add `/Game/Blueprints/GlobalPuzzleHandler.PuzzleCompletedDispatcher` _output_get (delegate `PuzzleCompleted`))
  (bind _outactors_2 (`GameplayStatics.GetAllActorsOfClass` "/Game/Blueprints/GenericPuzzle/BP_Puzzle.BP_Puzzle_C"))
  (for _array_element (`self.LinkedPuzzles`)
    (for _array_element_2 _outactors_2
      (bind _puzzleidentifier (`/Game/Blueprints/GenericPuzzle/BP_Puzzle.PuzzleIdentifier` _array_element_2))
      (if (`|EnumEquality` _puzzleidentifier _array_element)
        (`BlueprintMapLibrary.Map_Add` (`self.Puzzles`) _puzzleidentifier _array_element_2)
        (`BlueprintMapLibrary.Map_Add` (`self.PuzzlesCompleted`) _puzzleidentifier)
        (break)))))

(event `PuzzleCompleted`
  (params (PuzzleIdentifier :type "/Game/Blueprints/Puzzles/PuzzleIdentifier Enum" :default "NewEnumerator0"))
  (bind _puzzlescompleted (`self.PuzzlesCompleted`))
  (if (`BlueprintMapLibrary.Map_Contains` _puzzlescompleted PuzzleIdentifier)
    (`BlueprintMapLibrary.Map_Add` _puzzlescompleted PuzzleIdentifier true)))

(event `CheckAreaCompletion`
  (if (not (`self.AreaCompleted`))
    (bind _completed (`self.CheckForCompletion`))
    (if _completed
      (set `self.AreaCompleted` true)
      (`/Game/Blueprints/GlobalPuzzleHandler.PuzzlesInAreaCompletedDispatcher` (`self.GlobalPuzzleHandler`) (`self.PuzzleAreaIndicator`)))))

(fn `CheckForCompletion`
  (returns (Completed :type Boolean))
  (bind _puzzlescompleted (`self.PuzzlesCompleted`))
  (bind _keys (`BlueprintMapLibrary.Map_Keys` _puzzlescompleted))
  (for _array_element _keys
    (if (not (`BlueprintMapLibrary.Map_Find` _puzzlescompleted _array_element))
      (return false)))
  (return true))

(fn `UserConstructionScript`)