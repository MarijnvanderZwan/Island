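; Manager for a pushable-block puzzle that triggers its Goal once every goal block is solved.
; It registers as Parent on each GoalBlock, keeps a count through IncrementSolved and DecrementSolved, and polls it on Tick.
; Completion latches Solved and shows a BP_DialogueSystem message; until then, ResetPuzzle returns PushableBlocks to their starting locations with a message.
; CreateBoundary is empty, with its mesh-spawning loops left disconnected.
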(event `self.ReceiveBeginPlay`
  (for _array_element (`self.GoalBlocks`)
    (set `/Game/Blueprints/BlockPuzzle/BP_GoalBlock.Parent` self _array_element)))

(event `self.ReceiveTick`
  (params (DeltaSeconds :type "Float (single-precision)"))
  (if (not (`self.Solved`))
    (if (== (`self.SolvedBlocks`) (`KismetArrayLibrary.Array_Length` (`self.GoalBlocks`)))
      (set `self.Solved` true)
      (`/Game/Blueprints/BP_Goal.GoalReached` (`self.Goal`))
      (bind _outactors (`GameplayStatics.GetAllActorsOfClass` "/Game/Blueprints/BP_DialogueSystem.BP_DialogueSystem_C"))
      (`/Game/Blueprints/BP_DialogueSystem.ShowMessage` (`KismetArrayLibrary.Array_Get` _outactors) "Puzzle completed!"))))

(event `ResetPuzzle`
  (if (not (`self.Solved`))
    (for _array_element (`self.PushableBlocks`)
      (`/Game/Blueprints/BlockPuzzle/BP_PushableBlock.ResetToStartingLocation` _array_element)
      (bind _outactors (`GameplayStatics.GetAllActorsOfClass` "/Game/Blueprints/BP_DialogueSystem.BP_DialogueSystem_C"))
      (`/Game/Blueprints/BP_DialogueSystem.ShowMessage` (`KismetArrayLibrary.Array_Get` _outactors) "Reset Puzzle"))))

(fn `CreateBoundary`)

(fn `DecrementSolved`
  (set `self.SolvedBlocks` (- (`self.SolvedBlocks`) 1)))

(fn `IncrementSolved`
  (set `self.SolvedBlocks` (+ (`self.SolvedBlocks`) 1)))

(fn `UserConstructionScript`
  (`parent.UserConstructionScript`))