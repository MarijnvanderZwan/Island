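; BP_Hermes is a goal trigger in the block puzzle, tracking whether a pushable block sits in its box.
; On construction it finds the first BP_BlockPuzzle in the level, registers as a goal block and stores it as Parent.
; When a BP_PushableBlock enters or leaves the box, it toggles its Active flag, swaps that block's blue rune material and increments or decrements the puzzle's solved count.
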(event `self.ReceiveBeginPlay`)

(event `self.ReceiveTick`
  (params (DeltaSeconds :type "Float (single-precision)")))

(event `self.Box.OnComponentBeginOverlap`
  (params (OverlappedComponent :type "PrimitiveComponent Object Reference") (OtherActor :type "Actor Object Reference") (OtherComp :type "PrimitiveComponent Object Reference") (OtherBodyIndex :type Integer) (bFromSweep :type Boolean) (SweepResult :type "HitResult Structure (by ref)"))
  (if (not (`self.Active`))
    (bind _asbp_pushable_block (cast `/Game/Blueprints/BlockPuzzle/BP_PushableBlock` OtherActor))
    (set `self.Active` true)
    (`PrimitiveComponent.SetMaterial` (`DefaultPawn.MeshComponent` _asbp_pushable_block) 0 "/Game/Materials/M_BlockBlueRune.M_BlockBlueRune")
    (`/Game/Blueprints/BP_BlockPuzzle.IncrementSolved` (`self.Parent`))))

(event `self.Box.OnComponentEndOverlap`
  (params (OverlappedComponent :type "PrimitiveComponent Object Reference") (OtherActor :type "Actor Object Reference") (OtherComp :type "PrimitiveComponent Object Reference") (OtherBodyIndex :type Integer))
  (if (`self.Active`)
    (bind _asbp_pushable_block (cast `/Game/Blueprints/BlockPuzzle/BP_PushableBlock` OtherActor))
    (set `self.Active` false)
    (`PrimitiveComponent.SetMaterial` (`DefaultPawn.MeshComponent` _asbp_pushable_block) 0 "/Game/Materials/M_BlockBlueRune_off.M_BlockBlueRune_off")
    (`/Game/Blueprints/BP_BlockPuzzle.DecrementSolved` (`self.Parent`))))

(fn `UserConstructionScript`
  (bind _outactors (`GameplayStatics.GetAllActorsOfClass` "/Game/Blueprints/BP_BlockPuzzle.BP_BlockPuzzle_C"))
  (bind _item (`KismetArrayLibrary.Array_Get` _outactors))
  (`/Game/Blueprints/BP_BlockPuzzle.RegisterGoalBlock` _item self)
  (set `self.Parent` _item))