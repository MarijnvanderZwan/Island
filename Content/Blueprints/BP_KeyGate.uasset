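; BP_KeyGate is a key gate actor that tracks an opened state and plays its animation through open and close events.
; Its InteractionArea registers the gate as the player's OverlappingKeyGate on overlap while it is not opened, and clears that reference on exit.
; SetGateOpen also swaps a mesh material to M_Key1.
; SetGateClosed replays the same animation forward and leaves the material unchanged.
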(event `SetGateOpen`
  (`SkeletalMeshComponent.PlayAnimation` (`self.SkeletalMesh`) "/Game/Meshes/Animated/KeyGate_Anim.KeyGate_Anim" false)
  (set `self.Opened` true)
  (`PrimitiveComponent.SetMaterial` (`self.SkeletalMesh`) 1 "/Game/Materials/M_Key1.M_Key1"))

(event `SetGateClosed`
  (`SkeletalMeshComponent.PlayAnimation` (`self.SkeletalMesh`) "/Game/Meshes/Animated/KeyGate_Anim.KeyGate_Anim" false)
  (set `self.Opened` false))

(event `self.Interaction area.OnComponentBeginOverlap`
  (params (OverlappedComponent :type "PrimitiveComponent Object Reference") (OtherActor :type "Actor Object Reference") (OtherComp :type "PrimitiveComponent Object Reference") (OtherBodyIndex :type Integer) (bFromSweep :type Boolean) (SweepResult :type "HitResult Structure (by ref)"))
  (if (not (`self.Opened`))
    (bind _asbp_player (cast `/Game/Blueprints/BP_Player` OtherActor))
    (set `/Game/Blueprints/BP_Player.OverlappingKeyGate` self _asbp_player)))

(event `self.Interaction area.OnComponentEndOverlap`
  (params (OverlappedComponent :type "PrimitiveComponent Object Reference") (OtherActor :type "Actor Object Reference") (OtherComp :type "PrimitiveComponent Object Reference") (OtherBodyIndex :type Integer))
  (bind _asbp_player (cast `/Game/Blueprints/BP_Player` OtherActor))
  (set `/Game/Blueprints/BP_Player.OverlappingKeyGate` null _asbp_player))

(fn `UserConstructionScript`)