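; BP_Button is a trigger button that reacts when the player steps on or off it.
; Overlap events with BP_Player set a CurrentlyOverlappingPlayer flag and call ButtonActivated or ButtonDeactivated on a BP_ButtonHandler child actor.
; The construction script passes a self reference to that handler so it knows its owning button.
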(event `self.ReceiveActorBeginOverlap`
  (params (OtherActor :type "Actor Object Reference"))
  (cast `/Game/Blueprints/BP_Player` OtherActor)
  (set `self.CurrentlyOverlappingPlayer` true)
  (bind _asbp_button_handler (cast `/Game/Blueprints/Buttons/BP_ButtonHandler` (`ChildActorComponent.ChildActor` (`self.ButtonHandler`))))
  (`/Game/Blueprints/Buttons/BP_ButtonHandler.ButtonActivated` _asbp_button_handler))

(event `self.ReceiveActorEndOverlap`
  (params (OtherActor :type "Actor Object Reference"))
  (cast `/Game/Blueprints/BP_Player` OtherActor)
  (set `self.CurrentlyOverlappingPlayer` false)
  (bind _asbp_button_handler (cast `/Game/Blueprints/Buttons/BP_ButtonHandler` (`ChildActorComponent.ChildActor` (`self.ButtonHandler`))))
  (`/Game/Blueprints/Buttons/BP_ButtonHandler.ButtonDeactivated` _asbp_button_handler))

(fn `UserConstructionScript`
  (bind _asbp_button_handler (cast `/Game/Blueprints/Buttons/BP_ButtonHandler` (`ChildActorComponent.ChildActor` (`self.ButtonHandler`))))
  (set `/Game/Blueprints/Buttons/BP_ButtonHandler.Button` self _asbp_button_handler))