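; BP_BlockButtonHandler is a button handler Blueprint that moves the block belonging to a BP_BlockButton when that button changes state.
; Its activated and deactivated events each cast the Button reference to BP_BlockButton and set the Block component's relative location.
; The block snaps between two fixed heights, lower when activated, with no sweep or interpolation.
; The construction script only calls its parent.
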(event `self.ButtonActivated`
  (bind _asbp_block_button (cast `/Game/Blueprints/Buttons/BP_BlockButton` (`self.Button`)))
  (`SceneComponent.K2_SetRelativeLocation` (`/Game/Blueprints/Buttons/BP_BlockButton.Block` _asbp_block_button) (0.0 0.0 -300.0) false false))

(event `self.ButtonDeactivated`
  (bind _asbp_block_button (cast `/Game/Blueprints/Buttons/BP_BlockButton` (`self.Button`)))
  (`SceneComponent.K2_SetRelativeLocation` (`/Game/Blueprints/Buttons/BP_BlockButton.Block` _asbp_block_button) (0.0 0.0 -250.0) false false))

(fn `UserConstructionScript`
  (`parent.UserConstructionScript`))