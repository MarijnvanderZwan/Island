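; A totem goal element that displays coin collection progress and puzzle completion as a vertical stack of meshes.
; On BeginPlay it spawns one static mesh per coin to collect, plus a completion mesh on top.
; CoinCollected increments the count and turns the mesh at that new index emerald, while PuzzleSolved does the same to the top mesh.
; PlayerDied is an empty handler.
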(event `self.ReceiveBeginPlay`
  (bind _coinstocollect (`self.CoinsToCollect`))
  (for _index (range _coinstocollect)
    (bind _returnvalue (`AddComponent|NODE_AddStaticMeshComponent-0` :`RelativeTransform` (`KismetMathLibrary.MakeTransform` (* (0.0 0.0 120.0) _index) (struct) (0.5 0.5 0.5))))
    (`KismetArrayLibrary.Array_Add` (`self.CoinMeshes`) _returnvalue))
  (bind _returnvalue_2 (`AddComponent|NODE_AddStaticMeshComponent-1` :`RelativeTransform` (`KismetMathLibrary.MakeTransform` (* (0.0 0.0 120.0) _coinstocollect) (struct) (0.5 0.5 0.5))))
  (set `self.CompletedMesh` _returnvalue_2))

(event `self.PuzzleSolved`
  (`PrimitiveComponent.SetMaterial` (`self.CompletedMesh`) 0 "/Game/Materials/M_Emerald.M_Emerald"))

(event `Coin Collected`
  (bind _output_get (set `self.CoinsCollected` (+ (`self.CoinsCollected`) 1)))
  (`PrimitiveComponent.SetMaterial` (`|GetArrayItem` (`self.CoinMeshes`) _output_get) 0 "/Game/Materials/M_Emerald.M_Emerald"))

(event `PlayerDied`)

(fn `UserConstructionScript`)