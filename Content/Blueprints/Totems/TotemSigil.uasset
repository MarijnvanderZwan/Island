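; TotemSigil is a totem sigil Blueprint that displays a symbol through two decals and tracks whether it is active.
; SetActive and SetInactive toggle the visibility of the Activated component, without propagating to its children, and update the Active flag to match.
; SetDecalMaterial stores the supplied material and applies it to both decal components.
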(event `SetActive`
  (`SceneComponent.SetVisibility` (`self.Activated`) true false)
  (set `self.Active` true))

(event `SetInactive`
  (`SceneComponent.SetVisibility` (`self.Activated`) false false)
  (set `self.Active` false))

(event `SetDecalMaterial`
  (params (DecalMaterial :type "MaterialInstance Object Reference"))
  (bind _output_get (set `self.DecalMaterial` DecalMaterial))
  (`DecalComponent.SetDecalMaterial` (`self.Decal2`) _output_get)
  (`DecalComponent.SetDecalMaterial` (`self.Decal1`) _output_get))

(fn `UserConstructionScript`)