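; BP_BlockWall is an actor that builds a wall of blocks as a 3D grid sized by Width, Depth, Height and CellSize.
; The Construction Script calls CreateGrid, whose nested loops add a separate static mesh component for each cell.
; GetTopLeft supplies an offset that centers the grid on the actor in X and Y, while layers stack upward from Z zero.
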(event `self.ReceiveBeginPlay`)

(fn `CreateGrid`
  (bind _cellsize (`self.CellSize`))
  (bind _topleft (`self.GetTopLeft`))
  (for _index (range 1 (+ (`self.Depth`) 1))
    (for _index_2 (range 1 (+ (`self.Width`) 1))
      (for _index_3 (range (`self.Height`))
        (`AddComponent|StaticMeshComponent_17` :`RelativeTransform` (`KismetMathLibrary.MakeTransform` (+ _topleft (`KismetMathLibrary.MakeVector` (* _index_2 _cellsize) (* _index _cellsize) (* _index_3 _cellsize))) (struct) (1.0 1.0 1.0)))))))

(fn `GetTopLeft`
  (returns (TopLeft :type "Vector Structure"))
  (return (`KismetMathLibrary.MakeVector` (* (+ (`KismetMathLibrary.Conv_IntToDouble` (`self.Width`)) 1.0) (`self.CellSize`) -0.5) (* (+ (`KismetMathLibrary.Conv_IntToDouble` (`self.Depth`)) 1.0) (`self.CellSize`) -0.5))))

(fn `UserConstructionScript`
  (`self.CreateGrid`))