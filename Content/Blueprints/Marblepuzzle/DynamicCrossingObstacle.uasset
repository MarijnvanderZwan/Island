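; A lever-operated crossing obstacle for the marble puzzle that the player flips between two mirrored orientations.
; A Sphere overlap tracks when BP_Player is in range, enabling the Action input to call LeverToggle.
; LeverToggle negates the obstacle's world yaw, prints a debug message and plays the up or down lever animation based on the yaw sign.
; An unconnected node for rotating the whole actor a quarter turn never runs.
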(event `InputAction|Action` :consume false
  (params (Key :type "Key Structure" :default "AnyKey"))
  (:`Pressed`
    (if (`self.OverlappingPlayer`)
      (`self.LeverToggle`))))

(event `LeverToggle`
  (bind _dynamicobstacle (`self.DynamicObstacle`))
  (bind _lever (`self.Lever`))
  (bind (_returnvalue_roll _returnvalue_pitch _returnvalue_yaw) (`KismetMathLibrary.BreakRotator` (`SceneComponent.K2_GetComponentRotation` _dynamicobstacle)))
  (bind _returnvalue (* _returnvalue_yaw -1.0))
  (`SceneComponent.K2_SetWorldRotation` _dynamicobstacle (`KismetMathLibrary.MakeRotator` _returnvalue_roll _returnvalue_pitch _returnvalue) false false)
  (`KismetSystemLibrary.PrintString` "Toggled lever")
  (if (< _returnvalue 0.0)
    (`SkeletalMeshComponent.PlayAnimation` _lever "/Game/Animations/lever_Down.lever_Down" false)
    (else
      (`SkeletalMeshComponent.PlayAnimation` _lever "/Game/Animations/lever_Up.lever_Up" false))))

(event `self.Sphere.OnComponentBeginOverlap`
  (params (OverlappedComponent :type "PrimitiveComponent Object Reference") (OtherActor :type "Actor Object Reference") (OtherComp :type "PrimitiveComponent Object Reference") (OtherBodyIndex :type Integer) (bFromSweep :type Boolean) (SweepResult :type "HitResult Structure (by ref)"))
  (cast `/Game/Blueprints/BP_Player` OtherActor)
  (set `self.OverlappingPlayer` true))

(event `self.Sphere.OnComponentEndOverlap`
  (params (OverlappedComponent :type "PrimitiveComponent Object Reference") (OtherActor :type "Actor Object Reference") (OtherComp :type "PrimitiveComponent Object Reference") (OtherBodyIndex :type Integer))
  (cast `/Game/Blueprints/BP_Player` OtherActor)
  (set `self.OverlappingPlayer` false))

(fn `UserConstructionScript`)