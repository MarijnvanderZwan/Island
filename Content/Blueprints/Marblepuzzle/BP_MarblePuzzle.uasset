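; BP_MarblePuzzle is a marble puzzle actor with a lever that spawns a rolling ball and a goal flag that marks completion.
; Pressing the action input while the player overlaps the Sphere replaces any existing ball with a new one at the Cube's location and animates the lever down, then up.
; Every Tick it recounts unachieved Goals and, at zero, sets the child-actor BP_GoalFlag completed if it is not already.
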(event `LeverToggle`
  (bind _ball (`self.Ball`))
  (if (!= _ball null)
    (`self.K2_DestroyActor` _ball))
  (bind _returnvalue (`|SpawnActorFromClass` "/Game/Blueprints/Marblepuzzle/RollingBall.RollingBall_C" (`KismetMathLibrary.MakeTransform` (`SceneComponent.K2_GetComponentLocation` (`self.Cube`))) "AlwaysSpawn" "OverrideRootScale"))
  (set `self.Ball` _returnvalue)
  (`SkeletalMeshComponent.PlayAnimation` (`self.Lever`) "/Game/Animations/lever_Down.lever_Down" false)
  (`KismetSystemLibrary.Delay` 1.2)
  (`SkeletalMeshComponent.PlayAnimation` (`self.Lever`) "/Game/Animations/lever_Up.lever_Up" false))

(event `InputAction|Action` :consume false
  (params (Key :type "Key Structure" :default "AnyKey"))
  (:`Pressed`
    (if (`self.OverlappingPlayer`)
      (`self.LeverToggle`))))

(event `self.ReceiveTick`
  (params (DeltaSeconds :type "Float (single-precision)"))
  (`self.ComputeNUncompletedGoals`)
  (if (== (`self.nUncompletedGoals`) 0)
    (bind _asbp_goal_flag (cast `/Game/Blueprints/BP_GoalFlag` (`ChildActorComponent.ChildActor` (`self.GoalFlag`))))
    (if (not (`/Game/Blueprints/BP_GoalFlag.Completed` _asbp_goal_flag))
      (`/Game/Blueprints/BP_GoalFlag.SetCompleted` _asbp_goal_flag))))

(event `self.Sphere.OnComponentBeginOverlap`
  (params (OverlappedComponent :type "PrimitiveComponent Object Reference") (OtherActor :type "Actor Object Reference") (OtherComp :type "PrimitiveComponent Object Reference") (OtherBodyIndex :type Integer) (bFromSweep :type Boolean) (SweepResult :type "HitResult Structure (by ref)"))
  (cast `/Game/Blueprints/BP_Player` OtherActor)
  (set `self.OverlappingPlayer` true))

(event `self.Sphere.OnComponentEndOverlap`
  (params (OverlappedComponent :type "PrimitiveComponent Object Reference") (OtherActor :type "Actor Object Reference") (OtherComp :type "PrimitiveComponent Object Reference") (OtherBodyIndex :type Integer))
  (cast `/Game/Blueprints/BP_Player` OtherActor)
  (set `self.OverlappingPlayer` false))

(fn `ComputeNUncompletedGoals`
  (set `self.nUncompletedGoals` 0)
  (for _array_element (`self.Goals`)
    (if (not (`/Game/Blueprints/Marblepuzzle/BP_MarbleGoal.GoalAchieved` _array_element))
      (set `self.nUncompletedGoals` (+ (`self.nUncompletedGoals`) 1)))))

(fn `UserConstructionScript`)