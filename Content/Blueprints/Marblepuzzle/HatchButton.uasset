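; HatchButton is a marble puzzle button that opens a hatch for a limited time.
; PushButton calls HatchOpened on the BP_Luik child actor in its Hatch component and starts a countdown from HatchOpenTime.
; Tick decrements the timer while the hatch is open, then calls HatchClosed on that actor when time runs out.
; Pushing again restarts the countdown.
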(event `self.ReceiveTick`
  (params (DeltaSeconds :type "Float (single-precision)"))
  (if (`self.HatchOpened`)
    (bind _output_get (set `self.TimeToHatchClosed` (- (`self.TimeToHatchClosed`) DeltaSeconds)))
    (if (< _output_get 0.0)
      (bind _asbp_luik (cast `/Game/Blueprints/Marblepuzzle/BP_Luik` (`ChildActorComponent.ChildActor` (`self.Hatch`))))
      (`/Game/Blueprints/Marblepuzzle/BP_Luik.HatchClosed` _asbp_luik)
      (set `self.HatchOpened` false))))

(event `PushButton`
  (bind _asbp_luik (cast `/Game/Blueprints/Marblepuzzle/BP_Luik` (`ChildActorComponent.ChildActor` (`self.Hatch`))))
  (`/Game/Blueprints/Marblepuzzle/BP_Luik.HatchOpened` _asbp_luik)
  (set `self.HatchOpened` true)
  (set `self.TimeToHatchClosed` (`self.HatchOpenTime`)))

(fn `UserConstructionScript`)