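; BP_Luik is a hatch for the marble puzzle that either blocks or opens a path and shows its state with a rotating indicator.
; HatchOpened and HatchClosed set the target roll and Enabled flag, and toggle the collision component's collision and visibility.
; Tick turns the LuikAanwijzer component toward that target at a constant speed, clamped so it does not overshoot.
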(event `self.ReceiveTick`
  (params (DeltaSeconds :type "Float (single-precision)"))
  (bind _returnvalue (* DeltaSeconds 100.0))
  (bind _targetrotation (`self.TargetRotation`))
  (bind _luik_aanwijzer (`self.Luik_Aanwijzer`))
  (bind _relativerotation_roll (`KismetMathLibrary.BreakRotator` (`SceneComponent.RelativeRotation` (`self.Luik_Aanwijzer`))))
  (if (< _relativerotation_roll _targetrotation)
    (`SceneComponent.K2_SetRelativeRotation` _luik_aanwijzer (`KismetMathLibrary.MakeRotator` (`KismetMathLibrary.FMin` (+ _relativerotation_roll _returnvalue) (`self.TargetRotation`))) false false)
    (elif (> _relativerotation_roll _targetrotation)
      (`SceneComponent.K2_SetRelativeRotation` _luik_aanwijzer (`KismetMathLibrary.MakeRotator` (`KismetMathLibrary.FMax` (- _relativerotation_roll _returnvalue) (`self.TargetRotation`))) false false))))

(event `HatchOpened`
  (set `self.TargetRotation` 90.0)
  (set `self.Enabled` true)
  (`PrimitiveComponent.SetCollisionEnabled` (`self.Luik_Collission`) "NoCollision")
  (`SceneComponent.SetVisibility` (`self.Luik_Collission`) false false))

(event `HatchClosed`
  (bind _luik_collission (`self.Luik_Collission`))
  (set `self.TargetRotation` 0.0)
  (set `self.Enabled` false)
  (`PrimitiveComponent.SetCollisionEnabled` _luik_collission "QueryAndPhysics")
  (`PrimitiveComponent.SetCollisionResponseToChannel` _luik_collission "ECC_WorldDynamic" "ECR_Block")
  (`SceneComponent.SetVisibility` (`self.Luik_Collission`) true false))

(fn `UserConstructionScript`)