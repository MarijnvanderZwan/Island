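; BP_MarbleSpawner is an interactable spawner for the marble puzzle that creates RollingBall actors.
; A Sphere overlap tracks whether a BP_Player is in range through the OverlappingPlayer flag.
; Pressing the Action input while in range calls LeverToggle, which spawns a new ball at the Cube component's world transform.
; The spawner sets no limit on ball count and keeps no reference to spawned balls.
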(event `LeverToggle`
  (`|SpawnActorFromClass` "/Game/Blueprints/Marblepuzzle/RollingBall.RollingBall_C" (`SceneComponent.K2_GetComponentToWorld` (`self.Cube`)) "Undefined" "OverrideRootScale"))

(event `InputAction|Action` :consume false
  (params (Key :type "Key Structure" :default "AnyKey"))
  (:`Pressed`
    (if (`self.OverlappingPlayer`)
      (`self.LeverToggle`))))

(event `self.Sphere.OnComponentBeginOverlap`
  (params (OverlappedComponent :type "PrimitiveComponent Object Reference") (OtherActor :type "Actor Object Reference") (OtherComp :type "PrimitiveComponent Object Reference") (OtherBodyIndex :type Integer) (bFromSweep :type Boolean) (SweepResult :type "HitResult Structure (by ref)"))
  (cast `/Game/Blueprints/BP_Player` OtherActor)
  (set `self.OverlappingPlayer` true))

(event `self.Sphere.OnComponentEndOverlap`
  (params (OverlappedComponent :type "PrimitiveComponent Object Reference") (OtherActor :type "Actor Object Reference") (OtherComp :type "PrimitiveComponent Object Reference") (OtherBodyIndex :type Integer))
  (cast `/Game/Blueprints/BP_Player` OtherActor)
  (set `self.OverlappingPlayer` false))

(fn `UserConstructionScript`)