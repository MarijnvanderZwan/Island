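; Block-pushing puzzle manager that builds a centred floor grid and detects when every goal block is solved.
; The construction script lays meshes from Width, Depth and CellSize; a CreateBoundary helper exists but is not called here.
; Goal and pushable blocks register through functions, while Tick compares the solved counter to the goal count, then triggers Goal and a dialogue message.
; ResetPuzzle returns pushable blocks to their starts until solved.
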(event `self.ReceiveBeginPlay`)

(event `self.ReceiveTick`
  (params (DeltaSeconds :type "Float (single-precision)"))
  (if (not (`self.Solved`))
    (if (== (`self.SolvedBlocks`) (`KismetArrayLibrary.Array_Length` (`self.GoalBlocks`)))
      (set `self.Solved` true)
      (`/Game/Blueprints/BP_Goal.GoalReached` (`self.Goal`))
      (bind _outactors (`GameplayStatics.GetAllActorsOfClass` "/Game/Blueprints/BP_DialogueSystem.BP_DialogueSystem_C"))
      (`/Game/Blueprints/BP_DialogueSystem.ShowMessage` (`KismetArrayLibrary.Array_Get` _outactors) "Puzzle completed!"))))

(event `ResetPuzzle`
  (if (not (`self.Solved`))
    (for _array_element (`self.PushableBlocks`)
      (bind _asbp_pushable_block (cast `/Game/Blueprints/BP_PushableBlock` _array_element))
      (`/Game/Blueprints/BP_PushableBlock.ResetToStartingLocation` _asbp_pushable_block)
      (bind _outactors (`GameplayStatics.GetAllActorsOfClass` "/Game/Blueprints/BP_DialogueSystem.BP_DialogueSystem_C"))
      (`/Game/Blueprints/BP_DialogueSystem.ShowMessage` (`KismetArrayLibrary.Array_Get` _outactors) "Reset Puzzle"))))

(fn `CreateBoundary`
  (bind _topleft (`self.GetTopLeft`))
  (for _index (range (+ (+ (`self.Depth`) 1) 1))
    (bind _returnvalue (* _index (`self.CellSize`)))
    (`AddComponent|StaticMeshComponent_1` :`RelativeTransform` (`KismetMathLibrary.MakeTransform` (+ _topleft (`KismetMathLibrary.MakeVector` 0.0 _returnvalue)) (struct) (1.0 1.0 1.0)))
    (`AddComponent|StaticMeshComponent_2` :`RelativeTransform` (`KismetMathLibrary.MakeTransform` (+ (`KismetMathLibrary.MakeVector` (* (+ (`self.Width`) 1) (`self.CellSize`)) _returnvalue) _topleft) (struct) (1.0 1.0 1.0))))
  (bind _topleft_2 (`self.GetTopLeft`))
  (for _index_2 (range 1 (+ (`self.Width`) 1))
    (bind _returnvalue_2 (* _index_2 (`self.CellSize`)))
    (`AddComponent|StaticMeshComponent_3` :`RelativeTransform` (`KismetMathLibrary.MakeTransform` (+ _topleft_2 (`KismetMathLibrary.MakeVector` _returnvalue_2 (* (+ (`self.Depth`) 1) (`self.CellSize`)))) (struct) (1.0 1.0 1.0)))
    (`AddComponent|StaticMeshComponent_4` :`RelativeTransform` (`KismetMathLibrary.MakeTransform` (+ (`KismetMathLibrary.MakeVector` _returnvalue_2) _topleft_2) (struct) (1.0 1.0 1.0)))))

(fn `CreateGrid`
  (bind _cellsize (`self.CellSize`))
  (for _index (range 1 (+ (`self.Depth`) 1))
    (for _index_2 (range 1 (+ (`self.Width`) 1))
      (bind _topleft (`self.GetTopLeft`))
      (`AddComponent|StaticMeshComponent_0` :`RelativeTransform` (`KismetMathLibrary.MakeTransform` (+ _topleft (`KismetMathLibrary.MakeVector` (* _index_2 _cellsize) (* _index _cellsize))) (struct) (1.0 1.0 1.0))))))

(fn `DecrementSolved`
  (set `self.SolvedBlocks` (- (`self.SolvedBlocks`) 1)))

(fn `GetTopLeft`
  (returns (TopLeft :type "Vector Structure"))
  (return (`KismetMathLibrary.MakeVector` (* (+ (`KismetMathLibrary.Conv_IntToDouble` (`self.Width`)) 1.0) (`self.CellSize`) -0.5) (* (+ (`KismetMathLibrary.Conv_IntToDouble` (`self.Depth`)) 1.0) (`self.CellSize`) -0.5))))

(fn `IncrementSolved`
  (set `self.SolvedBlocks` (+ (`self.SolvedBlocks`) 1)))

(fn `RegisterGoalBlock`
  (params (Target :type "/Game/Blueprints/BP_Hermes Object Reference"))
  (`KismetArrayLibrary.Array_Add` (`self.GoalBlocks`) Target)
  (`KismetSystemLibrary.PrintString` (`KismetStringLibrary.Conv_IntToString` (`KismetArrayLibrary.Array_Length` (`self.GoalBlocks`)))))

(fn `RegisterPushableblock`
  (params (NewParam :type "Actor Object Reference"))
  (`KismetArrayLibrary.Array_Add` (`self.PushableBlocks`) NewParam))

(fn `UserConstructionScript`
  (`self.CreateGrid`))