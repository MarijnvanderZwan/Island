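; Decoration Blueprint that repeats a static mesh along a spline, built in the construction script.
; It adds mesh components at MeshSize intervals, offset from the actor location and rotated only in yaw to follow the spline plus RotationYawOffset.
; A final mesh sits at the spline end, Y-scaled to the leftover fraction of MeshSize and using the yaw of the last whole step.
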(fn `UserConstructionScript`
  (bind _spline (`self.Spline`))
  (bind _spline_2 (`self.Spline`))
  (bind _meshsize (`self.MeshSize`))
  (bind _returnvalue (`SplineComponent.GetSplineLength` _spline))
  (bind _returnvalue_2 (`KismetMathLibrary.FTrunc` (/ (`SplineComponent.GetSplineLength` (`self.Spline`)) (`self.MeshSize`))))
  (bind _returnvalue_3 (* _returnvalue_2 _meshsize))
  (bind (_returnvalue_roll _returnvalue_pitch _returnvalue_yaw) (`KismetMathLibrary.BreakRotator` (`SplineComponent.GetRotationAtDistanceAlongSpline` _spline _returnvalue_3 "Local")))
  (for _index (range (+ _returnvalue_2 1))
    (bind _returnvalue_4 (* _index (`self.MeshSize`)))
    (bind (_returnvalue_roll_2 _returnvalue_pitch_2 _returnvalue_yaw_2) (`KismetMathLibrary.BreakRotator` (`SplineComponent.GetRotationAtDistanceAlongSpline` _spline_2 _returnvalue_4 "Local")))
    (`AddComponent|NODE_AddStaticMeshComponent-0` :`RelativeTransform` (`KismetMathLibrary.MakeTransform` (- (`SplineComponent.GetLocationAtDistanceAlongSpline` _spline_2 _returnvalue_4 "World") (`self.K2_GetActorLocation`)) (`KismetMathLibrary.MakeRotator` 0.0 0.0 (+ _returnvalue_yaw_2 (`self.RotationYawOffset`))))))
  (`AddComponent|NODE_AddStaticMeshComponent-3` :`RelativeTransform` (`KismetMathLibrary.MakeTransform` (- (`SplineComponent.GetLocationAtDistanceAlongSpline` _spline _returnvalue "World") (`self.K2_GetActorLocation`)) (`KismetMathLibrary.MakeRotator` 0.0 0.0 (+ _returnvalue_yaw (`self.RotationYawOffset`))) (`KismetMathLibrary.MakeVector` 1.0 (/ (- _returnvalue _returnvalue_3) _meshsize) 1.0))))