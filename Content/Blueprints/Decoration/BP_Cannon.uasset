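; BP_Cannon is an interactable decorative cannon that fires a BP_Cannonball when used.
; InteractwithObject calls Fire, which spawns the ball at the Arrow component, sets its velocity to max speed, activates the particle system and plays a sound.
; Tick then animates recoil along the negative forward vector on a half-sine curve, returning to the position saved at BeginPlay.
; Fire is ignored until the recoil finishes.
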(event `self.ReceiveBeginPlay`
  (set `self.OriginalWorldPosition` (`self.K2_GetActorLocation`)))

(event `self.ReceiveTick`
  (params (DeltaSeconds :type "Float (single-precision)"))
  (bind _timetoanimate (`self.TimeToAnimate`))
  (if (`self.AnimationPlaying`)
    (bind _output_get (set `self.TimeAnimated` (+ (`self.TimeAnimated`) DeltaSeconds)))
    (if (< _output_get _timetoanimate)
      (`self.K2_SetActorLocation` (+ (* (* (`self.GetActorForwardVector`) (* (`self.AnimationDistance`) (`KismetMathLibrary.Sin` (* (/ _output_get _timetoanimate) 3.14)))) -1.0) (`self.OriginalWorldPosition`)) false true)
      (else
        (set `self.AnimationPlaying` false)
        (`self.K2_SetActorLocation` (`self.OriginalWorldPosition`) false true)
        (set `self.TimeAnimated` 0.0)))))

(event `Fire`
  (bind _arrow (`self.Arrow`))
  (if (not (`self.AnimationPlaying`))
    (bind _returnvalue (`|SpawnActorFromClass` "/Game/Blueprints/Decoration/BP_Cannonball.BP_Cannonball_C" (`KismetMathLibrary.MakeTransform` (`SceneComponent.K2_GetComponentLocation` _arrow) (`SceneComponent.K2_GetComponentRotation` _arrow)) "Undefined" "OverrideRootScale" null null))
    (bind _projectilemovement (`/Game/Blueprints/Decoration/BP_Cannonball.ProjectileMovement` _returnvalue))
    (`ProjectileMovementComponent.SetVelocityInLocalSpace` _projectilemovement (* (`SceneComponent.GetForwardVector` _arrow) (`MovementComponent.GetMaxSpeed` _projectilemovement)))
    (`ActorComponent.Activate` (`self.ParticleSystem`) true)
    (set `self.AnimationPlaying` true)
    (`GameplayStatics.PlaySoundAtLocation` "/Game/Audio/Effect/Cannon.Cannon" (`self.OriginalWorldPosition`) (struct) 1.0 1.0 0.0 null null null)))

(event `/Game/Blueprints/Gameplay/InteractableObject.InteractWithObject`
  (params (TriggerLocation :type "Vector Structure"))
  (`self.Fire`))

(fn `UserConstructionScript`)