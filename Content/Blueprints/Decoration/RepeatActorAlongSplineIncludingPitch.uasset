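; Decoration Blueprint that repeats a chosen static mesh along a spline, built entirely in the construction script.
; It spawns mesh components at intervals of mesh size times object scale, positioned from the spline and rotated by its yaw plus an offset.
; An extra piece at the spline's end is scaled on Y to the leftover length.
; Despite the asset name, spline pitch is not applied.
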(fn `NewFunction_0`)

(fn `UserConstructionScript`
  (bind _spline (`self.Spline`))
  (bind _spline_2 (`self.Spline`))
  (bind _returnvalue (`SplineComponent.GetSplineLength` _spline))
  (bind _returnvalue_2 (* (`self.MeshSize`) (`self.ObjectScale`)))
  (bind _returnvalue_3 (`KismetMathLibrary.FTrunc` (/ (`SplineComponent.GetSplineLength` (`self.Spline`)) (* (`self.MeshSize`) (`self.ObjectScale`)))))
  (bind _returnvalue_4 (* _returnvalue_3 _returnvalue_2))
  (bind (_returnvalue_roll _returnvalue_pitch _returnvalue_yaw) (`KismetMathLibrary.BreakRotator` (`SplineComponent.GetRotationAtDistanceAlongSpline` _spline _returnvalue_4 "World")))
  (for _index (range (+ _returnvalue_3 1))
    (bind _returnvalue_5 (* _index (* (`self.MeshSize`) (`self.ObjectScale`))))
    (bind (_returnvalue_roll_2 _returnvalue_pitch_2 _returnvalue_yaw_2) (`KismetMathLibrary.BreakRotator` (`SplineComponent.GetRotationAtDistanceAlongSpline` _spline_2 _returnvalue_5 "World")))
    (bind _returnvalue_6 (`AddComponent|NODE_AddStaticMeshComponent-0` :`RelativeTransform` (`KismetMathLibrary.MakeTransform` (- (`SplineComponent.GetLocationAtDistanceAlongSpline` _spline_2 _returnvalue_5 "World") (`self.K2_GetActorLocation`)) (`KismetMathLibrary.MakeRotator` 0.0 0.0 (+ _returnvalue_yaw_2 (`self.RotationYawOffset`))) (* (`KismetMathLibrary.MakeVector` 1.0 1.0 1.0) (`self.ObjectScale`)))))
    (`StaticMeshComponent.SetStaticMesh` _returnvalue_6 (`self.MeshToRepeat`)))
  (bind _returnvalue_7 (`AddComponent|NODE_AddStaticMeshComponent-3` :`RelativeTransform` (`KismetMathLibrary.MakeTransform` (- (`SplineComponent.GetLocationAtDistanceAlongSpline` _spline _returnvalue "World") (`self.K2_GetActorLocation`)) (`KismetMathLibrary.MakeRotator` 0.0 0.0 (+ _returnvalue_yaw (`self.RotationYawOffset`))) (`KismetMathLibrary.MakeVector` (`self.ObjectScale`) (* (/ (- _returnvalue _returnvalue_4) _returnvalue_2) (`self.ObjectScale`)) (`self.ObjectScale`)))))
  (`StaticMeshComponent.SetStaticMesh` _returnvalue_7 (`self.MeshToRepeat`)))