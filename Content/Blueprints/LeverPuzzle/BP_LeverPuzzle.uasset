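; BP_LeverPuzzle is the manager actor for a lever-and-door puzzle and detects when the puzzle is completed.
; On BeginPlay it passes its Doors array to the handler child actor of each entry in Levers, printing debug messages.
; Until solved, Tick polls CheckCompleted on the first door only, then latches Solved and shows a completion message through the first BP_DialogueSystem found in the level.
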(event `self.ReceiveBeginPlay`
  (bind _doors (`self.Doors`))
  (for _array_element (`self.Levers`)
    (bind _asbp_lever_puzzle_lever_handler (cast `/Game/Blueprints/Levers/BP_LeverPuzzleLeverHandler` (`ChildActorComponent.ChildActor` (`/Game/Blueprints/Levers/BP_Lever.LeverHandler` _array_element)))
      (:`then`
        (set `/Game/Blueprints/Levers/BP_LeverPuzzleLeverHandler.Doors` _doors _asbp_lever_puzzle_lever_handler)
        (`KismetSystemLibrary.PrintString` (`KismetStringLibrary.Conv_IntToString` (`KismetArrayLibrary.Array_Length` _doors))))
      (:`CastFailed`
        (`KismetSystemLibrary.PrintString` "Cast failed!")))))

(event `self.ReceiveTick`
  (params (DeltaSeconds :type "Float (single-precision)"))
  (if (not (`self.Solved`))
    (bind _completed (`/Game/Blueprints/LeverPuzzle/BP_door.CheckCompleted` (`KismetArrayLibrary.Array_Get` (`self.Doors`))))
    (if _completed
      (set `self.Solved` true)
      (bind _outactors (`GameplayStatics.GetAllActorsOfClass` "/Game/Blueprints/BP_DialogueSystem.BP_DialogueSystem_C"))
      (`/Game/Blueprints/BP_DialogueSystem.ShowMessage` (`KismetArrayLibrary.Array_Get` _outactors) "Puzzle completed!" "NewEnumerator0"))))

(fn `UserConstructionScript`
  (`parent.UserConstructionScript`))