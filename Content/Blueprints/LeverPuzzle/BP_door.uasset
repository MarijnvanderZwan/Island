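; BP_door is a lever puzzle door built from a vertical stack of animated skeletal mesh segments.
; The construction script rebuilds NumberOfSegments evenly spaced mesh components and a parallel array of active flags, all starting false.
; ToggleSegment flips one segment's flag and plays the matching one-shot clockwise or anti-clockwise Tourniquet animation.
; ToggleSegments is an empty stub, and the ToggleSegment calls in the event graph are unwired.
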(event `Key|One` :consume false
  (params (Key :type "Key Structure" :default "AnyKey")))

(event `Key|Two` :consume false
  (params (Key :type "Key Structure" :default "AnyKey")))

(event `Key|Three` :consume false
  (params (Key :type "Key Structure" :default "AnyKey")))

(event `Key|Four` :consume false
  (params (Key :type "Key Structure" :default "AnyKey")))

(event `Key|Five` :consume false
  (params (Key :type "Key Structure" :default "AnyKey")))

(fn `ToggleSegment`
  (params (index :type Integer))
  (bind _segmentactive (`self.SegmentActive`))
  (bind _item (`KismetArrayLibrary.Array_Get` (`self.Segments`) index))
  (bind _returnvalue (not (`KismetArrayLibrary.Array_Get` _segmentactive index)))
  (`KismetArrayLibrary.Array_Set` _segmentactive index _returnvalue)
  (if _returnvalue
    (`SkeletalMeshComponent.PlayAnimation` _item "/Game/Meshes/Arnimated/Tourniquet_ClockW.Tourniquet_ClockW" false)
    (else
      (`SkeletalMeshComponent.PlayAnimation` _item "/Game/Meshes/Arnimated/Tourniquet_AntiClockW.Tourniquet_AntiClockW" false))))

(fn `ToggleSegments`
  (params (NewParam :type "Array of Integer")))

(fn `UserConstructionScript`
  (`KismetArrayLibrary.Array_Clear` (`self.Segments`))
  (`KismetArrayLibrary.Array_Clear` (`self.SegmentActive`))
  (for _index (range 1 (+ (`self.NumberOfSegments`) 1))
    (bind _returnvalue (`AddComponent|Skeletal Mesh Component_0` :`RelativeTransform` (`KismetMathLibrary.MakeTransform` (`KismetMathLibrary.MakeVector` 0.0 0.0 (* (- _index 1) 40.0)))))
    (`KismetArrayLibrary.Array_Add` (`self.Segments`) _returnvalue)
    (`KismetArrayLibrary.Array_Add` (`self.SegmentActive`) false)))