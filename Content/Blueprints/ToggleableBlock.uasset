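; ToggleableBlock is a block actor that switches between visible and solid or hidden and passable when toggled.
; The Toggle event runs the parent's toggle logic, then passes the Toggled state to SetActorActive.
; SetActorActive sets the Block component's visibility without propagating to children and switches its collision between query-and-physics and none.
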(event `self.Toggle`
  (`parent.Toggle`)
  (`self.SetActorActive` (`self.Toggled`)))

(fn `SetActorActive`
  (params (Active :type Boolean))
  (bind _block (`self.Block`))
  (`SceneComponent.SetVisibility` _block Active false)
  (if Active
    (`PrimitiveComponent.SetCollisionEnabled` (`self.Block`) "QueryAndPhysics")
    (else
      (`PrimitiveComponent.SetCollisionEnabled` _block "NoCollision"))))

(fn `UserConstructionScript`
  (`parent.UserConstructionScript`))