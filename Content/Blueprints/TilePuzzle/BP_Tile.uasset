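; BP_Tile is a floor tile in a tile puzzle that toggles on or off when the player overlaps its box.
; Each toggle swaps the mesh material between ruby and cube and increments or decrements the owning Puzzle's solved-tile count.
; Toggling stops once the Puzzle reports it is solved.
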(event `Toggle`
  (bind _staticmesh (`self.StaticMesh`))
  (bind _puzzle (`self.Puzzle`))
  (if (not (`/Game/Blueprints/BP_Puzzle.Solved` (`self.Puzzle`)))
    (bind _output_get (set `self.Enabled` (not (`self.Enabled`))))
    (if _output_get
      (`PrimitiveComponent.SetMaterial` _staticmesh 0 "/Game/Materials/M_Ruby.M_Ruby")
      (`/Game/Blueprints/TilePuzzle/BP_TilePuzzle.IncrementNumberOfSolvedTiles` _puzzle)
      (else
        (`PrimitiveComponent.SetMaterial` _staticmesh 0 "/Game/Materials/M_Cube.M_Cube")
        (`/Game/Blueprints/TilePuzzle/BP_TilePuzzle.DecrementNumberOfSolvedTiles` _puzzle)))))

(event `self.Box.OnComponentBeginOverlap`
  (params (OverlappedComponent :type "PrimitiveComponent Object Reference") (OtherActor :type "Actor Object Reference") (OtherComp :type "PrimitiveComponent Object Reference") (OtherBodyIndex :type Integer) (bFromSweep :type Boolean) (SweepResult :type "HitResult Structure (by ref)"))
  (cast `/Game/Blueprints/BP_Player` OtherActor)
  (`self.Toggle`))

(fn `UserConstructionScript`)