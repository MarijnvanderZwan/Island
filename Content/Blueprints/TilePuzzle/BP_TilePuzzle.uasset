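; Tile puzzle actor that spawns a grid of BP_Tile and completes its child goal flag once every tile is solved.
; Grid size drives the trigger box and tile layout; cells blocked by collision get no tile and are excluded from the total.
; While unsolved, the box disables player jumping and shows the remaining-tile counter.
; Increment and decrement functions track solved tiles, update that counter and restore jumping on completion.
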(event `self.ReceiveBeginPlay`
  (`self.UpdatePuzzleCollision`)
  (`self.InitializeTileGrid`)
  (bind _foundwidgets (`WidgetBlueprintLibrary.GetAllWidgetsOfClass` "/Game/Blueprints/UI/UI_CollectableCounter.UI_CollectableCounter_C"))
  (`/Game/Blueprints/UI/UI_CollectableCounter.SetTileCounterDisabled` (`|GetArrayItem` _foundwidgets)))

(event `self.Box.OnComponentBeginOverlap`
  (params (OverlappedComponent :type "PrimitiveComponent Object Reference") (OtherActor :type "Actor Object Reference") (OtherComp :type "PrimitiveComponent Object Reference") (OtherBodyIndex :type Integer) (bFromSweep :type Boolean) (SweepResult :type "HitResult Structure (by ref)"))
  (if (not (`self.Solved`))
    (bind _asbp_player (cast `/Game/Blueprints/BP_Player` OtherActor))
    (set `Character.JumpMaxCount` 0 _asbp_player)
    (bind _foundwidgets (`WidgetBlueprintLibrary.GetAllWidgetsOfClass` "/Game/Blueprints/UI/UI_CollectableCounter.UI_CollectableCounter_C"))
    (bind _output (`|GetArrayItem` _foundwidgets))
    (`/Game/Blueprints/UI/UI_CollectableCounter.SetTileCounterEnabled` _output)
    (`/Game/Blueprints/UI/UI_CollectableCounter.UpdateTileCounter` _output (- (`self.TotalTiles`) (`self.TilesSolved`)))))

(event `self.Box.OnComponentEndOverlap`
  (params (OverlappedComponent :type "PrimitiveComponent Object Reference") (OtherActor :type "Actor Object Reference") (OtherComp :type "PrimitiveComponent Object Reference") (OtherBodyIndex :type Integer))
  (if (not (`self.Solved`))
    (bind _asbp_player (cast `/Game/Blueprints/BP_Player` OtherActor))
    (set `Character.JumpMaxCount` 1 _asbp_player)
    (bind _foundwidgets (`WidgetBlueprintLibrary.GetAllWidgetsOfClass` "/Game/Blueprints/UI/UI_CollectableCounter.UI_CollectableCounter_C"))
    (`/Game/Blueprints/UI/UI_CollectableCounter.SetTileCounterDisabled` (`|GetArrayItem` _foundwidgets))))

(fn `DecrementNumberOfSolvedTiles`
  (bind _returnvalue (- (`self.TotalTiles`) (`self.TilesSolved`)))
  (set `self.TilesSolved` (- (`self.TilesSolved`) 1))
  (bind _foundwidgets (`WidgetBlueprintLibrary.GetAllWidgetsOfClass` "/Game/Blueprints/UI/UI_CollectableCounter.UI_CollectableCounter_C"))
  (`/Game/Blueprints/UI/UI_CollectableCounter.UpdateTileCounter` (`|GetArrayItem` _foundwidgets) _returnvalue)
  (if (== _returnvalue 0)
    (`self.PuzzleCompleted`)))

(fn `IncrementNumberOfSolvedTiles`
  (bind _returnvalue (- (`self.TotalTiles`) (`self.TilesSolved`)))
  (set `self.TilesSolved` (+ (`self.TilesSolved`) 1))
  (bind _foundwidgets (`WidgetBlueprintLibrary.GetAllWidgetsOfClass` "/Game/Blueprints/UI/UI_CollectableCounter.UI_CollectableCounter_C"))
  (`/Game/Blueprints/UI/UI_CollectableCounter.UpdateTileCounter` (`|GetArrayItem` _foundwidgets) _returnvalue)
  (if (== _returnvalue 0)
    (`self.PuzzleCompleted`)))

(fn `InitializeTileGrid`
  (bind _cellsize (`self.CellSize`))
  (bind _topleft (`self.GetTopLeft`))
  (for _index (range 1 (+ (`self.Width`) 1))
    (for _index_2 (range 1 (+ (`self.Depth`) 1))
      (bind _returnvalue (`|SpawnActorFromClass` "/Game/Blueprints/TilePuzzle/BP_Tile.BP_Tile_C" (`KismetMathLibrary.MakeTransform` (+ (+ _topleft (`KismetMathLibrary.MakeVector` (* _index _cellsize) (* _index_2 _cellsize))) (`self.K2_GetActorLocation`) (0.0 0.0 200.0))) "DontSpawnIfColliding" "OverrideRootScale" null null))
      (if (`KismetSystemLibrary.IsValid` _returnvalue)
        (set `/Game/Blueprints/TilePuzzle/BP_Tile.Puzzle` self _returnvalue)
        (set `self.TotalTiles` (+ (`self.TotalTiles`) 1))))))

(fn `PuzzleCompleted`
  (set `self.Solved` true)
  (bind _asbp_goal_flag (cast `/Game/Blueprints/Goals/BP_GoalFlag` (`ChildActorComponent.ChildActor` (`self.ChildActor`))))
  (`/Game/Blueprints/Goals/BP_GoalFlag.SetCompleted` _asbp_goal_flag)
  (bind _outactors (`GameplayStatics.GetAllActorsOfClass` "/Game/Blueprints/BP_Player.BP_Player_C"))
  (set `Character.JumpMaxCount` 1 (`|GetArrayItem` _outactors)))

(fn `UpdatePuzzleCollision`
  (`BoxComponent.SetBoxExtent` (`self.Box`) (`KismetMathLibrary.MakeVector` (* (* (`self.Width`) (`self.CellSize`)) 0.5) (* (* (`self.Depth`) (`self.CellSize`)) 0.5) 400.0) false))

(fn `UserConstructionScript`
  (`parent.UserConstructionScript`))