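; Lever handler for a lever puzzle that toggles segments on the puzzle's doors when its lever moves.
; LeverUp and LeverDown each call the parent event, then share one loop that calls ToggleSegment on every entry in Doors for each of LinkedSegments.
; Both directions perform the same toggle rather than setting an explicit state.
; The assignment of Doors from LeverPuzzle is disconnected, so this graph never fills that array.
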(event `self.ReceiveBeginPlay`)

(event `self.LeverUp`
  (`parent.LeverUp`)
  (for _array_element (`self.LinkedSegments`) :!label _label
    (for _array_element_2 (`self.Doors`)
      (`/Game/Blueprints/LeverPuzzle/BP_door.ToggleSegment` _array_element_2 _array_element))))

(event `self.LeverDown`
  (`parent.LeverDown`)
  (goto _label))

(fn `UserConstructionScript`
  (`parent.UserConstructionScript`))