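; BP_Lever is an interactable lever that toggles between up and down.
; Its Interact event checks the LeverUp flag, calls LeverDown or LeverUp on a BP_LeverHandler child actor, then flips the flag.
; The construction script passes its Lever reference to that handler, keeping the up and down behavior in the child actor.
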(event `Interact`
  (bind _asbp_lever_handler (cast `/Game/Blueprints/Levers/BP_LeverHandler` (`ChildActorComponent.ChildActor` (`self.LeverHandler`))))
  (if (`self.LeverUp`)
    (`/Game/Blueprints/Levers/BP_LeverHandler.LeverDown` _asbp_lever_handler)
    (set `self.LeverUp` false)
    (else
      (`/Game/Blueprints/Levers/BP_LeverHandler.LeverUp` _asbp_lever_handler)
      (set `self.LeverUp` true))))

(fn `UserConstructionScript`
  (bind _asbp_lever_handler (cast `/Game/Blueprints/Levers/BP_LeverHandler` (`ChildActorComponent.ChildActor` (`self.LeverHandler`))))
  (set `/Game/Blueprints/Levers/BP_LeverHandler.Lever` (`self.Lever`) _asbp_lever_handler))